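; BP_UIManager manages the game's HUD widgets: a unit actions menu, info messages and faction turn announcements.
; Each display function lazily creates its widget, caches it and adds it to the viewport only when not already shown, then passes the message or faction to it.
; Other functions forward unit actions, enabled state and faction button styling to the cached actions menu, disabling it on a faction change.
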(fn `ChangeActionsMenuFaction`
  (params (Faction :type "/Game/Blueprint/E_Faction Enum" :default "NewEnumerator0"))
  (bind _actionsmenu (`self.ActionsMenu`))
  (`/Game/UserInterface/WBP_ActionsMenu.SetButtonsStyle` _actionsmenu Faction)
  (`Widget.SetIsEnabled` _actionsmenu false)
  (return))

(fn `DisplayActionsMenu`
  (bind _actionsmenu (`self.ActionsMenu`))
  (`/Engine/EditorBlueprintResources/StandardMacros.IsValid` _actionsmenu
    (:`Is Valid`
      (if (not (`Widget.IsInViewport` _actionsmenu))
        (`UserWidget.AddToViewport` (stale _output_get) 0 :!label _label)
        (return)))
    (:`Is Not Valid`
      (bind _returnvalue (`|CreateWidget` "/Game/UserInterface/WBP_ActionsMenu.WBP_ActionsMenu_C"))
      (bind _output_get (set `self.ActionsMenu` _returnvalue))
      (goto _label))))

(fn `DisplayFactionTurnMessage`
  (params (Faction :type "/Game/Blueprint/E_Faction Enum" :default "NewEnumerator0"))
  (bind _factionturnmessage (`self.FactionTurnMessage`))
  (`/Engine/EditorBlueprintResources/StandardMacros.IsValid` _factionturnmessage
    (:`Is Valid`
      (if (not (`Widget.IsInViewport` _factionturnmessage))
        (`UserWidget.AddToViewport` (stale _output_get) 0 :!label _label)))
    (:`Is Not Valid`
      (bind _returnvalue (`|CreateWidget` "/Game/UserInterface/WBP_FactionTurnMessage.WBP_FactionTurnMessage_C"))
      (bind _output_get (set `self.FactionTurnMessage` _returnvalue))
      (goto _label)))
  (`/Game/UserInterface/WBP_FactionTurnMessage.DisplayFactionTurn` (`self.FactionTurnMessage`) Faction)
  (return))

(fn `DisplayInfoMessage`
  (params (Message :type String))
  (bind _infomessage (`self.InfoMessage`))
  (`/Engine/EditorBlueprintResources/StandardMacros.IsValid` _infomessage
    (:`Is Valid`
      (if (not (`Widget.IsInViewport` _infomessage))
        (`UserWidget.AddToViewport` (stale _output_get) 0 :!label _label)))
    (:`Is Not Valid`
      (bind _returnvalue (`|CreateWidget` "/Game/UserInterface/WBP_InfoMessage.WBP_InfoMessage_C"))
      (bind _output_get (set `self.InfoMessage` _returnvalue))
      (goto _label)))
  (`/Game/UserInterface/WBP_InfoMessage.DisplayInfoMessage` (`self.InfoMessage`) Message)
  (return))

(fn `SetIsActionsMenuEnabled`
  (params (IsEnabled :type Boolean))
  (`Widget.SetIsEnabled` (`self.ActionsMenu`) IsEnabled)
  (return))

(fn `UpdateActionsMenu`
  (params (UnitActions :type "/Game/Blueprint/S_UnitActions Structure"))
  (`/Game/UserInterface/WBP_ActionsMenu.UpdateMenu` (`self.ActionsMenu`) UnitActions)
  (return))

(fn `UserConstructionScript`)