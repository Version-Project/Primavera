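; BP_Cursor is a cursor actor that attaches to a given unit and shows a spinning model.
; BeginPlay hides CursorModel and calls Rotate, which applies a yaw step, waits RotationSpeed seconds, then re-calls itself while IsEnabled is true.
; AttachCursorToUnit shows the model, attaches the actor, sets IsEnabled and calls Rotate.
; DetachCursorFromUnit hides the model, detaches and clears IsEnabled to end the loop.
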(event `self.ReceiveBeginPlay`
  (`SceneComponent.SetVisibility` (`self.CursorModel`) false false)
  (`self.Rotate`))

(event `Rotate`
  (`SceneComponent.K2_AddWorldRotation` (`self.CursorModel`) (`KismetMathLibrary.MakeRotator` 0.0 0.0 (`self.RotationAngle`)) false false)
  (`KismetSystemLibrary.Delay` (`self.RotationSpeed`))
  (if (`self.IsEnabled`)
    (`self.Rotate`)))

(fn `AttachCursorToUnit`
  (params (Unit :type "Actor Object Reference"))
  (`SceneComponent.SetVisibility` (`self.CursorModel`) true false)
  (`self.K2_AttachToActor` Unit "None" "KeepRelative" "KeepRelative" "KeepRelative")
  (set `self.IsEnabled` true)
  (`self.Rotate`))

(fn `DetachCursorFromUnit`
  (`SceneComponent.SetVisibility` (`self.CursorModel`) false false)
  (`self.K2_DetachFromActor` "KeepRelative")
  (set `self.IsEnabled` false))

(fn `UserConstructionScript`)