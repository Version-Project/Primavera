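; BP_Block is a clickable board tile in a turn-based faction tactics game, linked to an optional unit at BeginPlay.
; Construction colors the cube by owning faction and incrustation level, and derives grid coordinates from the number in the actor's display name.
; A hover plane follows the cursor.
; Clicks depend on BP_GameState's phase: selecting or clearing the acting unit, or moving it onto range-highlighted tiles and otherwise cancelling the move.
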(event `self.ReceiveBeginPlay`
  (bind _bindedunit (`self.BindedUnit`))
  ;[1 1 1] Bind Block to Unit
  (`/Engine/EditorBlueprintResources/StandardMacros.IsValid` _bindedunit
    (:`Is Valid`
      (`/Game/Blueprint/Units/BP_Unit.BindBlock` _bindedunit self))))

(event `self.ReceiveActorBeginCursorOver`
  ;[1 1 1] Manage Hovering Plane visibility
  (`SceneComponent.SetVisibility` (`self.HoveringPlane`) true false))

(event `self.ReceiveActorEndCursorOver`
  ;[1 1 1] Manage Hovering Plane visibility
  (`SceneComponent.SetVisibility` (`self.HoveringPlane`) false false))

(event `self.ReceiveActorOnClicked`
  (params (ButtonPressed :type "Key Structure"))
  (`self.ManageClick`))

(fn `ManageClick`
  (locals (GameState :type "/Game/Blueprint/Core/BP_GameState Object Reference"))
  (bind _gamestate (`local.GameState`))
  (bind _bindedunit (`self.BindedUnit`))
  (bind _asbp_game_state (cast `/Game/Blueprint/Core/BP_GameState` (`GameplayStatics.GetGameState`)))
  (bind _output_get (set `local.GameState` _asbp_game_state))
  (switch `/Game/Blueprint/Enum_Phase` (`/Game/Blueprint/Core/BP_GameState.CurrPhase` _output_get)
    (:`NewEnumerator0`
      (bind _hasacted (`/Game/Blueprint/Core/BP_GameState.CheckIfUnitHasActed` (`local.GameState`)))
      (if (not _hasacted)
        (`/Engine/EditorBlueprintResources/StandardMacros.IsValid` _bindedunit
          (:`Is Valid`
            (if (`|EnumEquality` (`/Game/Blueprint/Core/BP_GameState.CurrFaction` (`local.GameState`)) (`/Game/Blueprint/Units/BP_Unit.Faction` _bindedunit))
              (if (`/Game/Blueprint/Units/BP_Unit.HasAlreadyBeenPlayed` (`self.BindedUnit`))
                (`/Game/Blueprint/Core/BP_GameState.DefineUnitToAct` (`local.GameState`) null :!label _label)
                (else
                  (`/Game/Blueprint/Core/BP_GameState.DefineUnitToAct` (`local.GameState`) (`self.BindedUnit`))))
              (else
                (goto _label))))
          (:`Is Not Valid`
            (goto _label)))))
    (:`NewEnumerator1`
      (if (`SceneComponent.IsVisible` (`self.ActionRangePlane`))
        (bind _unittoact (`/Game/Blueprint/Core/BP_GameState.GetUnitToAct` (`local.GameState`)))
        (`/Game/Blueprint/Units/BP_Unit.MoveUnit` _unittoact self)
        (else
          (`/Game/Blueprint/Core/BP_GameState.Hide Move Range` _gamestate)
          (set `/Game/Blueprint/Core/BP_GameState.CurrPhase` "NewEnumerator0" _gamestate))))))

(fn `UpdateColor`
  (bind _cube (`self.Cube`))
  (switch `/Game/Blueprint/Enum_Faction` (`self.BlockOwner`)
    (:`NewEnumerator1`
      (switch `int` (`self.IncrustationLevel`)
        (:`1`
          (`PrimitiveComponent.SetMaterial` _cube 0 "/Game/Materials/Mat_BlueLV1.Mat_BlueLV1"))
        (:`2`
          (`PrimitiveComponent.SetMaterial` _cube 0 "/Game/Materials/Mat_BlueLV2.Mat_BlueLV2"))
        (:`3`
          (`PrimitiveComponent.SetMaterial` _cube 0 "/Game/Materials/Mat_BlueLV3.Mat_BlueLV3"))))
    (:`NewEnumerator2`
      (switch `int` (`self.IncrustationLevel`)
        (:`1`
          (`PrimitiveComponent.SetMaterial` _cube 0 "/Game/Materials/Mat_OrangeLV1.Mat_OrangeLV1"))
        (:`2`
          (`PrimitiveComponent.SetMaterial` _cube 0 "/Game/Materials/Mat_OrangeLV2.Mat_OrangeLV2"))
        (:`3`
          (`PrimitiveComponent.SetMaterial` _cube 0 "/Game/Materials/Mat_OrangeLV3.Mat_OrangeLV3"))))))

(fn `UserConstructionScript`
  (`self.UpdateColor`)
  (bind _output_get (set `self.Index` (`KismetStringLibrary.Conv_StringToInt` (`.RightS` (`KismetStringLibrary.Split` (`KismetSystemLibrary.GetDisplayName` self) "k" "IgnoreCase" "FromEnd")))))
  (bind (_x _y) (`/Game/Blueprint/BP_CoordsFunctionLibrary.GetBlockCoordinates` _output_get))
  (set `self.Coords` (make `/Game/Blueprint/Struct_Coords` _x _y))
  (`SceneComponent.SetVisibility` (`self.HoveringPlane`) false false)
  (`SceneComponent.SetVisibility` (`self.ActionRangePlane`) false false))