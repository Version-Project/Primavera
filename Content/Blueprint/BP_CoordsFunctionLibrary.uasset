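; BP_CoordsFunctionLibrary is a Blueprint function library of coordinate helpers for a fixed 16 by 11 block grid.
; It converts between a flat block index and X/Y coordinates with X * 11 + Y, and can return them as an SCoords struct.
; Other helpers compare coordinates, offset relative ones from a reference point and check bounds.
; The index check accepts 0 to 174, excluding the grid's last cell at 175.
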(fn `AreCoordsEqual`
  (params (Coords1 :type "/Game/Blueprint/S_Coords Structure") (Coords2 :type "/Game/Blueprint/S_Coords Structure"))
  (returns (bAreEqual :type Boolean))
  (return (and (== Coords1_X_5_364656D3417FA6B1F82E4585A34E5C6B Coords2_X_5_364656D3417FA6B1F82E4585A34E5C6B) (== Coords1_Y_6_2DC6362D4EE28ABEA56491A3230A1BE6 Coords2_Y_6_2DC6362D4EE28ABEA56491A3230A1BE6))))

(fn `AreCoordsInBounds`
  (params (X :type Integer) (Y :type Integer))
  (returns (bInBounds :type Boolean))
  (return (and (>= X 0) (< X 16) (>= Y 0) (< Y 11))))

(fn `GetAbsoluteCoordsFromRelatives`
  (params (ReferencePoint :type "/Game/Blueprint/S_Coords Structure") (RelativeCoords :type "/Game/Blueprint/S_Coords Structure"))
  (returns (AbsoluteCoords :type "/Game/Blueprint/S_Coords Structure"))
  (return (make `/Game/Blueprint/S_Coords` (+ ReferencePoint_X_5_364656D3417FA6B1F82E4585A34E5C6B RelativeCoords_X_5_364656D3417FA6B1F82E4585A34E5C6B) (+ ReferencePoint_Y_6_2DC6362D4EE28ABEA56491A3230A1BE6 RelativeCoords_Y_6_2DC6362D4EE28ABEA56491A3230A1BE6))))

(fn `GetBlockCoordinates`
  (params (Index :type Integer))
  (returns (X :type Integer) (Y :type Integer))
  (bind (_remainder _returnvalue) (`KismetMathLibrary.FMod` (`KismetMathLibrary.Conv_IntToDouble` Index) 11.0))
  (return _returnvalue (`KismetMathLibrary.FTrunc` _remainder)))

(fn `GetBlockIndex`
  (params (X :type Integer) (Y :type Integer))
  (returns (Index :type Integer))
  (return (+ (* X 11) Y)))

(fn `GetStructCoordsFromIndex`
  (params (BlockIndex :type Integer))
  (returns (Coords :type "/Game/Blueprint/S_Coords Structure"))
  (bind (_x _y) (`self.GetBlockCoordinates` BlockIndex))
  (return (make `/Game/Blueprint/S_Coords` _x _y)))

(fn `IsIndexInBounds`
  (params (Index :type Integer))
  (returns (bInBounds :type Boolean))
  (return (and (>= Index 0) (< Index 175))))