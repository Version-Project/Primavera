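; BP_Protector is a grid-based unit Blueprint for the Protector, a shield-bearing class that belongs to the Blue or Orange faction.
; Its construction script runs the parent setup, sets the unit class, and applies the faction's level-one material to both shield components.
; On BeginPlay it builds MoveRange row by row as a diamond of relative coordinates within three Manhattan steps, excluding its own tile.
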(event `self.ReceiveBeginPlay`
  (`self.DefineMoveRange`))

(fn `DefineMoveRange`
  (bind _moverange (`self.MoveRange`))
  (`self.AddConsecutivePossibleCoords` 0 0 -3 -3 _moverange)
  (`self.AddConsecutivePossibleCoords` -1 1 -2 -2 _moverange)
  (`self.AddConsecutivePossibleCoords` -2 2 -1 -1 _moverange)
  (`self.AddConsecutivePossibleCoords` -3 -1 0 0 _moverange)
  (`self.AddConsecutivePossibleCoords` 1 3 0 0 _moverange)
  (`self.AddConsecutivePossibleCoords` -2 2 1 1 _moverange)
  (`self.AddConsecutivePossibleCoords` -1 1 2 2 _moverange)
  (`self.AddConsecutivePossibleCoords` 0 0 3 3 _moverange))

(fn `UserConstructionScript`
  (`parent.UserConstructionScript`)
  (set `self.Class` "NewEnumerator1")
  (switch `/Game/Blueprint/Enum_Faction` (`self.Faction`)
    (:`NewEnumerator1`
      (`PrimitiveComponent.SetMaterial` (`self.Shield1`) 0 "/Game/Materials/Mat_BlueLV1.Mat_BlueLV1")
      (`PrimitiveComponent.SetMaterial` (`self.Shield2`) 0 "/Game/Materials/Mat_BlueLV1.Mat_BlueLV1"))
    (:`NewEnumerator2`
      (`PrimitiveComponent.SetMaterial` (`self.Shield1`) 0 "/Game/Materials/Mat_OrangeLV1.Mat_OrangeLV1")
      (`PrimitiveComponent.SetMaterial` (`self.Shield2`) 0 "/Game/Materials/Mat_OrangeLV1.Mat_OrangeLV1"))))