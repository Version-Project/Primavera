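; BP_Sniper is a unit Blueprint that defines the Sniper's class and its movement range on a coordinate grid.
; The construction script runs the parent's script, then sets the Class enum.
; On BeginPlay, DefineMoveRange fills MoveRange row by row through AddConsecutivePossibleCoords, forming a diamond of offsets up to three cells away by Manhattan distance, excluding the unit's own cell.
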(event `self.ReceiveBeginPlay`
  (`self.DefineMoveRange`))

(fn `DefineMoveRange`
  (bind _moverange (`self.MoveRange`))
  (`self.AddConsecutivePossibleCoords` 0 0 -3 -3 _moverange)
  (`self.AddConsecutivePossibleCoords` -1 1 -2 -2 _moverange)
  (`self.AddConsecutivePossibleCoords` -2 2 -1 -1 _moverange)
  (`self.AddConsecutivePossibleCoords` -3 -1 0 0 _moverange)
  (`self.AddConsecutivePossibleCoords` 1 3 0 0 _moverange)
  (`self.AddConsecutivePossibleCoords` -2 2 1 1 _moverange)
  (`self.AddConsecutivePossibleCoords` -1 1 2 2 _moverange)
  (`self.AddConsecutivePossibleCoords` 0 0 3 3 _moverange))

(fn `UserConstructionScript`
  (`parent.UserConstructionScript`)
  (set `self.Class` "NewEnumerator0"))