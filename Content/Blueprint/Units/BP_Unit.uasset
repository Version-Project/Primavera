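; BP_Unit is the base grid unit, colored by Blue or Orange faction in its construction script.
; Clicking it opens the player state's actions menu, and hovering toggles the hover plane on its bound block.
; MoveUnit relinks the two-way unit-block binding, teleports onto the new block and hides the move range.
; DefineMoveRange is a print-only superclass stub, alongside a helper that fills rectangular coordinate ranges.
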(event `self.ReceiveActorOnClicked`
  (params (ButtonPressed :type "Key Structure"))
  (bind _asbp_player_state (cast `/Game/Blueprint/Core/BP_PlayerState` (`GameplayStatics.GetPlayerState` 0)))
  (`/Game/Blueprint/Core/BP_PlayerState.ShowActionsMenu` _asbp_player_state self))

(event `self.ReceiveActorBeginCursorOver`
  (`SceneComponent.SetVisibility` (`/Game/Blueprint/BP_Block.HoveringPlane` (`self.BindedBlock`)) true false))

(event `self.ReceiveActorEndCursorOver`
  (`SceneComponent.SetVisibility` (`/Game/Blueprint/BP_Block.HoveringPlane` (`self.BindedBlock`)) false false))

(fn `AddConsecutivePossibleCoords`
  (params (FirstX :type Integer) (LastX :type Integer) (FirstY :type Integer) (LastY :type Integer) (Array :type "Array of /Game/Blueprint/Struct_Coords Structure"))
  (for _index (range FirstX (+ LastX 1))
    (for _index_2 (range FirstY (+ LastY 1))
      (`KismetArrayLibrary.Array_Add` Array (make `/Game/Blueprint/Struct_Coords` _index _index_2)))))

(fn `BindBlock`
  (params (Block :type "/Game/Blueprint/BP_Block Object Reference"))
  (set `self.BindedBlock` Block))

(fn `DefineMoveRange`
  (`KismetSystemLibrary.PrintString` "Defining Move Range for Unit superclass."))

(fn `MoveUnit`
  (params (NewBindedBlock :type "/Game/Blueprint/BP_Block Object Reference"))
  (bind (_returnvalue_x _returnvalue_y) (`KismetMathLibrary.BreakVector` (`self.K2_GetActorLocation` NewBindedBlock)))
  (set `/Game/Blueprint/BP_Block.BindedUnit` null (`self.BindedBlock`)) ; Remove prev link from Block to Unit.
  (bind _output_get (set `self.BindedBlock` NewBindedBlock)) ; Add new link from Unit to Block.
  (set `/Game/Blueprint/BP_Block.BindedUnit` self _output_get) ; Add new link from Block to Unit.
  (`self.K2_SetActorLocation` (`KismetMathLibrary.MakeVector` _returnvalue_x _returnvalue_y 75.0) false true)
  (bind _asbp_player_state (cast `/Game/Blueprint/Core/BP_PlayerState` (`GameplayStatics.GetPlayerState` 0)))
  (`/Game/Blueprint/Core/BP_PlayerState.HideMoveRange` _asbp_player_state))

(fn `UserConstructionScript`
  (switch `/Game/Blueprint/Enum_Faction` (`self.Faction`)
    (:`NewEnumerator1`
      (`PrimitiveComponent.SetMaterial` (`self.Head`) 0 "/Game/Materials/Mat_BlueLV2.Mat_BlueLV2")
      (`PrimitiveComponent.SetMaterial` (`self.Body`) 0 "/Game/Materials/Mat_BlueLV3.Mat_BlueLV3"))
    (:`NewEnumerator2`
      (`PrimitiveComponent.SetMaterial` (`self.Head`) 0 "/Game/Materials/Mat_OrangeLV2.Mat_OrangeLV2")
      (`PrimitiveComponent.SetMaterial` (`self.Body`) 0 "/Game/Materials/Mat_OrangeLV3.Mat_OrangeLV3"))))