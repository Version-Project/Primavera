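; Game state for a turn-based grid tactics game where Blue and Orange factions alternate after each unit's turn.
; On BeginPlay it indexes all BP_Blocks into a Battlefield map and shows turn and faction messages through BP_UIManager.
; A History struct, sized to MaxTurns, records each acting unit and its move, attack, buff and capacity flags.
; Functions select units, show unoccupied move-range blocks, close phases and switch factions, updating the actions menu and BP_Cursor.
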(event `self.ReceiveBeginPlay`
  (bind _uimanager (`self.UIManager`))
  (bind _returnvalue (`GameplayStatics.GetActorOfClass` "/Game/Blueprint/BP_UIManager.BP_UIManager_C"))
  (set `self.UIManager` _returnvalue)
  (bind _returnvalue_2 (`GameplayStatics.GetActorOfClass` "/Game/Blueprint/BP_Cursor.BP_Cursor_C"))
  (set `self.Cursor` _returnvalue_2)
  (`|ExecutionSequence`
    (:`then_0`
      ;[1 1 1] Fill the Battlefield array with all the BP_Block.
      (bind _outactors (`GameplayStatics.GetAllActorsOfClass` "/Game/Blueprint/BP_Block.BP_Block_C"))
      (for _array_element _outactors
        (`BlueprintMapLibrary.Map_Add` (`self.Battlefield`) (`/Game/Blueprint/BP_Block.Index` _array_element) _array_element)))
    (:`then_1`
      ;[1 1 1] Display the ActionsMenu without enabling it and updates its colors.
      (`/Game/Blueprint/BP_UIManager.DisplayActionsMenu` _uimanager)
      (`/Game/Blueprint/BP_UIManager.ChangeActionsMenuFaction` _uimanager "NewEnumerator2"))
    (:`then_2`
      (`self.DisplayTurnMessage`))
    (:`then_3`
      ;[1 1 1] Display the FactionTurnMessage right before the previous InfoMessage disappears.
      (`KismetSystemLibrary.Delay` (- (`WidgetAnimation.GetEndTime` (`/Game/UserInterface/UI_InfoMessage.Appear` (`/Game/Blueprint/BP_UIManager.InfoMessage` (`self.UIManager`)))) 1.25))
      (`self.DisplayFactionMessage`))))

(event `DisplayTurnMessage`
  (bind _uimanager (`self.UIManager`))
  (bind _infomessage (`/Game/Blueprint/BP_UIManager.InfoMessage` _uimanager))
  ;[1 1 1] Event called each time a new turn starts.
  (bind _currentturn (`self.GetCurrentTurn`))
  (`/Game/Blueprint/BP_UIManager.DisplayInfoMessage` _uimanager (`KismetStringLibrary.Concat_StrStr` "TURN " (`KismetStringLibrary.Conv_IntToString` _currentturn) " / " (`KismetStringLibrary.Conv_IntToString` (`self.MaxTurns`))))
  (`KismetSystemLibrary.Delay` (`WidgetAnimation.GetEndTime` (`/Game/UserInterface/UI_InfoMessage.Appear` _infomessage)))
  (`Widget.RemoveFromParent` _infomessage))

(event `DisplayFactionMessage`
  (bind _uimanager (`self.UIManager`))
  (bind _factionturnmessage (`/Game/Blueprint/BP_UIManager.FactionTurnMessage` _uimanager))
  ;[1 1 1] Event called each time the current playing faction changes.
  (`/Game/Blueprint/BP_UIManager.DisplayFactionTurnMessage` _uimanager (`self.CurrFaction`))
  (`KismetSystemLibrary.Delay` (`WidgetAnimation.GetEndTime` (`/Game/UserInterface/UI_FactionTurnMessage.Appear` _factionturnmessage)))
  (`Widget.RemoveFromParent` _factionturnmessage))

(fn `CheckIfUnitHasActed`
  (returns (HasActed :type Boolean))
  (bind (_history_turnsactions _history_currturnidx) (break `/Game/Blueprint/Struct_GameHistory` (`self.History`)))
  (bind (_output_unitsactions _output_currentunitidx) (break `/Game/Blueprint/Struct_TurnActionsHistory` (`|GetArrayItem` _history_turnsactions _history_currturnidx)))
  (bind (_output_unit _output_moved _output_attacked _output_buffed _output_usedcapacity) (break `/Game/Blueprint/Struct_UnitActions` (`|GetArrayItem` _output_unitsactions _output_currentunitidx)))
  (return (or _output_moved _output_attacked _output_buffed _output_usedcapacity)))

(fn `DefineUnitToAct`
  (params (UnitToAct :type "/Game/Blueprint/Units/BP_Unit Object Reference"))
  (bind (_history_turnsactions _history_currturnidx) (break `/Game/Blueprint/Struct_GameHistory` (`self.History`)))
  (bind _uimanager (`self.UIManager`))
  (bind (_output_unitsactions _output_currentunitidx) (break `/Game/Blueprint/Struct_TurnActionsHistory` (`|GetArrayItem` _history_turnsactions _history_currturnidx)))
  (`KismetArrayLibrary.Array_Set` _output_unitsactions _output_currentunitidx (make `/Game/Blueprint/Struct_UnitActions` UnitToAct))
  (`/Engine/EditorBlueprintResources/StandardMacros.IsValid` UnitToAct
    (:`Is Valid`
      (`/Game/Blueprint/BP_UIManager.SetIsActionsMenuEnabled` _uimanager true)
      (`/Game/Blueprint/BP_Cursor.AttachCursorToUnit` (`self.Cursor`) UnitToAct))
    (:`Is Not Valid`
      (`/Game/Blueprint/BP_UIManager.SetIsActionsMenuEnabled` _uimanager false)
      (`/Game/Blueprint/BP_Cursor.DetachCursorFromUnit` (`self.Cursor`)))))

(fn `EndCurrentPhase`
  (bind (_history_turnsactions _history_currturnidx) (break `/Game/Blueprint/Struct_GameHistory` (`self.History`)))
  (bind (_history_turnsactions_2 _history_currturnidx_2) (break `/Game/Blueprint/Struct_GameHistory` (`self.History`)))
  (bind (_history_turnsactions_3 _history_currturnidx_3) (break `/Game/Blueprint/Struct_GameHistory` (`self.History`)))
  (bind (_history_turnsactions_4 _history_currturnidx_4) (break `/Game/Blueprint/Struct_GameHistory` (`self.History`)))
  (bind (_history_turnsactions_5 _history_currturnidx_5) (break `/Game/Blueprint/Struct_GameHistory` (`self.History`)))
  (bind (_output_unitsactions _output_currentunitidx) (break `/Game/Blueprint/Struct_TurnActionsHistory` (`|GetArrayItem` _history_turnsactions _history_currturnidx)))
  (bind (_output_unitsactions_2 _output_currentunitidx_2) (break `/Game/Blueprint/Struct_TurnActionsHistory` (`|GetArrayItem` _history_turnsactions_2 _history_currturnidx_2)))
  (bind (_output_unitsactions_3 _output_currentunitidx_3) (break `/Game/Blueprint/Struct_TurnActionsHistory` (`|GetArrayItem` _history_turnsactions_3 _history_currturnidx_3)))
  (bind (_output_unitsactions_4 _output_currentunitidx_4) (break `/Game/Blueprint/Struct_TurnActionsHistory` (`|GetArrayItem` _history_turnsactions_4 _history_currturnidx_4)))
  (bind (_output_unitsactions_5 _output_currentunitidx_5) (break `/Game/Blueprint/Struct_TurnActionsHistory` (`|GetArrayItem` _history_turnsactions_5 _history_currturnidx_5)))
  (bind (_output_unit _output_moved _output_attacked _output_buffed) (break `/Game/Blueprint/Struct_UnitActions` (`|GetArrayItem` _output_unitsactions _output_currentunitidx)))
  (bind (_output_unit_2 _output_moved_2 _output_attacked_2 _output_buffed_2 _output_usedcapacity) (break `/Game/Blueprint/Struct_UnitActions` (`|GetArrayItem` _output_unitsactions_2 _output_currentunitidx_2)))
  (bind (_output_unit_3 _output_moved_3 _output_attacked_3 _output_buffed_3 _output_usedcapacity_2) (break `/Game/Blueprint/Struct_UnitActions` (`|GetArrayItem` _output_unitsactions_4 _output_currentunitidx_4)))
  (bind (_output_unit_4 _output_moved_4 _output_attacked_4 _output_buffed_4 _output_usedcapacity_3) (break `/Game/Blueprint/Struct_UnitActions` (`|GetArrayItem` _output_unitsactions_5 _output_currentunitidx_5)))
  (switch `/Game/Blueprint/Enum_Phase` (`self.CurrPhase`)
    (:`NewEnumerator1`
      (`KismetArrayLibrary.Array_Set` _output_unitsactions_2 _output_currentunitidx_2 (make `/Game/Blueprint/Struct_UnitActions` _output_unit_2 true _output_attacked_2 _output_buffed_2 _output_usedcapacity)))
    (:`NewEnumerator2`
      (`KismetArrayLibrary.Array_Set` _output_unitsactions_5 _output_currentunitidx_5 (make `/Game/Blueprint/Struct_UnitActions` _output_unit_4 _output_moved_4 true _output_buffed_4 _output_usedcapacity_3)))
    (:`NewEnumerator3`
      (`KismetArrayLibrary.Array_Set` _output_unitsactions_4 _output_currentunitidx_4 (make `/Game/Blueprint/Struct_UnitActions` _output_unit_3 _output_moved_3 _output_attacked_3 true _output_usedcapacity_2)))
    (:`NewEnumerator4`
      (`KismetArrayLibrary.Array_Set` _output_unitsactions _output_currentunitidx (make `/Game/Blueprint/Struct_UnitActions` _output_unit _output_moved _output_attacked _output_buffed true))))
  (set `self.CurrPhase` "NewEnumerator0")
  (`/Game/Blueprint/BP_UIManager.UpdateActionsMenu` (`self.UIManager`) (`|GetArrayItem` _output_unitsactions_3 _output_currentunitidx_3)))

(fn `EndUnitTurn`
  (bind (_history_turnsactions _history_currturnidx) (break `/Game/Blueprint/Struct_GameHistory` (`self.History`)))
  (bind _uimanager (`self.UIManager`))
  (bind (_history_turnsactions_2 _history_currturnidx_2) (break `/Game/Blueprint/Struct_GameHistory` (`self.History`)))
  (bind (_output_unitsactions _output_currentunitidx) (break `/Game/Blueprint/Struct_TurnActionsHistory` (`|GetArrayItem` _history_turnsactions _history_currturnidx)))
  (bind (_output_unitsactions_2 _output_currentunitidx_2) (break `/Game/Blueprint/Struct_TurnActionsHistory` (`|GetArrayItem` _history_turnsactions_2 _history_currturnidx_2)))
  (`/Engine/EditorBlueprintResources/StandardMacros.IncrementInt` _output_currentunitidx_2
    (:`  `
      (switch `/Game/Blueprint/Enum_Faction` (`self.CurrFaction`)
        (:`NewEnumerator1`
          (set `self.CurrFaction` "NewEnumerator2"))
        (:`NewEnumerator2`
          (set `self.CurrFaction` "NewEnumerator1")))
      (`self.DisplayFactionMessage`)
      (`/Game/Blueprint/BP_UIManager.ChangeActionsMenuFaction` _uimanager (`self.CurrFaction`))
      (`/Game/Blueprint/BP_UIManager.UpdateActionsMenu` _uimanager (`|GetArrayItem` _output_unitsactions _output_currentunitidx))
      (`/Game/Blueprint/BP_Cursor.DetachCursorFromUnit` (`self.Cursor`)))))

(fn `GetCurrentTurn`
  (returns (CurrentTurn :type Integer))
  (bind (_history_turnsactions _history_currturnidx) (break `/Game/Blueprint/Struct_GameHistory` (`self.History`)))
  (return (+ _history_currturnidx 1)))

(fn `GetUnitToAct`
  (returns (UnitToAct :type "/Game/Blueprint/Units/BP_Unit Object Reference"))
  (bind (_history_turnsactions _history_currturnidx) (break `/Game/Blueprint/Struct_GameHistory` (`self.History`)))
  (bind (_output_unitsactions _output_currentunitidx) (break `/Game/Blueprint/Struct_TurnActionsHistory` (`|GetArrayItem` _history_turnsactions _history_currturnidx)))
  (bind _output_unit (break `/Game/Blueprint/Struct_UnitActions` (`|GetArrayItem` _output_unitsactions _output_currentunitidx)))
  (return _output_unit))

(fn `Hide Move Range`
  (for _index (range 176)
    (`SceneComponent.SetVisibility` (`/Game/Blueprint/BP_Block.ActionRangePlane` (`BlueprintMapLibrary.Map_Find` (`self.Battlefield`) _index)) false false)))

(fn `ShowMoveRange`
  (locals (CurrBlockCoords :type "/Game/Blueprint/Struct_Coords Structure") (AbsoluteX :type Integer) (AbsoluteY :type Integer))
  (bind _unittoact (`self.GetUnitToAct`))
  (bind _coords (`/Game/Blueprint/BP_CoordsFunctionLibrary.GetStructCoordsFromIndex` (`/Game/Blueprint/BP_Block.Index` (`/Game/Blueprint/Units/BP_Unit.BindedBlock` _unittoact))))
  (set `local.CurrBlockCoords` _coords)
  (for _array_element (`/Game/Blueprint/Units/BP_Unit.MoveRange` _unittoact)
    (bind _absolutecoords (`/Game/Blueprint/BP_CoordsFunctionLibrary.GetAbsoluteCoordsFromRelatives` (`local.CurrBlockCoords`) _array_element))
    (set `local.AbsoluteX` (break `/Game/Blueprint/Struct_Coords` _absolutecoords))
    (bind _output_get (set `local.AbsoluteY` (`.Y_6_2DC6362D4EE28ABEA56491A3230A1BE6` (break `/Game/Blueprint/Struct_Coords` _absolutecoords))))
    (bind _inbounds (`/Game/Blueprint/BP_CoordsFunctionLibrary.CheckIfCoordsAreInBounds` (break `/Game/Blueprint/Struct_Coords` _absolutecoords) _output_get))
    (if _inbounds
      (bind _index (`/Game/Blueprint/BP_CoordsFunctionLibrary.GetBlockIndex` (`local.AbsoluteX`) (`local.AbsoluteY`)))
      (bind _value (`BlueprintMapLibrary.Map_Find` (`self.Battlefield`) _index))
      ;[1 1 1] If there is already an Unit on the block, it should be out of the MoveRange.
      (`/Engine/EditorBlueprintResources/StandardMacros.IsValid` (`/Game/Blueprint/BP_Block.BindedUnit` _value)
        (:`Is Not Valid`
          (`SceneComponent.SetVisibility` (`/Game/Blueprint/BP_Block.ActionRangePlane` _value) true false)))))
  (set `self.CurrPhase` "NewEnumerator1"))

(fn `UserConstructionScript`
  (bind _history_turnsactions (break `/Game/Blueprint/Struct_GameHistory` (`self.History`)))
  (`KismetArrayLibrary.Array_Resize` _history_turnsactions (`self.MaxTurns`)))