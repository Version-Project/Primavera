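; Player state for a turn-based grid tactics game, handling turn announcements and the selected unit's move range.
; BeginPlay caches the UI manager and game state, then shows turn and faction messages timed to their widget animations.
; DefineUnitToAct stores the unit and enables the actions menu.
; ShowMoveRange turns its relative offsets into in-bounds Battlefield blocks, reveals their range planes and changes phase, while HideMoveRange clears every plane.
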(event `self.ReceiveBeginPlay`
  (bind _uimanager (`self.UIManager`))
  (bind _factionturnmessage (`/Game/Blueprint/BP_UIManager.FactionTurnMessage` (`self.UIManager`)))
  (bind _returnvalue (`GameplayStatics.GetActorOfClass` "/Game/Blueprint/BP_UIManager.BP_UIManager_C"))
  (set `self.UIManager` _returnvalue)
  (bind _asbp_game_state (cast `/Game/Blueprint/Core/BP_GameState` (`GameplayStatics.GetGameState`)))
  (set `self.GameState` _asbp_game_state)
  (`|ExecutionSequence`
    (:`then_0`
      (`/Game/Blueprint/BP_UIManager.ShowActionsMenu` (`self.UIManager`) false))
    (:`then_1`
      (`self.StartTurn`))
    (:`then_2`
      (`KismetSystemLibrary.Delay` (- (`WidgetAnimation.GetEndTime` (`/Game/UserInterface/UI_InfoMessage.Appear` (`/Game/Blueprint/BP_UIManager.InfoMessage` _uimanager))) 1.25))
      (`/Game/Blueprint/BP_UIManager.ShowFactionTurnMessage` _uimanager (`/Game/Blueprint/Core/BP_GameState.CurrFaction` (`self.GameState`)))
      (`KismetSystemLibrary.Delay` (`WidgetAnimation.GetEndTime` (`/Game/UserInterface/UI_FactionTurnMessage.Appear` _factionturnmessage)))
      (`Widget.RemoveFromParent` _factionturnmessage))))

(event `StartTurn`
  (bind _uimanager (`self.UIManager`))
  (bind _gamestate (`self.GameState`))
  (bind _infomessage (`/Game/Blueprint/BP_UIManager.InfoMessage` _uimanager))
  ;[1 1 1] Event called each time a new turn starts.
  (`/Game/Blueprint/BP_UIManager.ShowInfoMessage` _uimanager (`KismetStringLibrary.Concat_StrStr` "TURN " (`KismetStringLibrary.Conv_IntToString` (`/Game/Blueprint/Core/BP_GameState.CurrTurn` _gamestate)) " / " (`KismetStringLibrary.Conv_IntToString` (`/Game/Blueprint/Core/BP_GameState.MaxTurns` _gamestate))))
  (`KismetSystemLibrary.Delay` (`WidgetAnimation.GetEndTime` (`/Game/UserInterface/UI_InfoMessage.Appear` _infomessage)))
  (`Widget.RemoveFromParent` _infomessage))

(fn `DefineUnitToAct`
  (params (UnitToAct :type "/Game/Blueprint/Units/BP_Unit Object Reference"))
  (set `self.UnitToAct` UnitToAct)
  (`/Game/UserInterface/UI_ActionsMenu.SetIsMenuEnabled` (`/Game/Blueprint/BP_UIManager.ActionsMenu` (`self.UIManager`)) true))

(fn `HideMoveRange`
  (bind _asbp_game_state (cast `/Game/Blueprint/Core/BP_GameState` (`GameplayStatics.GetGameState`)))
  (for _index (range 176)
    (`SceneComponent.SetVisibility` (`/Game/Blueprint/BP_Block.ActionRangePlane` (`BlueprintMapLibrary.Map_Find` (`/Game/Blueprint/Core/BP_GameState.Battlefield` _asbp_game_state) _index)) false false)))

(fn `ShowMoveRange`
  (locals (Diff :type Integer) (ReportedIndex :type Integer) (IsOnFirstRow :type Boolean) (IsOnLastRow :type Boolean) (CurrBlockCoords :type "/Game/Blueprint/Struct_Coords Structure"))
  (bind _unittoact (`self.UnitToAct`))
  (bind _coords (`/Game/Blueprint/BP_CoordsFunctionLibrary.GetStructCoordsFromIndex` (`/Game/Blueprint/BP_Block.Index` (`/Game/Blueprint/Units/BP_Unit.BindedBlock` _unittoact))))
  (set `local.CurrBlockCoords` _coords)
  (for _array_element (`/Game/Blueprint/Units/BP_Unit.MoveRange` _unittoact)
    (bind _absolutecoords (`/Game/Blueprint/BP_CoordsFunctionLibrary.GetAbsoluteCoordsFromRelatives` (`local.CurrBlockCoords`) _array_element))
    (bind _inbounds (`/Game/Blueprint/BP_CoordsFunctionLibrary.CheckIfCoordsAreInBounds` (break `/Game/Blueprint/Struct_Coords` _absolutecoords) (`.Y_6_2DC6362D4EE28ABEA56491A3230A1BE6` (break `/Game/Blueprint/Struct_Coords` _absolutecoords))))
    (if _inbounds
      (bind _asbp_game_state (cast `/Game/Blueprint/Core/BP_GameState` (`GameplayStatics.GetGameState`)))
      (bind _index (`/Game/Blueprint/BP_CoordsFunctionLibrary.GetBlockIndex` (break `/Game/Blueprint/Struct_Coords` _absolutecoords) (`.Y_6_2DC6362D4EE28ABEA56491A3230A1BE6` (break `/Game/Blueprint/Struct_Coords` _absolutecoords))))
      (`SceneComponent.SetVisibility` (`/Game/Blueprint/BP_Block.ActionRangePlane` (`BlueprintMapLibrary.Map_Find` (`/Game/Blueprint/Core/BP_GameState.Battlefield` _asbp_game_state) _index)) true false)))
  (set `self.CurrentPhase` "NewEnumerator1"))

(fn `UserConstructionScript`)