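; AI behaviour for a unit in a block-based tactics game, choosing its move, attack, buff or capacity actions for a turn.
; BehaviourKind selects one of six priority chains of goals, falling back to self-buff or doing nothing.
; Goals compare precomputed best attack and capacity impacts, pick randomly among the winner's ties and prepend a move if needed; buffing rolls a chance.
; StayCloseFromAllies and MoveTowardsEnemy are stubs that always fail.
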(fn `Buff?`
  (params (ChancePercentage :type "Float (double-precision)"))
  (returns (bCanExecuteAction :type Boolean))
  (bind _array (`|MakeArray` (struct) :!type "/Game/AI/S_ActionImpact Structure"))
  (bind _array_2 (`|MakeArray` 0))
  (if (`/Game/Units/BP_Unit.bBuffed` (`self.Unit`))
    (return false)
    (elif (<= (`KismetMathLibrary.RandomFloat`) (`local.ChancePercentage`))
      (bind _bcanexecuteaction (`self.GetBestActionForSpecificGoal` _array _array_2 _array _array_2 "NewEnumerator6"))
      (return _bcanexecuteaction)
      (else
        (return false)))))

(fn `CreateAlliedObstacle?`
  (returns (bCanExecuteAction :type Boolean))
  (bind (_allattackimpacts_actionsimpacts _allattackimpacts_mostalliedblocksidx _allattackimpacts_mostenemyblocksidx _allattackimpacts_mostneutralblocksidx _allattackimpacts_mostalliedobstaclescreatedidx) (break `/Game/AI/S_AllActionsImpacts` (`self.AllAttackImpacts`)))
  (bind (_allcapacityimpacts_actionsimpacts _allcapacityimpacts_mostalliedblocksidx _allcapacityimpacts_mostenemyblocksidx _allcapacityimpacts_mostneutralblocksidx _allcapacityimpacts_mostalliedobstaclescreatedidx) (break `/Game/AI/S_AllActionsImpacts` (`self.AllCapacityImpacts`)))
  (`/Game/AI/BP_AIFunctionLibrary.PrintAIMessage` "Try to create an obstacle")
  (bind _bcanexecuteaction (`self.GetBestActionForSpecificGoal` _allattackimpacts_actionsimpacts _allattackimpacts_mostalliedobstaclescreatedidx _allcapacityimpacts_actionsimpacts _allcapacityimpacts_mostalliedobstaclescreatedidx "NewEnumerator3"))
  (return _bcanexecuteaction))

(fn `Find Action to Execute`
  (params (AttackImpacts :type "/Game/AI/S_AllActionsImpacts Structure") (CapacityImpacts :type "/Game/AI/S_AllActionsImpacts Structure"))
  (returns (ActionImpact :type "/Game/AI/S_ActionImpact Structure") (FirstAction :type "/Game/AI/S_AIAction Structure") (SecondAction :type "/Game/AI/S_AIAction Structure"))
  (set `self.AllAttackImpacts` AttackImpacts)
  (set `self.AllCapacityImpacts` CapacityImpacts)
  (`|ExecutionSequence`
    (:`then_0`
      (switch `/Game/AI/E_BehaviourKind` (`self.BehaviourKind`)
        (:`NewEnumerator0`
          ;[1 1 1] Blocker behaviour tree.
          (bind _bcanexecuteaction (`self.ObstructEnemyMoves?`))
          (if (not _bcanexecuteaction)
            (bind _bcanexecuteaction_2 (`self.CreateAlliedObstacle?`))
            (if (not _bcanexecuteaction_2)
              (bind _bcanexecuteaction_3 (`self.StayCloseFromAllies?`))
              (if (not _bcanexecuteaction_3)
                (bind _bcanexecuteaction_4 (`self.UpgradeAlliedBlocks?`))
                (if (not _bcanexecuteaction_4)
                  (bind _bcanexecuteaction_5 (`self.Buff?` 0.65))
                  (if (not _bcanexecuteaction_5)
                    (bind _bcanexecuteaction_6 (`self.FreeAllyFromEnemyObstacle?`))
                    (if (not _bcanexecuteaction_6)
                      (bind _bcanexecuteaction_7 (`self.TakeNeutralBlocks?`))
                      (if (not _bcanexecuteaction_7)
                        (bind _bcanexecuteaction_8 (`self.TakeEnemyBlocks?`))
                        (if (not _bcanexecuteaction_8)
                          (bind _bcanexecuteaction_9 (`self.MoveTowardsEnemy?`))
                          (if (not _bcanexecuteaction_9)
                            (if (`/Game/Units/BP_Unit.bBuffed` (`self.Unit`)) :!label _label
                              (return (struct) (make `/Game/AI/S_AIAction` false false false false true))
                              (else
                                (return (struct) (make `/Game/AI/S_AIAction` false false true))))))))))))))
        (:`NewEnumerator1`
          ;[1 1 1] Defender behaviour tree.
          (bind _bcanexecuteaction_10 (`self.StayCloseFromAllies?`))
          (if (not _bcanexecuteaction_10)
            (bind _bcanexecuteaction_11 (`self.CreateAlliedObstacle?`))
            (if (not _bcanexecuteaction_11)
              (bind _bcanexecuteaction_12 (`self.UpgradeAlliedBlocks?`))
              (if (not _bcanexecuteaction_12)
                (bind _bcanexecuteaction_13 (`self.FreeAllyFromEnemyObstacle?`))
                (if (not _bcanexecuteaction_13)
                  (bind _bcanexecuteaction_14 (`self.ObstructEnemyMoves?`))
                  (if (not _bcanexecuteaction_14)
                    (bind _bcanexecuteaction_15 (`self.Buff?` 0.75))
                    (if (not _bcanexecuteaction_15)
                      (bind _bcanexecuteaction_16 (`self.MoveTowardsEnemy?`))
                      (if (not _bcanexecuteaction_16)
                        (bind _bcanexecuteaction_17 (`self.TakeNeutralBlocks?`))
                        (if (not _bcanexecuteaction_17)
                          (bind _bcanexecuteaction_18 (`self.TakeEnemyBlocks?`))
                          (if (not _bcanexecuteaction_18)
                            (goto _label)))))))))))
        (:`NewEnumerator2`
          ;[1 1 1] Upgrader behaviour tree.
          (bind _bcanexecuteaction_19 (`self.Buff?` 0.5))
          (if (not _bcanexecuteaction_19)
            (bind _bcanexecuteaction_20 (`self.UpgradeAlliedBlocks?`))
            (if (not _bcanexecuteaction_20)
              (bind _bcanexecuteaction_21 (`self.CreateAlliedObstacle?`))
              (if (not _bcanexecuteaction_21)
                (bind _bcanexecuteaction_22 (`self.TakeNeutralBlocks?`))
                (if (not _bcanexecuteaction_22)
                  (bind _bcanexecuteaction_23 (`self.StayCloseFromAllies?`))
                  (if (not _bcanexecuteaction_23)
                    (bind _bcanexecuteaction_24 (`self.FreeAllyFromEnemyObstacle?`))
                    (if (not _bcanexecuteaction_24)
                      (bind _bcanexecuteaction_25 (`self.ObstructEnemyMoves?`))
                      (if (not _bcanexecuteaction_25)
                        (bind _bcanexecuteaction_26 (`self.TakeEnemyBlocks?`))
                        (if (not _bcanexecuteaction_26)
                          (bind _bcanexecuteaction_27 (`self.MoveTowardsEnemy?`))
                          (if (not _bcanexecuteaction_27)
                            (goto _label)))))))))))
        (:`NewEnumerator3`
          ;[1 1 1] Explorer behaviour tree.
          (bind _bcanexecuteaction_28 (`self.TakeNeutralBlocks?`))
          (if (not _bcanexecuteaction_28)
            (bind _bcanexecuteaction_29 (`self.TakeEnemyBlocks?`))
            (if (not _bcanexecuteaction_29)
              (bind _bcanexecuteaction_30 (`self.MoveTowardsEnemy?`))
              (if (not _bcanexecuteaction_30)
                (bind _bcanexecuteaction_31 (`self.Buff?` 0.5))
                (if (not _bcanexecuteaction_31)
                  (bind _bcanexecuteaction_32 (`self.ObstructEnemyMoves?`))
                  (if (not _bcanexecuteaction_32)
                    (bind _bcanexecuteaction_33 (`self.UpgradeAlliedBlocks?`))
                    (if (not _bcanexecuteaction_33)
                      (bind _bcanexecuteaction_34 (`self.CreateAlliedObstacle?`))
                      (if (not _bcanexecuteaction_34)
                        (bind _bcanexecuteaction_35 (`self.FreeAllyFromEnemyObstacle?`))
                        (if (not _bcanexecuteaction_35)
                          (bind _bcanexecuteaction_36 (`self.StayCloseFromAllies?`))
                          (if (not _bcanexecuteaction_36)
                            (goto _label)))))))))))
        (:`NewEnumerator4`
          ;[1 1 1] Conqueror behaviour tree.
          (bind _bcanexecuteaction_37 (`self.FreeAllyFromEnemyObstacle?`))
          (if (not _bcanexecuteaction_37)
            (bind _bcanexecuteaction_38 (`self.TakeEnemyBlocks?`))
            (if (not _bcanexecuteaction_38)
              (bind _bcanexecuteaction_39 (`self.TakeNeutralBlocks?`))
              (if (not _bcanexecuteaction_39)
                (bind _bcanexecuteaction_40 (`self.MoveTowardsEnemy?`))
                (if (not _bcanexecuteaction_40)
                  (bind _bcanexecuteaction_41 (`self.Buff?` 0.75))
                  (if (not _bcanexecuteaction_41)
                    (bind _bcanexecuteaction_42 (`self.ObstructEnemyMoves?`))
                    (if (not _bcanexecuteaction_42)
                      (bind _bcanexecuteaction_43 (`self.CreateAlliedObstacle?`))
                      (if (not _bcanexecuteaction_43)
                        (bind _bcanexecuteaction_44 (`self.UpgradeAlliedBlocks?`))
                        (if (not _bcanexecuteaction_44)
                          (bind _bcanexecuteaction_45 (`self.StayCloseFromAllies?`))
                          (if (not _bcanexecuteaction_45)
                            (goto _label)))))))))))
        (:`NewEnumerator5`
          ;[1 1 1] Neutralizer behaviour tree.
          (bind _bcanexecuteaction_46 (`self.ObstructEnemyMoves?`))
          (if (not _bcanexecuteaction_46)
            (bind _bcanexecuteaction_47 (`self.CreateAlliedObstacle?`))
            (if (not _bcanexecuteaction_47)
              (bind _bcanexecuteaction_48 (`self.MoveTowardsEnemy?`))
              (if (not _bcanexecuteaction_48)
                (bind _bcanexecuteaction_49 (`self.TakeEnemyBlocks?`))
                (if (not _bcanexecuteaction_49)
                  (bind _bcanexecuteaction_50 (`self.FreeAllyFromEnemyObstacle?`))
                  (if (not _bcanexecuteaction_50)
                    (bind _bcanexecuteaction_51 (`self.UpgradeAlliedBlocks?`))
                    (if (not _bcanexecuteaction_51)
                      (bind _bcanexecuteaction_52 (`self.TakeNeutralBlocks?`))
                      (if (not _bcanexecuteaction_52)
                        (bind _bcanexecuteaction_53 (`self.StayCloseFromAllies?`))
                        (if (not _bcanexecuteaction_53)
                          (bind _bcanexecuteaction_54 (`self.Buff?` 1.0))
                          (if (not _bcanexecuteaction_54)
                            (goto _label)))))))))))))
    (:`then_1`
      (return (`self.ChosenAction`) (`self.FirstAction`) (`self.SecondAction`)))))

(fn `FreeAllyFromEnemyObstacle?`
  (returns (bCanExecuteAction :type Boolean))
  (bind (_allattackimpacts_actionsimpacts _allattackimpacts_mostalliedblocksidx _allattackimpacts_mostenemyblocksidx _allattackimpacts_mostneutralblocksidx _allattackimpacts_mostalliedobstaclescreatedidx _allattackimpacts_mostalliesonenemyobstaclesidx) (break `/Game/AI/S_AllActionsImpacts` (`self.AllAttackImpacts`)))
  (bind (_allcapacityimpacts_actionsimpacts _allcapacityimpacts_mostalliedblocksidx _allcapacityimpacts_mostenemyblocksidx _allcapacityimpacts_mostneutralblocksidx _allcapacityimpacts_mostalliedobstaclescreatedidx _allcapacityimpacts_mostalliesonenemyobstaclesidx) (break `/Game/AI/S_AllActionsImpacts` (`self.AllCapacityImpacts`)))
  (`/Game/AI/BP_AIFunctionLibrary.PrintAIMessage` "Try to free an ally from an enemy obstacle")
  (bind _bcanexecuteaction (`self.GetBestActionForSpecificGoal` _allattackimpacts_actionsimpacts _allattackimpacts_mostalliesonenemyobstaclesidx _allcapacityimpacts_actionsimpacts _allcapacityimpacts_mostalliesonenemyobstaclesidx "NewEnumerator4"))
  (return _bcanexecuteaction))

(fn `GetBestActionForSpecificGoal`
  (params (CurrAttackImpacts :type "Array of /Game/AI/S_ActionImpact Structure") (BestAttackIdxToCheck :type "Array of Integer") (CurrCapacityImpacts :type "Array of /Game/AI/S_ActionImpact Structure") (BestCapacityIdxToCheck :type "Array of Integer") (Goal :type "/Game/AI/E_AIGoal Enum" :default "NewEnumerator0"))
  (returns (bCanExecuteAction :type Boolean))
  (bind _goal (`local.Goal`))
  (if (`|EnumEquality` "NewEnumerator6" Goal)
    (set `self.FirstAction` (make `/Game/AI/S_AIAction` false false true false))
    (set `self.SecondAction` (struct))
    (return true)
    (else
      (if (`KismetArrayLibrary.Array_IsEmpty` (`local.BestAttackIdxToCheck`))
        (if (or (`KismetArrayLibrary.Array_IsEmpty` (`local.BestCapacityIdxToCheck`)) (not (`self.bCanUseCapacity`)))
          (return false)
          (else
            _))
        (elif (or (`KismetArrayLibrary.Array_IsEmpty` (`local.BestCapacityIdxToCheck`)) (not (`self.bCanUseCapacity`)))
          ;[1 1 1] Get an action from the best - Attack
          (bind (_bactionavailable _chosenaction) (`self.GetRandomActionFromBest` (`local.CurrAttackImpacts`) (`local.BestAttackIdxToCheck`) :!label _label))
          (bind _output_get (set `self.ChosenAction` _chosenaction))
          (if (== (break `/Game/AI/S_ActionImpact` _output_get) (`/Game/Units/BP_Unit.BindedBlock` (`self.Unit`)))
            (set `self.FirstAction` (make `/Game/AI/S_AIAction` false true))
            (set `self.SecondAction` (struct))
            (return true)
            (else
              (set `self.FirstAction` (make `/Game/AI/S_AIAction` true))
              (set `self.SecondAction` (make `/Game/AI/S_AIAction` false true))
              (return true)))
          (else
            (bind _value (`self.GetGoalValueFromActionImpact` (`|GetArrayItem` (`local.CurrCapacityImpacts`) (`|GetArrayItem` (`local.BestCapacityIdxToCheck`))) _goal))
            (bind _value_2 (`self.GetGoalValueFromActionImpact` (`|GetArrayItem` (`local.CurrAttackImpacts`) (`|GetArrayItem` (`local.BestAttackIdxToCheck`))) _goal))
            (if (>= _value_2 _value)
              (goto _label)
              (else
                _)))))
      ;[1 1 1] Get an action from the best - Capacity
      (bind (_bactionavailable_2 _chosenaction_2) (`self.GetRandomActionFromBest` (`local.CurrCapacityImpacts`) (`local.BestCapacityIdxToCheck`)))
      (bind _output_get_2 (set `self.ChosenAction` _chosenaction_2))
      (if (== (break `/Game/AI/S_ActionImpact` _output_get_2) (`/Game/Units/BP_Unit.BindedBlock` (`self.Unit`)))
        (set `self.FirstAction` (make `/Game/AI/S_AIAction` false false false true))
        (set `self.SecondAction` (struct))
        (return true)
        (else
          (set `self.FirstAction` (make `/Game/AI/S_AIAction` true))
          (set `self.SecondAction` (make `/Game/AI/S_AIAction` false false false true))
          (return true))))))

(fn `GetGoalValueFromActionImpact`
  (params (ActionImpact :type "/Game/AI/S_ActionImpact Structure") (Goal :type "/Game/AI/E_AIGoal Enum" :default "NewEnumerator0"))
  (returns (Value :type Integer))
  (switch `/Game/AI/E_AIGoal` Goal
    (:`NewEnumerator0`
      (return ActionImpact_NbAlliedBlocksHit_18_1D29E06146940FBFFC930AB440FB9786))
    (:`NewEnumerator1`
      (return ActionImpact_NbEnemyBlocksHit_19_18810DDB42BF6124134C7D88CFE662A0))
    (:`NewEnumerator2`
      (return ActionImpact_NbNeutralBlocksHit_21_18E4838C47369BB2144D1FBC5BAC4CB6))
    (:`NewEnumerator3`
      (return ActionImpact_NbAlliedObstaclesCreated_27_526F5A2240FC5D890C4112968A71D354))
    (:`NewEnumerator4`
      (return ActionImpact_NbAlliesOnEnemyObstacles_31_C9EECE1749439389D6DB9F93E6338122))
    (:`NewEnumerator5`
      (return ActionImpact_NbEnemiesOnFutureAlliedObstacles_35_279DB32F45BE410E74213CBB3BBE3322))))

(fn `GetRandomActionFromBest`
  (params (ActionsImpacts :type "Array of /Game/AI/S_ActionImpact Structure") (BestIdx :type "Array of Integer"))
  (returns (bActionAvailable :type Boolean) (ChosenAction :type "/Game/AI/S_ActionImpact Structure"))
  (bind _bestidx (`local.BestIdx`))
  (if (`KismetArrayLibrary.Array_IsEmpty` BestIdx)
    (return false)
    (else
      (return true (`|GetArrayItem` (`local.ActionsImpacts`) (`|GetArrayItem` _bestidx (`KismetMathLibrary.RandomInteger` (`KismetArrayLibrary.Array_Length` _bestidx))))))))

(fn `MoveTowardsEnemy?`
  (returns (bCanExecuteAction :type Boolean))
  (`/Game/AI/BP_AIFunctionLibrary.PrintAIMessage` "Try to move towards an enemy")
  (return false))

(fn `ObstructEnemyMoves?`
  (returns (bCanExecuteAction :type Boolean))
  (bind (_allattackimpacts_actionsimpacts _allattackimpacts_mostalliedblocksidx _allattackimpacts_mostenemyblocksidx _allattackimpacts_mostneutralblocksidx _allattackimpacts_mostalliedobstaclescreatedidx _allattackimpacts_mostalliesonenemyobstaclesidx _allattackimpacts_mostenemiesonfuturealliedobstaclesidx) (break `/Game/AI/S_AllActionsImpacts` (`self.AllAttackImpacts`)))
  (bind (_allcapacityimpacts_actionsimpacts _allcapacityimpacts_mostalliedblocksidx _allcapacityimpacts_mostenemyblocksidx _allcapacityimpacts_mostneutralblocksidx _allcapacityimpacts_mostalliedobstaclescreatedidx _allcapacityimpacts_mostalliesonenemyobstaclesidx _allcapacityimpacts_mostenemiesonfuturealliedobstaclesidx) (break `/Game/AI/S_AllActionsImpacts` (`self.AllCapacityImpacts`)))
  (`/Game/AI/BP_AIFunctionLibrary.PrintAIMessage` "Try to obstruct enemy moves")
  (bind _bcanexecuteaction (`self.GetBestActionForSpecificGoal` _allattackimpacts_actionsimpacts _allattackimpacts_mostenemiesonfuturealliedobstaclesidx _allcapacityimpacts_actionsimpacts _allcapacityimpacts_mostenemiesonfuturealliedobstaclesidx "NewEnumerator5"))
  (return _bcanexecuteaction))

(fn `StayCloseFromAllies?`
  (returns (bCanExecuteAction :type Boolean))
  (`/Game/AI/BP_AIFunctionLibrary.PrintAIMessage` "Try to stay close from your allies")
  (return false))

(fn `TakeEnemyBlocks?`
  (returns (bCanExecuteAction :type Boolean))
  (locals (CanExecute :type Boolean))
  (bind (_allattackimpacts_actionsimpacts _allattackimpacts_mostalliedblocksidx _allattackimpacts_mostenemyblocksidx) (break `/Game/AI/S_AllActionsImpacts` (`self.AllAttackImpacts`)))
  (bind (_allcapacityimpacts_actionsimpacts _allcapacityimpacts_mostalliedblocksidx _allcapacityimpacts_mostenemyblocksidx) (break `/Game/AI/S_AllActionsImpacts` (`self.AllCapacityImpacts`)))
  (`/Game/AI/BP_AIFunctionLibrary.PrintAIMessage` "Try to take ennemy Blocks")
  (bind _bcanexecuteaction (`self.GetBestActionForSpecificGoal` _allattackimpacts_actionsimpacts _allattackimpacts_mostenemyblocksidx _allcapacityimpacts_actionsimpacts _allcapacityimpacts_mostenemyblocksidx "NewEnumerator1"))
  (return _bcanexecuteaction))

(fn `TakeNeutralBlocks?`
  (returns (bCanExecuteAction :type Boolean))
  (locals (CanExecute :type Boolean :default true))
  (bind (_allattackimpacts_actionsimpacts _allattackimpacts_mostalliedblocksidx _allattackimpacts_mostenemyblocksidx _allattackimpacts_mostneutralblocksidx) (break `/Game/AI/S_AllActionsImpacts` (`self.AllAttackImpacts`)))
  (bind (_allcapacityimpacts_actionsimpacts _allcapacityimpacts_mostalliedblocksidx _allcapacityimpacts_mostenemyblocksidx _allcapacityimpacts_mostneutralblocksidx) (break `/Game/AI/S_AllActionsImpacts` (`self.AllCapacityImpacts`)))
  (`/Game/AI/BP_AIFunctionLibrary.PrintAIMessage` "Try to take neutral Blocks")
  (bind _bcanexecuteaction (`self.GetBestActionForSpecificGoal` _allattackimpacts_actionsimpacts _allattackimpacts_mostneutralblocksidx _allcapacityimpacts_actionsimpacts _allcapacityimpacts_mostneutralblocksidx "NewEnumerator2"))
  (return _bcanexecuteaction))

(fn `UpgradeAlliedBlocks?`
  (returns (bCanExecuteAction :type Boolean))
  (bind (_allattackimpacts_actionsimpacts _allattackimpacts_mostalliedblocksidx) (break `/Game/AI/S_AllActionsImpacts` (`self.AllAttackImpacts`)))
  (bind (_allcapacityimpacts_actionsimpacts _allcapacityimpacts_mostalliedblocksidx) (break `/Game/AI/S_AllActionsImpacts` (`self.AllCapacityImpacts`)))
  (`/Game/AI/BP_AIFunctionLibrary.PrintAIMessage` "Try to upgrade some allied Blocks")
  (bind _bcanexecuteaction (`self.GetBestActionForSpecificGoal` _allattackimpacts_actionsimpacts _allattackimpacts_mostalliedblocksidx _allcapacityimpacts_actionsimpacts _allcapacityimpacts_mostalliedblocksidx))
  (return _bcanexecuteaction))