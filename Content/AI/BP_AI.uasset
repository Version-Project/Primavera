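; AI opponent for a turn-based grid battle, playing the Winter faction's units through BP_GS_Battle.
; PlayUnitTurn waits out turn messages, randomly picks Sniper or Inlayer (RandomInteger(2) never reaches Protector), then calls ChooseAction twice with delays.
; ChooseAction moves the unit left or, once moved, scores attacks from reachable blocks by ally, enemy and neutral blocks hit.
; Work in progress: scores go unused, ExecuteAttack is never reached and Behaviour_TakeEnemyBlock is empty.
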(event `self.ReceiveBeginPlay`
  (`KismetSystemLibrary.PrintString` "AI: \"I'm ready to fight!\"" true true (struct :`R` 1.0 :`G` 0.226966 :`A` 1.0) 4.0)
  (bind _asbp_gs_battle (cast `/Game/Core/GameMode/BattleScene/BP_GS_Battle` (`GameplayStatics.GetGameState`)))
  (bind _output_get (set `self.GameState` _asbp_gs_battle))
  (for _array_element (`/Game/Core/GameMode/BattleScene/BP_GS_Battle.WinterUnits` _output_get)
    (`BlueprintMapLibrary.Map_Add` (`self.WinterUnits`) (`|GetEnumeratorNameAsString` (`/Game/Units/BP_Unit.Class` _array_element)) _array_element)))

(event `PlayUnitTurn`
  (params (bStartingNewPlayingTurn :type Boolean))
  (bind _waitingtime (`self.GetWaitingTimeWhenNewTurnStarts` bStartingNewPlayingTurn))
  (`KismetSystemLibrary.Delay` _waitingtime)
  (`self.ChooseUnitToAct`)
  (`KismetSystemLibrary.Delay` (`self.WaitingTime`))
  (bind _waitingtimebeforenextaction (`self.ChooseAction`))
  (`KismetSystemLibrary.Delay` _waitingtimebeforenextaction)
  (bind _waitingtimebeforenextaction_2 (`self.ChooseAction`))
  (`KismetSystemLibrary.Delay` _waitingtimebeforenextaction_2))

(event `ExecuteMove`
  (params (DestBlock :type "/Game/Battlefield/Block/BP_Block Object Reference") (NbPossibleMoves :type Integer))
  (bind _gamestate (`self.GameState`))
  ;[1 1 1] Display the MoveRange, display the ConfirmArrow at the destination then move the chosen Unit.
  (`KismetSystemLibrary.PrintString` (`KismetStringLibrary.Concat_StrStr` "AI: \"" (`|GetEnumeratorNameAsString` (`/Game/Units/BP_Unit.Class` (`self.ChosenUnit`))) ", move!\"") true true (struct :`R` 1.0 :`G` 0.226966 :`A` 1.0) 4.0)
  (set `/Game/Core/GameMode/BattleScene/BP_GS_Battle.CurrPhase` "NewEnumerator1" (`self.GameState`))
  (`/Game/Core/GameMode/BattleScene/BP_GS_Battle.HideActionRange` _gamestate true)
  (`/Game/Core/GameMode/BattleScene/BP_GS_Battle.DetermineMoveRange` _gamestate (`/Game/Battlefield/Block/BP_Block.Coords` (`/Game/Units/BP_Unit.BindedBlock` (`self.ChosenUnit`))) "NewEnumerator1" NbPossibleMoves)
  (`/Game/Core/GameMode/BattleScene/BP_GS_Battle.ShowActionRange` (`self.GameState`))
  (`KismetSystemLibrary.Delay` (`self.WaitingTime`))
  (`/Game/Core/GameMode/BattleScene/BP_GS_Battle.ShowArrow` (`self.GameState`) "NewEnumerator0" DestBlock)
  (`KismetSystemLibrary.Delay` (`self.WaitingTime`))
  (`/Game/Units/BP_Unit.Move` (`self.ChosenUnit`) DestBlock 0)
  (`/Game/Core/GameMode/BattleScene/BP_GS_Battle.ResetUIElements` (`self.GameState`)))

(event `ExecuteAttack`
  (params (Direction :type "/Game/Core/E_Direction Enum" :default "NewEnumerator0"))
  (bind _gamestate (`self.GameState`))
  ;[1 1 1] Display the directional arrows, display the AttackRange in the correct direction then make the Unit attack.
  (`KismetSystemLibrary.PrintString` (`KismetStringLibrary.Concat_StrStr` "AI: \"" (`|GetEnumeratorNameAsString` (`/Game/Units/BP_Unit.Class` (`self.ChosenUnit`))) ", attack!\"") true true (struct :`R` 1.0 :`G` 0.226966 :`A` 1.0) 4.0)
  (set `/Game/Core/GameMode/BattleScene/BP_GS_Battle.CurrPhase` "NewEnumerator2" (`self.GameState`))
  (`/Game/Core/GameMode/BattleScene/BP_GS_Battle.ShowDirectionalArrows` (`self.GameState`))
  (`KismetSystemLibrary.Delay` (`self.WaitingTime`))
  (`/Game/Core/GameMode/BattleScene/BP_GS_Battle.HideActionRange` _gamestate true)
  (`/Game/Core/GameMode/BattleScene/BP_GS_Battle.DetermineAttackRange` _gamestate Direction null)
  (`/Game/Core/GameMode/BattleScene/BP_GS_Battle.ShowActionRange` (`self.GameState`))
  (bind _output_get (set `/Game/Units/BP_Unit.CurrActionDirection` Direction (`self.ChosenUnit`)))
  (bind _enumvalue (foreach `/Game/Core/E_Direction` false)
    (:`LoopBody`
      (if (`|EnumInequality` _output_get _enumvalue)
        (`/Game/UserInterface/Arrow/BP_Arrow.Undisplay` (`BlueprintMapLibrary.Map_Find` (`/Game/Core/GameMode/BattleScene/BP_GS_Battle.Arrows` (`self.GameState`)) _enumvalue))))
    (:`then`
      (`KismetSystemLibrary.Delay` (`self.WaitingTime`))
      (`/Game/Units/BP_Unit.Attack` (`self.ChosenUnit`))
      (`/Game/Core/GameMode/BattleScene/BP_GS_Battle.ResetUIElements` (`self.GameState`)))))

(fn `Behaviour_TakeEnemyBlock`)

(fn `ChooseAction`
  (returns (WaitingTimeBeforeNextAction :type "Float (double-precision)"))
  (locals (NbPossibleMoves :type Integer :default 3))
  (bind _chosenunit (`self.ChosenUnit`))
  (bind (_history_turnsactions _history_currturnidx) (break `/Game/Core/S_GameHistory` (`/Game/Core/GameMode/BattleScene/BP_GS_Battle.History` (`self.GameState`))))
  (bind (_output_unitsactions _output_currentunitidx) (break `/Game/Core/S_TurnActionsHistory` (`|GetArrayItem` _history_turnsactions _history_currturnidx)))
  (bind (_output_unit _output_bmoved) (break `/Game/Core/S_UnitActions` (`|GetArrayItem` _output_unitsactions _output_currentunitidx)))
  (if _output_bmoved
    (`self.DetermineAttackImpacts` (`self.ChosenUnit`))
    (else
      ;[1 1 1] If Move is chosen.
      (if (`/Game/Units/BP_Unit.bStuck` _chosenunit)
        (set `local.NbPossibleMoves` 1)
        (else
          (set `local.NbPossibleMoves` 3)))
      (bind _finishblock (`/Game/Core/GameMode/BattleScene/BP_GS_Battle.GetAdjacentBlock` (`self.GameState`) (`/Game/Units/BP_Unit.BindedBlock` _chosenunit) "NewEnumerator3"))
      (`self.ExecuteMove` _finishblock (`local.NbPossibleMoves`))
      (return (* (`self.WaitingTime`) 3)))))

(fn `ChooseUnitToAct`
  ;[1 1 1] Random selection of an Unit to act.
  (switch `int` (`KismetMathLibrary.RandomInteger` 2)
    (:`0`
      (set `self.ChosenUnit` (`BlueprintMapLibrary.Map_Find` (`self.WinterUnits`) "Sniper")))
    (:`1`
      (set `self.ChosenUnit` (`BlueprintMapLibrary.Map_Find` (`self.WinterUnits`) "Inlayer")))
    (:`2`
      (set `self.ChosenUnit` (`BlueprintMapLibrary.Map_Find` (`self.WinterUnits`) "Protector"))))
  (`/Game/Core/GameMode/BattleScene/BP_GS_Battle.DefineUnitToAct` (`self.GameState`) (`self.ChosenUnit`))
  (`KismetSystemLibrary.PrintString` "AI: \"I chose an Unit to act.\"" true true (struct :`R` 1.0 :`G` 0.226966 :`A` 1.0) 4.0))

(fn `DetermineAttackImpacts`
  (params (AttackingUnit :type "/Game/Units/BP_Unit Object Reference"))
  (locals (AttackImpacts :type "/Game/AI/S_AllAttackImpacts Structure") (MoveRange :type "Array of /Game/Battlefield/Block/BP_Block Object Reference") (Key :type String) (CurrBlock :type "/Game/Battlefield/Block/BP_Block Object Reference") (CurrDirection :type "/Game/Core/E_Direction Enum") (NbAlliedBlocks :type Integer) (NbEnemyBlocks :type Integer) (NbNeutralBlocks :type Integer) (BestAtkOnAllyIdx :type Integer) (BestAtkOnEnemyIdx :type Integer) (BestAtkOnNeutralIdx :type Integer) (CurrIdx :type Integer :default 0))
  (bind _attackimpacts_attackimpacts (break `/Game/AI/S_AllAttackImpacts` (`local.AttackImpacts`)))
  (bind _attackimpacts_attackimpacts_2 (break `/Game/AI/S_AllAttackImpacts` (`local.AttackImpacts`)))
  (bind _attackimpacts_attackimpacts_3 (break `/Game/AI/S_AllAttackImpacts` (`local.AttackImpacts`)))
  (set `local.Key` (`|GetEnumeratorNameAsString` (`/Game/Units/BP_Unit.Class` AttackingUnit)))
  (if (`/Game/Units/BP_Unit.bStuck` (`local.AttackingUnit`))
    ;[1 1 1] If Unit is stuck, it cannot attack. Therefore, we just return a single AttackImpact, with all values at zero.
    (`BlueprintMapLibrary.Map_Add` (`self.AttackImpactsByUnit`) (`local.Key`) (make `/Game/AI/S_AllAttackImpacts` (`|MakeArray` (make `/Game/AI/S_AttackImpact` (`/Game/Units/BP_Unit.BindedBlock` (`local.AttackingUnit`))) :!type "/Game/AI/S_AttackImpact Structure")))
    (return)
    (else
      (`KismetArrayLibrary.Array_Clear` _attackimpacts_attackimpacts_3)
      (`/Game/Core/GameMode/BattleScene/BP_GS_Battle.DetermineMoveRange` (`self.GameState`) (`/Game/Battlefield/Block/BP_Block.Coords` (`/Game/Units/BP_Unit.BindedBlock` (`local.AttackingUnit`))) "NewEnumerator1" 3)
      (bind _output_get (set `local.MoveRange` (`/Game/Core/GameMode/BattleScene/BP_GS_Battle.BlocksInActionRange` (`self.GameState`))))
      (`KismetArrayLibrary.Array_Add` _output_get (`/Game/Units/BP_Unit.BindedBlock` (`local.AttackingUnit`)))
      (for _array_element (`local.MoveRange`)
        (set `local.CurrBlock` _array_element)
        (bind _enumvalue (foreach `/Game/Core/E_Direction` false) ; For each direction in which Unit can attack from the current Block...
          (:`LoopBody`
            (bind _output_get_2 (set `local.CurrDirection` _enumvalue))
            (switch `/Game/Core/E_Direction` _output_get_2
              (:`NewEnumerator1`
                _)
              (:`NewEnumerator2`
                _)
              (:`NewEnumerator3`
                _)
              (:`NewEnumerator4`
                _))
            (`/Game/Core/GameMode/BattleScene/BP_GS_Battle.HideActionRange` (`self.GameState`) true)
            (`|ExecutionSequence`
              (:`then_0`
                (set `local.NbAlliedBlocks` 0))
              (:`then_1`
                (set `local.NbEnemyBlocks` 0))
              (:`then_2`
                (set `local.NbNeutralBlocks` 0))
              (:`then_3`
                (`/Game/Core/GameMode/BattleScene/BP_GS_Battle.DetermineAttackRange` (`self.GameState`) (`local.CurrDirection`) (`local.CurrBlock`))
                (for _array_element_2 (`/Game/Core/GameMode/BattleScene/BP_GS_Battle.BlocksInActionRange` (`self.GameState`))
                  (switch `/Game/Core/E_Faction` (`/Game/Battlefield/Block/BP_Block.BlockOwner` _array_element_2)
                    (:`NewEnumerator0`
                      (`/Engine/EditorBlueprintResources/StandardMacros.IncrementInt` (`local.NbNeutralBlocks`)))
                    (:`NewEnumerator1`
                      (`/Engine/EditorBlueprintResources/StandardMacros.IncrementInt` (`local.NbAlliedBlocks`)))
                    (:`NewEnumerator2`
                      (`/Engine/EditorBlueprintResources/StandardMacros.IncrementInt` (`local.NbEnemyBlocks`)))))
                (`KismetArrayLibrary.Array_Add` _attackimpacts_attackimpacts (make `/Game/AI/S_AttackImpact` (`local.CurrBlock`) (`local.CurrDirection`) (`/Game/Core/GameMode/BattleScene/BP_GS_Battle.BlocksInActionRange` (`self.GameState`)) (`local.NbAlliedBlocks`) (`local.NbEnemyBlocks`) (`local.NbNeutralBlocks`))) ; Add a new AttackImpact to the list of the AttackingUnit.
              )))))
      (`/Game/Core/GameMode/BattleScene/BP_GS_Battle.HideActionRange` (`self.GameState`) true)
      ;[1 1 1] After all AttackImpacts have been collected, find the best ones for each kind of attack.
      (`|ExecutionSequence`
        (:`then_0`
          (set `local.NbAlliedBlocks` 0))
        (:`then_1`
          (set `local.NbEnemyBlocks` 0))
        (:`then_2`
          (set `local.NbNeutralBlocks` 0))
        (:`then_3`
          (for (_array_element_3 _array_index) _attackimpacts_attackimpacts_2
            (set `local.CurrIdx` _array_index)
            (`|ExecutionSequence`
              (:`then_0`
                (if (> (`.NbAlliedBlocksHit_18_1D29E06146940FBFFC930AB440FB9786` (break `/Game/AI/S_AttackImpact` _array_element_3)) (`local.NbAlliedBlocks`))
                  (set `local.BestAtkOnAllyIdx` (`local.CurrIdx`))
                  (set `local.NbAlliedBlocks` (`.NbAlliedBlocksHit_18_1D29E06146940FBFFC930AB440FB9786` (break `/Game/AI/S_AttackImpact` _array_element_3)))))
              (:`then_1`
                (if (> (`.NbEnemyBlocksHit_19_18810DDB42BF6124134C7D88CFE662A0` (break `/Game/AI/S_AttackImpact` _array_element_3)) (`local.NbEnemyBlocks`))
                  (set `local.BestAtkOnEnemyIdx` (`local.CurrIdx`))
                  (set `local.NbEnemyBlocks` (`.NbEnemyBlocksHit_19_18810DDB42BF6124134C7D88CFE662A0` (break `/Game/AI/S_AttackImpact` _array_element_3)))))
              (:`then_2`
                (if (> (`.NbNeutralBlocksHit_21_18E4838C47369BB2144D1FBC5BAC4CB6` (break `/Game/AI/S_AttackImpact` _array_element_3)) (`local.NbNeutralBlocks`))
                  (set `local.BestAtkOnNeutralIdx` (`local.CurrIdx`))
                  (set `local.NbNeutralBlocks` (`.NbNeutralBlocksHit_21_18E4838C47369BB2144D1FBC5BAC4CB6` (break `/Game/AI/S_AttackImpact` _array_element_3)))))))
          (`BlueprintMapLibrary.Map_Add` (`self.AttackImpactsByUnit`) (`local.Key`) (make `/Game/AI/S_AllAttackImpacts` _attackimpacts_attackimpacts_2 (`local.BestAtkOnAllyIdx`) (`local.BestAtkOnEnemyIdx`) (`local.BestAtkOnNeutralIdx`)))
          (return))))))

(fn `GetWaitingTimeWhenNewTurnStarts`
  (params (bStartingNewPlayingTurn :type Boolean))
  (returns (WaitingTime :type "Float (double-precision)"))
  (bind _uimanager (`/Game/Core/GameMode/BattleScene/BP_GS_Battle.UIManager` (`self.GameState`)))
  (if bStartingNewPlayingTurn
    (return (+ (`WidgetAnimation.GetEndTime` (`/Game/UserInterface/WBP_PlayingTurnMessage.Appear` (`/Game/Core/BP_UIManager.PlayingTurnMessage` _uimanager))) 1.0 (- (`WidgetAnimation.GetEndTime` (`/Game/UserInterface/WBP_UnitTurnMessage.Appear` (`/Game/Core/BP_UIManager.UnitTurnMessage` _uimanager))) 1.25)))
    (else
      (return (+ (`WidgetAnimation.GetEndTime` (`/Game/UserInterface/WBP_UnitTurnMessage.Appear` (`/Game/Core/BP_UIManager.UnitTurnMessage` (`/Game/Core/GameMode/BattleScene/BP_GS_Battle.UIManager` (`self.GameState`))))) 1.0)))))

(fn `UserConstructionScript`)