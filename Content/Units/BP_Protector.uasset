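; BP_Protector is a grid-battle unit whose capacity reinforces nearby blocks owned by its faction.
; On BeginPlay it builds wedge-shaped attack ranges per direction, wider buffed versions, and a diamond capacity range, all as relative coordinates.
; UseCapacity raises incrustation on friendly in-bounds blocks up to a cap and rechecks stuck status of enemy units in range.
; It then clears the buff and ends the phase.
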(event `self.ReceiveBeginPlay`
  (`self.SetGameStateAndManagers`)
  (`self.DefineAttackRange`)
  (`self.DefineBuffedAttackRange`)
  (`self.DefineCapacityRange`))

(fn `DefineAttackRange`
  (bind (_attackranges_up _attackranges_down _attackranges_left _attackranges_right) (break `/Game/Core/S_AttackRange` (`self.AttackRanges`)))
  (`self.AddConsecutiveAttackCoords` -1 1 -1 -1 "NewEnumerator1" 1 _attackranges_up)
  (`self.AddConsecutiveAttackCoords` 0 0 -2 -2 "NewEnumerator1" 1 _attackranges_up)
  (`self.AddConsecutiveAttackCoords` -1 1 1 1 "NewEnumerator2" 1 _attackranges_down)
  (`self.AddConsecutiveAttackCoords` 0 0 2 2 "NewEnumerator2" 1 _attackranges_down)
  (`self.AddConsecutiveAttackCoords` -1 -1 -1 1 "NewEnumerator3" 1 _attackranges_left)
  (`self.AddConsecutiveAttackCoords` -2 -2 0 0 "NewEnumerator3" 1 _attackranges_left)
  (`self.AddConsecutiveAttackCoords` 1 1 -1 1 "NewEnumerator4" 1 _attackranges_right)
  (`self.AddConsecutiveAttackCoords` 2 2 0 0 "NewEnumerator4" 1 _attackranges_right)
  (return))

(fn `DefineBuffedAttackRange`
  (bind (_buffedattackranges_up _buffedattackranges_down _buffedattackranges_left _buffedattackranges_right) (break `/Game/Core/S_AttackRange` (`self.BuffedAttackRanges`)))
  (`self.AddConsecutiveAttackCoords` -2 2 -1 -1 "NewEnumerator1" 1 _buffedattackranges_up)
  (`self.AddConsecutiveAttackCoords` -1 1 -2 -2 "NewEnumerator1" 1 _buffedattackranges_up)
  (`self.AddConsecutiveAttackCoords` -2 2 1 1 "NewEnumerator2" 1 _buffedattackranges_down)
  (`self.AddConsecutiveAttackCoords` -1 1 2 2 "NewEnumerator2" 1 _buffedattackranges_down)
  (`self.AddConsecutiveAttackCoords` -1 -1 -2 2 "NewEnumerator3" 1 _buffedattackranges_left)
  (`self.AddConsecutiveAttackCoords` -2 -2 -1 1 "NewEnumerator3" 1 _buffedattackranges_left)
  (`self.AddConsecutiveAttackCoords` 1 1 -2 2 "NewEnumerator4" 1 _buffedattackranges_right)
  (`self.AddConsecutiveAttackCoords` 2 2 -1 1 "NewEnumerator4" 1 _buffedattackranges_right)
  (return))

(fn `DefineCapacityRange`
  (bind _capacityrange (`self.CapacityRange`))
  (`self.AddConsecutiveCoords` -1 1 -1 1 _capacityrange)
  (`self.AddConsecutiveCoords` 0 0 -2 -2 _capacityrange)
  (`self.AddConsecutiveCoords` 0 0 2 2 _capacityrange)
  (`self.AddConsecutiveCoords` -2 -2 0 0 _capacityrange)
  (`self.AddConsecutiveCoords` 2 2 0 0 _capacityrange)
  (return))

(fn `UseCapacity`
  (params (TargetedBlock :type "/Game/Battlefield/Block/BP_Block Object Reference"))
  (locals (Block :type "/Game/Battlefield/Block/BP_Block Object Reference"))
  (bind _block (`local.Block`))
  (bind _bindedunit (`/Game/Battlefield/Block/BP_Block.BindedUnit` _block))
  (`/Game/Core/BP_SoundManager.PlayActionSound` (`self.SoundManager`) self "NewEnumerator4")
  (for _array_element (`self.CapacityRange`)
    ;[1 1 1] Find the Block corresponding to the relative coordinates of this element of the Capacity Range.
    (bind _absolutecoords (`/Game/Core/BP_CoordsFunctionLibrary.GetAbsoluteCoordsFromRelatives` (`/Game/Battlefield/Block/BP_Block.Coords` (`self.BindedBlock`)) _array_element))
    (bind _binbounds (`/Game/Core/BP_CoordsFunctionLibrary.AreCoordsInBounds` (break `/Game/Core/S_Coords` _absolutecoords) (`.Y_6_2DC6362D4EE28ABEA56491A3230A1BE6` (break `/Game/Core/S_Coords` _absolutecoords))))
    (if _binbounds
      (bind _index (`/Game/Core/BP_CoordsFunctionLibrary.CalculateBlockIndex` (break `/Game/Core/S_Coords` _absolutecoords) (`.Y_6_2DC6362D4EE28ABEA56491A3230A1BE6` (break `/Game/Core/S_Coords` _absolutecoords))))
      (bind _output_get (set `local.Block` (`BlueprintMapLibrary.Map_Find` (`/Game/Core/GameMode/BattleScene/BP_GS_Battle.Battlefield` (`self.GameState`)) _index)))
      (if (`|EnumEquality` (`/Game/Battlefield/Block/BP_Block.BlockOwner` _output_get) (`self.Faction`))
        (set `/Game/Battlefield/Block/BP_Block.IncrustationLevel` (`KismetMathLibrary.Clamp` (+ (`/Game/Battlefield/Block/BP_Block.IncrustationLevel` _block) 1) 0 3) _block)
        (`/Game/Battlefield/Block/BP_Block.UpdateColor` _block false))
      (`/Engine/EditorBlueprintResources/StandardMacros.IsValid` _bindedunit ; If there is Unit on the block, \ncheck if it is still stuck or not.
        (:`Is Valid`
          (if (`|EnumInequality` (`/Game/Units/BP_Unit.Faction` _bindedunit) (`self.Faction`))
            (`self.UpdateStuckStatus` _bindedunit false))))))
  (set `self.bBuffed` false)
  (`/Game/Core/GameMode/BattleScene/BP_GS_Battle.EndCurrentPhase` (`self.GameState`) true)
  (return))

(fn `UserConstructionScript`
  (`parent.UserConstructionScript`)
  (set `self.Class` "NewEnumerator1"))