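; Sniper unit for a grid tactics game, defining its attack and capacity ranges as relative coordinates at BeginPlay.
; Attacks run in straight lines in four directions, with the buffed version adding farther, differently powered cells.
; Its capacity targets a diamond excluding the nearest cells, clearing the targeted block's incrustation and ownership and lowering incrustation on adjacent other-faction blocks.
; UseCapacity also refreshes affected units' stuck status, removes the buff and ends the phase.
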(event `self.ReceiveBeginPlay`
  (`self.SetGameStateAndManagers`)
  (`self.DefineAttackRange`)
  (`self.DefineBuffedAttackRange`)
  (`self.DefineCapacityRange`))

(fn `DefineAttackRange`
  (bind (_attackranges_up _attackranges_down _attackranges_left _attackranges_right) (break `/Game/Core/S_AttackRange` (`self.AttackRanges`)))
  (`self.AddConsecutiveAttackCoords` 0 0 -4 -1 "NewEnumerator1" 1 _attackranges_up)
  (`self.AddConsecutiveAttackCoords` 0 0 1 4 "NewEnumerator2" 1 _attackranges_down)
  (`self.AddConsecutiveAttackCoords` -4 -1 0 0 "NewEnumerator3" 1 _attackranges_left)
  (`self.AddConsecutiveAttackCoords` 1 4 0 0 "NewEnumerator4" 1 _attackranges_right)
  (return))

(fn `DefineBuffedAttackRange`
  (bind (_buffedattackranges_up _buffedattackranges_down _buffedattackranges_left _buffedattackranges_right) (break `/Game/Core/S_AttackRange` (`self.BuffedAttackRanges`)))
  (`self.AddConsecutiveAttackCoords` 0 0 -4 -1 "NewEnumerator1" 1 _buffedattackranges_up)
  (`self.AddConsecutiveAttackCoords` 0 0 -6 -5 "NewEnumerator1" 2 _buffedattackranges_up)
  (`self.AddConsecutiveAttackCoords` 0 0 1 4 "NewEnumerator2" 1 _buffedattackranges_down)
  (`self.AddConsecutiveAttackCoords` 0 0 5 6 "NewEnumerator2" 2 _buffedattackranges_down)
  (`self.AddConsecutiveAttackCoords` -4 -1 0 0 "NewEnumerator3" 1 _buffedattackranges_left)
  (`self.AddConsecutiveAttackCoords` -6 -5 0 0 "NewEnumerator3" 2 _buffedattackranges_left)
  (`self.AddConsecutiveAttackCoords` 1 4 0 0 "NewEnumerator4" 1 _buffedattackranges_right)
  (`self.AddConsecutiveAttackCoords` 5 6 0 0 "NewEnumerator4" 2 _buffedattackranges_right)
  (return))

(fn `DefineCapacityRange`
  (bind _capacityeffectrange (`self.CapacityEffectRange`))
  (bind _capacityrange (`self.CapacityRange`))
  (`|ExecutionSequence`
    (:`then_0`
      (`self.AddConsecutiveCoords` 0 0 -4 -4 _capacityrange)
      (`self.AddConsecutiveCoords` -1 1 -3 -3 _capacityrange)
      (`self.AddConsecutiveCoords` -2 2 -2 -2 _capacityrange)
      (`self.AddConsecutiveCoords` -3 -1 -1 -1 _capacityrange)
      (`self.AddConsecutiveCoords` 1 3 -1 -1 _capacityrange)
      (`self.AddConsecutiveCoords` -4 -2 0 0 _capacityrange)
      (`self.AddConsecutiveCoords` 2 4 0 0 _capacityrange)
      (`self.AddConsecutiveCoords` -3 -1 1 1 _capacityrange)
      (`self.AddConsecutiveCoords` 1 3 1 1 _capacityrange)
      (`self.AddConsecutiveCoords` -2 2 2 2 _capacityrange)
      (`self.AddConsecutiveCoords` -1 1 3 3 _capacityrange)
      (`self.AddConsecutiveCoords` 0 0 4 4 _capacityrange))
    (:`then_1`
      (`self.AddConsecutiveCapacityCoords` 0 0 0 0 "NewEnumerator0" "NewEnumerator0" _capacityeffectrange)
      (`self.AddConsecutiveCapacityCoords` 0 0 -1 -1 "NewEnumerator0" "NewEnumerator1" _capacityeffectrange)
      (`self.AddConsecutiveCapacityCoords` 0 0 1 1 "NewEnumerator0" "NewEnumerator1" _capacityeffectrange)
      (`self.AddConsecutiveCapacityCoords` -1 -1 0 0 "NewEnumerator0" "NewEnumerator1" _capacityeffectrange)
      (`self.AddConsecutiveCapacityCoords` 1 1 0 0 "NewEnumerator0" "NewEnumerator1" _capacityeffectrange))
    (:`then_2`
      (return))))

(fn `UseCapacity`
  (params (TargetedBlock :type "/Game/Battlefield/Block/BP_Block Object Reference"))
  (locals (CurrBlock :type "/Game/Battlefield/Block/BP_Block Object Reference"))
  (bind _currblock (`local.CurrBlock`))
  (bind _currblock_2 (`local.CurrBlock`))
  (bind _bindedunit (`/Game/Battlefield/Block/BP_Block.BindedUnit` _currblock))
  (`/Game/Core/BP_SoundManager.PlayActionSound` (`self.SoundManager`) self "NewEnumerator4")
  (`|ExecutionSequence`
    (:`then_0`
      (for _array_element (`self.CapacityEffectRange`)
        (bind (_absolutecoords _block _bcoordsinbounds) (`/Game/Core/GameMode/BattleScene/BP_GS_Battle.FindBlockFromRelativeCoords` (`self.GameState`) (`/Game/Battlefield/Block/BP_Block.Coords` (`local.TargetedBlock`)) (break `/Game/Core/S_CapacityCoords` _array_element)))
        (if _bcoordsinbounds
          (set `local.CurrBlock` _block)
          (switch `/Game/Core/E_CapacityEffect` (`.Effect_10_E7EC0D8145F20EB8AFCAA2B64F41EB9D` (break `/Game/Core/S_CapacityCoords` _array_element))
            (:`NewEnumerator0`
              (set `/Game/Battlefield/Block/BP_Block.IncrustationLevel` 0 (`local.CurrBlock`))
              (set `/Game/Battlefield/Block/BP_Block.BlockOwner` "NewEnumerator0" _currblock :!label _label)
              (`/Game/Battlefield/Block/BP_Block.UpdateColor` _currblock false :!label _label_2)
              (`/Engine/EditorBlueprintResources/StandardMacros.IsValid` _bindedunit ; If there is Unit on the block, \ncheck if it is still stuck or not.
                (:`Is Valid`
                  (`self.UpdateStuckStatus` _bindedunit false))))
            (:`NewEnumerator1`
              (if (`|EnumInequality` (`self.Faction`) (`/Game/Battlefield/Block/BP_Block.BlockOwner` _currblock_2))
                (bind _output_get (set `/Game/Battlefield/Block/BP_Block.IncrustationLevel` (`KismetMathLibrary.Clamp` (- (`/Game/Battlefield/Block/BP_Block.IncrustationLevel` _currblock_2) 1) 0 3) (`local.CurrBlock`)))
                (if (== _output_get 0)
                  (goto _label)
                  (else
                    (goto _label_2)))))))))
    (:`then_1`
      (set `self.bBuffed` false)
      (`/Game/Core/GameMode/BattleScene/BP_GS_Battle.EndCurrentPhase` (`self.GameState`) true)
      (return))))

(fn `UserConstructionScript`
  (`parent.UserConstructionScript`)
  (set `self.Class` "NewEnumerator0"))