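; BP_Inlayer is a faction-based unit for a grid tactics game, built on a parent unit Blueprint.
; The construction script sets its class and colors its arms and hands blue or orange by faction.
; On BeginPlay it sets game state, then fills coordinate arrays through range helper functions.
; Movement forms a diamond around the unit, while attacks run in four straight directions, reaching farther when buffed.
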(event `self.ReceiveBeginPlay`
  (`self.SetGameState`)
  (`self.DefineMoveRange`)
  (`self.DefineAttackRange`)
  (`self.DefineBuffedAttackRange`))

(fn `DefineAttackRange`
  (bind (_attackranges_up _attackranges_down _attackranges_left _attackranges_right) (break `/Game/Core/S_AttackRange` (`self.AttackRanges`)))
  (`self.AddConsecutiveAttackCoords` 0 0 -2 -1 "NewEnumerator1" 2 _attackranges_up)
  (`self.AddConsecutiveAttackCoords` 0 0 1 2 "NewEnumerator2" 2 _attackranges_down)
  (`self.AddConsecutiveAttackCoords` -2 -1 0 0 "NewEnumerator3" 2 _attackranges_left)
  (`self.AddConsecutiveAttackCoords` 1 2 0 0 "NewEnumerator4" 2 _attackranges_right)
  (return))

(fn `DefineBuffedAttackRange`
  (bind (_buffedattackranges_up _buffedattackranges_down _buffedattackranges_left _buffedattackranges_right) (break `/Game/Core/S_AttackRange` (`self.BuffedAttackRanges`)))
  (`self.AddConsecutiveAttackCoords` 0 0 -3 0 "NewEnumerator1" 2 _buffedattackranges_up)
  (`self.AddConsecutiveAttackCoords` 0 0 0 3 "NewEnumerator2" 2 _buffedattackranges_down)
  (`self.AddConsecutiveAttackCoords` -3 0 0 0 "NewEnumerator3" 2 _buffedattackranges_left)
  (`self.AddConsecutiveAttackCoords` 0 3 0 0 "NewEnumerator4" 2 _buffedattackranges_right)
  (return))

(fn `DefineMoveRange`
  (bind _moverange (`self.MoveRange`))
  (`self.AddConsecutiveCoords` 0 0 -3 -3 _moverange)
  (`self.AddConsecutiveCoords` -1 1 -2 -2 _moverange)
  (`self.AddConsecutiveCoords` -2 2 -1 -1 _moverange)
  (`self.AddConsecutiveCoords` -3 -1 0 0 _moverange)
  (`self.AddConsecutiveCoords` 1 3 0 0 _moverange)
  (`self.AddConsecutiveCoords` -2 2 1 1 _moverange)
  (`self.AddConsecutiveCoords` -1 1 2 2 _moverange)
  (`self.AddConsecutiveCoords` 0 0 3 3 _moverange)
  (return))

(fn `UserConstructionScript`
  (`parent.UserConstructionScript`)
  (set `self.Class` "NewEnumerator2")
  (switch `/Game/Core/E_Faction` (`self.Faction`)
    (:`NewEnumerator1`
      (`PrimitiveComponent.SetMaterial` (`self.BigArm1`) 0 "/Game/MaterialLibrary/M_BlueLV1.M_BlueLV1")
      (`PrimitiveComponent.SetMaterial` (`self.Hand1`) 0 "/Game/MaterialLibrary/M_BlueLV1.M_BlueLV1")
      (`PrimitiveComponent.SetMaterial` (`self.BigArm2`) 0 "/Game/MaterialLibrary/M_BlueLV1.M_BlueLV1")
      (`PrimitiveComponent.SetMaterial` (`self.Hand2`) 0 "/Game/MaterialLibrary/M_BlueLV1.M_BlueLV1"))
    (:`NewEnumerator2`
      (`PrimitiveComponent.SetMaterial` (`self.BigArm1`) 0 "/Game/MaterialLibrary/M_OrangeLV1.M_OrangeLV1")
      (`PrimitiveComponent.SetMaterial` (`self.Hand1`) 0 "/Game/MaterialLibrary/M_OrangeLV1.M_OrangeLV1")
      (`PrimitiveComponent.SetMaterial` (`self.BigArm2`) 0 "/Game/MaterialLibrary/M_OrangeLV1.M_OrangeLV1")
      (`PrimitiveComponent.SetMaterial` (`self.Hand2`) 0 "/Game/MaterialLibrary/M_OrangeLV1.M_OrangeLV1"))))