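; Base class for a faction unit on the grid battlefield, bound two-way to the block it stands on and forwarding clicks and hover to it.
; Move relinks blocks; Attack applies directional, optionally buffed ranges to shift block ownership and incrustation, marking units stuck on enemy max-level blocks, and both end the phase.
; Class-specific timelines loop a jump cue for selectable units.
; Range definitions and capacity are placeholders for subclasses.
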(event `self.ReceiveActorOnClicked`
  (params (ButtonPressed :type "Key Structure"))
  (`/Game/Battlefield/BP_Block.HandleClick` (`self.BindedBlock`)))

(event `self.ReceiveActorBeginCursorOver`
  (`SceneComponent.SetVisibility` (`/Game/Battlefield/BP_Block.HoveringPlane` (`self.BindedBlock`)) true false))

(event `self.ReceiveActorEndCursorOver`
  (`SceneComponent.SetVisibility` (`/Game/Battlefield/BP_Block.HoveringPlane` (`self.BindedBlock`)) false false))

(event `TriggerJump`
  ;[1 1 1] Make the Unit jump to inform the player that it can be chosen this turn.
  (switch `/Game/Core/E_Class` (`self.Class`)
    (:`NewEnumerator0`
      (bind (_direction _alpha) (`Timeline|SniperJump` :!via `PlayFromStart`)
        (:`Update`
          (`SceneComponent.K2_SetWorldLocation` (`self.Character`) (`KismetMathLibrary.VLerp` (`SceneComponent.K2_GetComponentLocation` (`self.BottomPoint`)) (`SceneComponent.K2_GetComponentLocation` (`self.TopPoint`)) _alpha) false false))
        (:`Finished`
          (if (`self.bMustJump`)
            (`self.TriggerJump`)))))
    (:`NewEnumerator1`
      (bind (_direction_2 _alpha_2) (`Timeline|ProtectorJump` :!via `PlayFromStart`)
        (:`Update`
          (`SceneComponent.K2_SetWorldLocation` (`self.Character`) (`KismetMathLibrary.VLerp` (`SceneComponent.K2_GetComponentLocation` (`self.BottomPoint`)) (`SceneComponent.K2_GetComponentLocation` (`self.TopPoint`)) _alpha_2) false false))
        (:`Finished`
          (if (`self.bMustJump`)
            (`self.TriggerJump`)))))
    (:`NewEnumerator2`
      (bind (_direction_3 _alpha_3) (`Timeline|InlayerJump` :!via `PlayFromStart`)
        (:`Update`
          (`SceneComponent.K2_SetWorldLocation` (`self.Character`) (`KismetMathLibrary.VLerp` (`SceneComponent.K2_GetComponentLocation` (`self.BottomPoint`)) (`SceneComponent.K2_GetComponentLocation` (`self.TopPoint`)) _alpha_3) false false))
        (:`Finished`
          (if (`self.bMustJump`)
            (`self.TriggerJump`)))))))

(fn `AddConsecutiveAttackCoords`
  (params (FirstX :type Integer) (LastX :type Integer) (FirstY :type Integer) (LastY :type Integer) (Direction :type "/Game/Core/E_Direction Enum" :default "NewEnumerator0") (Power :type Integer) (Array :type "Array of /Game/Core/S_AttackCoords Structure"))
  (for _index (range FirstX (+ LastX 1))
    (for _index_2 (range FirstY (+ LastY 1))
      (`KismetArrayLibrary.Array_Add` Array (make `/Game/Core/S_AttackCoords` (make `/Game/Core/S_Coords` _index _index_2) Direction Power))))
  (return))

(fn `AddConsecutiveCoords`
  (params (FirstX :type Integer) (LastX :type Integer) (FirstY :type Integer) (LastY :type Integer) (Array :type "Array of /Game/Core/S_Coords Structure"))
  (for _index (range FirstX (+ LastX 1))
    (for _index_2 (range FirstY (+ LastY 1))
      (`KismetArrayLibrary.Array_Add` Array (make `/Game/Core/S_Coords` _index _index_2))))
  (return))

(fn `Attack`
  (locals (AttackRange :type "Array of /Game/Core/S_AttackCoords Structure") (Power :type Integer) (Block :type "/Game/Battlefield/BP_Block Object Reference"))
  (bind (_attackranges_up _attackranges_down _attackranges_left _attackranges_right) (break `/Game/Core/S_AttackRange` (`self.AttackRanges`)))
  (bind (_buffedattackranges_up _buffedattackranges_down _buffedattackranges_left _buffedattackranges_right) (break `/Game/Core/S_AttackRange` (`self.BuffedAttackRanges`)))
  (bind _block (`local.Block`))
  (bind _bindedunit (`/Game/Battlefield/BP_Block.BindedUnit` _block))
  (bind _returnvalue (- (`/Game/Battlefield/BP_Block.IncrustationLevel` (`local.Block`)) (`local.Power`)))
  (if (`self.bBuffed`)
    (switch `/Game/Core/E_Direction` (`self.CurrActionDirection`)
      (:`NewEnumerator1`
        (set `local.AttackRange` _buffedattackranges_up))
      (:`NewEnumerator2`
        (set `local.AttackRange` _buffedattackranges_down))
      (:`NewEnumerator3`
        (set `local.AttackRange` _buffedattackranges_left))
      (:`NewEnumerator4`
        (set `local.AttackRange` _buffedattackranges_right)))
    (else
      (switch `/Game/Core/E_Direction` (`self.CurrActionDirection`)
        (:`NewEnumerator1`
          (set `local.AttackRange` _attackranges_up))
        (:`NewEnumerator2`
          (set `local.AttackRange` _attackranges_down))
        (:`NewEnumerator3`
          (set `local.AttackRange` _attackranges_left))
        (:`NewEnumerator4`
          (set `local.AttackRange` _attackranges_right)))))
  (for _array_element (`local.AttackRange`)
    ;[1 1 1] Find the Block corresponding to the relative coordinates of this element of the Attack Range.
    (set `local.Power` (`.Power_5_E7EC0D8145F20EB8AFCAA2B64F41EB9D` (break `/Game/Core/S_AttackCoords` _array_element)))
    (bind _absolutecoords (`/Game/Core/BP_CoordsFunctionLibrary.GetAbsoluteCoordsFromRelatives` (`/Game/Battlefield/BP_Block.Coords` (`self.BindedBlock`)) (break `/Game/Core/S_AttackCoords` _array_element)))
    (bind _binbounds (`/Game/Core/BP_CoordsFunctionLibrary.AreCoordsInBounds` (break `/Game/Core/S_Coords` _absolutecoords) (`.Y_6_2DC6362D4EE28ABEA56491A3230A1BE6` (break `/Game/Core/S_Coords` _absolutecoords))))
    (if _binbounds
      (bind _index (`/Game/Core/BP_CoordsFunctionLibrary.CalculateBlockIndex` (break `/Game/Core/S_Coords` _absolutecoords) (`.Y_6_2DC6362D4EE28ABEA56491A3230A1BE6` (break `/Game/Core/S_Coords` _absolutecoords))))
      (bind _output_get (set `local.Block` (`BlueprintMapLibrary.Map_Find` (`/Game/Core/GameMode/BP_GameState.Battlefield` (`self.GameState`)) _index)))
      (if (`SceneComponent.IsVisible` (`/Game/Battlefield/BP_Block.ActionRangePlane` _output_get))
        ;[1 1 1] Logic to apply to know what happen to the Block after the Unit attack, depending on their respective Factions and the power level of the attack.
        (if (`|EnumEquality` (`/Game/Battlefield/BP_Block.BlockOwner` (`local.Block`)) (`self.Faction`))
          (set `/Game/Battlefield/BP_Block.IncrustationLevel` (`KismetMathLibrary.Clamp` (+ (`/Game/Battlefield/BP_Block.IncrustationLevel` (`local.Block`)) (`local.Power`)) 0 3) (`local.Block`))
          (elif (== _returnvalue 0)
            (set `/Game/Battlefield/BP_Block.BlockOwner` "NewEnumerator0" (`local.Block`))
            (set `/Game/Battlefield/BP_Block.IncrustationLevel` 0 (`local.Block`))
            (elif (< _returnvalue 0)
              (set `/Game/Battlefield/BP_Block.BlockOwner` (`self.Faction`) (`local.Block`))
              (set `/Game/Battlefield/BP_Block.IncrustationLevel` (`KismetMathLibrary.Abs_Int` _returnvalue) (`local.Block`))
              (else
                (set `/Game/Battlefield/BP_Block.IncrustationLevel` _returnvalue (`local.Block`))))))
        (`/Game/Battlefield/BP_Block.UpdateColor` (`local.Block`))
        ;[1 1 1] Set the Unit on the current Block to "stuck" if the Block is an obstacle and they are from opposite Factions.
        (`/Engine/EditorBlueprintResources/StandardMacros.IsValid` _bindedunit
          (:`Is Valid`
            (set `/Game/Units/BP_Unit.bStuck` (and (`|EnumInequality` (`/Game/Units/BP_Unit.Faction` _bindedunit) (`/Game/Battlefield/BP_Block.BlockOwner` _block)) (== (`/Game/Battlefield/BP_Block.IncrustationLevel` _block) 3)) _bindedunit))))))
  (set `self.bBuffed` false)
  (`/Game/Core/GameMode/BP_GameState.EndCurrentPhase` (`self.GameState`) true)
  (return))

(fn `BindBlock`
  (params (Block :type "/Game/Battlefield/BP_Block Object Reference"))
  (set `self.BindedBlock` Block)
  (return))

(fn `Buff`
  (set `self.bBuffed` true)
  (return))

(fn `DefineAttackRange`
  (`KismetSystemLibrary.PrintString` "Defining Attack Range for Unit superclass.")
  (return))

(fn `DefineBuffedAttackRange`
  (`KismetSystemLibrary.PrintString` "Defining Buffed Attack Range for Unit superclass.")
  (return))

(fn `DefineCapacityRange`
  (`KismetSystemLibrary.PrintString` "Defining Capacity Range for Unit superclass.")
  (return))

(fn `Move`
  (params (NewBindedBlock :type "/Game/Battlefield/BP_Block Object Reference"))
  (bind (_returnvalue_x _returnvalue_y) (`KismetMathLibrary.BreakVector` (`self.K2_GetActorLocation` NewBindedBlock)))
  (set `/Game/Battlefield/BP_Block.BindedUnit` null (`self.BindedBlock`)) ; Remove prev link from Block to Unit.
  (bind _output_get (set `self.BindedBlock` NewBindedBlock)) ; Add new link from Unit to Block.
  (set `/Game/Battlefield/BP_Block.BindedUnit` self _output_get) ; Add new link from Block to Unit.
  (`self.K2_SetActorLocation` (`KismetMathLibrary.MakeVector` _returnvalue_x _returnvalue_y 75.0) false true)
  (set `self.bStuck` false) ; If Unit has been able to move, \nit means it is not stuck anymore.
  (`/Game/Core/GameMode/BP_GameState.EndCurrentPhase` (`self.GameState`) true)
  (return))

(fn `SetGameState`
  (bind _asbp_game_state (cast `/Game/Core/GameMode/BP_GameState` (`GameplayStatics.GetGameState`)))
  (set `self.GameState` _asbp_game_state)
  (return))

(fn `UseCapacity`
  (params (Sniper_BlockToWipeOut :type "/Game/Battlefield/BP_Block Object Reference"))
  (`KismetSystemLibrary.PrintString` "Defining Capacity use for Unit superclass.")
  (return))

(fn `UserConstructionScript`
  (`|ExecutionSequence`
    (:`then_0`
      (switch `/Game/Core/E_Faction` (`self.Faction`)
        (:`NewEnumerator1`
          (`PrimitiveComponent.SetMaterial` (`self.Head`) 0 "/Game/MaterialLibrary/M_BlueLV2.M_BlueLV2")
          (`PrimitiveComponent.SetMaterial` (`self.Body`) 0 "/Game/MaterialLibrary/M_BlueLV3.M_BlueLV3"))
        (:`NewEnumerator2`
          (`PrimitiveComponent.SetMaterial` (`self.Head`) 0 "/Game/MaterialLibrary/M_OrangeLV2.M_OrangeLV2")
          (`PrimitiveComponent.SetMaterial` (`self.Body`) 0 "/Game/MaterialLibrary/M_OrangeLV3.M_OrangeLV3"))))
    (:`then_1`
      (`SceneComponent.K2_SetRelativeLocation` (`self.TopPoint`) (`KismetMathLibrary.MakeVector` 0.0 0.0 (`self.TopPosition`)) false false))))