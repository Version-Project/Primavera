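; Blueprint function library of grid coordinate and faction helpers for a game with Winter and Spring factions on a 16 by 11 block board.
; It converts between flat indices and X/Y coordinates using X * 11 + Y, checks bounds and offsets relative coordinates from a reference point.
; Other helpers return the opposing faction, the direction between two orthogonally adjacent blocks, and print coordinates for debugging.
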(fn `AreBlocksAdjacentInOneDirection`
  (params (StartingBlock :type "/Game/Battlefield/Block/BP_Block Object Reference") (FinishBlock :type "/Game/Battlefield/Block/BP_Block Object Reference"))
  (returns (Direction :type "/Game/Core/E_Direction Enum"))
  (locals (StartingCoords :type "/Game/Core/S_Coords Structure") (FinishCoords :type "/Game/Core/S_Coords Structure") (DiffX :type Integer) (DiffY :type Integer))
  (bind _finishcoords_x (break `/Game/Core/S_Coords` (`local.FinishCoords`)))
  (bind (_startingcoords_x _startingcoords_y) (break `/Game/Core/S_Coords` (`local.StartingCoords`)))
  (bind (_finishcoords_x_2 _finishcoords_y) (break `/Game/Core/S_Coords` (`local.FinishCoords`)))
  (bind _startingcoords_x_2 (break `/Game/Core/S_Coords` (`local.StartingCoords`)))
  (set `local.StartingCoords` (`/Game/Battlefield/Block/BP_Block.Coords` StartingBlock))
  (set `local.FinishCoords` (`/Game/Battlefield/Block/BP_Block.Coords` FinishBlock))
  (set `local.DiffX` (- _finishcoords_x _startingcoords_x_2))
  (set `local.DiffY` (- _finishcoords_y _startingcoords_y))
  (`|ExecutionSequence`
    (:`then_0`
      (if (and (== (`local.DiffX`) 0) (== (`local.DiffY`) -1))
        (return "NewEnumerator1")))
    (:`then_1`
      (if (and (== (`local.DiffX`) 0) (== (`local.DiffY`) 1))
        (return "NewEnumerator2")))
    (:`then_2`
      (if (and (== (`local.DiffX`) -1) (== (`local.DiffY`) 0))
        (return "NewEnumerator3")))
    (:`then_3`
      (if (and (== (`local.DiffX`) 1) (== (`local.DiffY`) 0))
        (return "NewEnumerator4")))
    (:`then_4`
      (return "NewEnumerator0"))))

(fn `AreCoordsInBounds`
  (params (X :type Integer) (Y :type Integer))
  (returns (bInBounds :type Boolean))
  (return (and (>= X 0) (< X 16) (>= Y 0) (< Y 11))))

(fn `CalculateBlockCoordinates`
  (params (Index :type Integer))
  (returns (X :type Integer) (Y :type Integer))
  (bind (_remainder _returnvalue) (`KismetMathLibrary.FMod` (`KismetMathLibrary.Conv_IntToDouble` Index) 11.0))
  (return _returnvalue (`KismetMathLibrary.FTrunc` _remainder)))

(fn `CalculateBlockIndex`
  (params (X :type Integer) (Y :type Integer))
  (returns (Index :type Integer))
  (return (+ (* X 11) Y)))

(fn `GetAbsoluteCoordsFromRelatives`
  (params (ReferencePoint :type "/Game/Core/S_Coords Structure") (RelativeCoords :type "/Game/Core/S_Coords Structure"))
  (returns (AbsoluteCoords :type "/Game/Core/S_Coords Structure"))
  (return (make `/Game/Core/S_Coords` (+ ReferencePoint_X_5_364656D3417FA6B1F82E4585A34E5C6B RelativeCoords_X_5_364656D3417FA6B1F82E4585A34E5C6B) (+ ReferencePoint_Y_6_2DC6362D4EE28ABEA56491A3230A1BE6 RelativeCoords_Y_6_2DC6362D4EE28ABEA56491A3230A1BE6))))

(fn `GetBlockCoordsFromIndex`
  (params (BlockIndex :type Integer))
  (returns (Coords :type "/Game/Core/S_Coords Structure"))
  (bind (_x _y) (`self.CalculateBlockCoordinates` BlockIndex))
  (return (make `/Game/Core/S_Coords` _x _y)))

(fn `GetOppositeFaction`
  (params (Faction :type "/Game/Core/E_Faction Enum" :default "NewEnumerator0"))
  (returns (OppositeFaction :type "/Game/Core/E_Faction Enum"))
  (switch `/Game/Core/E_Faction` Faction
    (:`NewEnumerator0`
      (return "NewEnumerator0"))
    (:`NewEnumerator1`
      (return "NewEnumerator2"))
    (:`NewEnumerator2`
      (return "NewEnumerator1"))))

(fn `PrintCoords`
  (params (PrevText :type String) (Coords :type "/Game/Core/S_Coords Structure") (Duration :type "Float (double-precision)"))
  (`KismetSystemLibrary.PrintString` null (`KismetStringLibrary.Concat_StrStr` PrevText "(" (`KismetStringLibrary.Conv_IntToString` Coords_X_5_364656D3417FA6B1F82E4585A34E5C6B) " ; " (`KismetStringLibrary.Conv_IntToString` Coords_Y_6_2DC6362D4EE28ABEA56491A3230A1BE6) ")") true true (struct :`R` 0.044062 :`G` 0.536458 :`A` 1.0) Duration)
  (return))