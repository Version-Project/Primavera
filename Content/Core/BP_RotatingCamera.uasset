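; BP_RotatingCamera is a spring-arm camera rig that keeps its rotation and zoom within configured limits.
; Its construction script clamps the SpringArm's world pitch and yaw to vertical and horizontal bounds, zeroes roll, and clamps arm length to the zoom range.
; Tick is empty, and the nodes deriving limits from half-ranges around the current rotation are disconnected, as is a yaw debug print.
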(event `self.ReceiveTick`
  (params (DeltaSeconds :type "Float (single-precision)")))

(fn `UserConstructionScript`
  (bind _springarm (`self.SpringArm`))
  (bind (_returnvalue_roll _returnvalue_pitch _returnvalue_yaw) (`KismetMathLibrary.BreakRotator` (`SceneComponent.K2_GetComponentRotation` (`self.SpringArm`))))
  (`SceneComponent.K2_SetWorldRotation` _springarm (`KismetMathLibrary.MakeRotator` 0.0 (`KismetMathLibrary.FClamp` _returnvalue_pitch (`self.V_InfLimit`) (`self.V_SupLimit`)) (`KismetMathLibrary.FClamp` _returnvalue_yaw (`self.H_InfLimit`) (`self.H_SupLimit`))) false false)
  (set `SpringArmComponent.TargetArmLength` (`KismetMathLibrary.FClamp` (`SpringArmComponent.TargetArmLength` _springarm) (`self.Zoom_InfLimit`) (`self.Zoom_SupLimit`)) _springarm))