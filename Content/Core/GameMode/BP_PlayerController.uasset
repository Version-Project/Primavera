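; Player controller that lets the player orbit and zoom a BP_RotatingCamera around the battlefield.
; On BeginPlay it finds and caches the camera actor in the level.
; While the ClickCamera input is held, mouse axes turn the spring arm's yaw and pitch within the camera's limits.
; The mouse wheel zooms via arm length in perspective or ortho width in orthographic, using speeds and limits stored on the camera.
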(event `self.ReceiveBeginPlay`
  (bind _returnvalue (`GameplayStatics.GetActorOfClass` "/Game/Core/BP_RotatingCamera.BP_RotatingCamera_C"))
  (`/Engine/EditorBlueprintResources/StandardMacros.IsValid` _returnvalue
    (:`Is Valid`
      (set `self.RotatingCamera` _returnvalue))))

(event `InputAction|InputAction_ClickCamera`
  (params (Key :type "Key Structure"))
  (:`Pressed`
    (set `self.bCanRotateCamera` true))
  (:`Released`
    (set `self.bCanRotateCamera` false)))

(event `InputAxisKey|MouseX`
  (params (AxisValue :type "Float (single-precision)"))
  (bind _rotatingcamera (`self.RotatingCamera`))
  (bind _springarm (`/Game/Core/BP_RotatingCamera.SpringArm` (`self.RotatingCamera`)))
  (bind (_returnvalue_roll _returnvalue_pitch _returnvalue_yaw) (`KismetMathLibrary.BreakRotator` (`SceneComponent.K2_GetComponentRotation` _springarm)))
  ;[1 1 1] Moving Camera horizontally around the battlefield.
  (if (`self.bCanRotateCamera`)
    (`SceneComponent.K2_SetWorldRotation` _springarm (`KismetMathLibrary.MakeRotator` _returnvalue_roll _returnvalue_pitch (`KismetMathLibrary.FClamp` (+ _returnvalue_yaw (* AxisValue (`/Game/Core/BP_RotatingCamera.RotationSpeed` (`self.RotatingCamera`)))) (`/Game/Core/BP_RotatingCamera.H_InfLimit` _rotatingcamera) (`/Game/Core/BP_RotatingCamera.H_SupLimit` _rotatingcamera))) false false)))

(event `InputAxisKey|MouseY`
  (params (AxisValue :type "Float (single-precision)"))
  (bind _rotatingcamera (`self.RotatingCamera`))
  (bind _springarm (`/Game/Core/BP_RotatingCamera.SpringArm` (`self.RotatingCamera`)))
  (bind (_returnvalue_roll _returnvalue_pitch _returnvalue_yaw) (`KismetMathLibrary.BreakRotator` (`SceneComponent.K2_GetComponentRotation` _springarm)))
  ;[1 1 1] Moving Camera vertically around the battlefield.
  (if (`self.bCanRotateCamera`)
    (`SceneComponent.K2_SetWorldRotation` _springarm (`KismetMathLibrary.MakeRotator` _returnvalue_roll (`KismetMathLibrary.FClamp` (+ _returnvalue_pitch (* AxisValue (`/Game/Core/BP_RotatingCamera.RotationSpeed` (`self.RotatingCamera`)))) (`/Game/Core/BP_RotatingCamera.V_InfLimit` _rotatingcamera) (`/Game/Core/BP_RotatingCamera.V_SupLimit` _rotatingcamera)) _returnvalue_yaw) false false)))

(event `InputAxisKey|MouseWheelAxis`
  (params (AxisValue :type "Float (single-precision)"))
  (bind _rotatingcamera (`self.RotatingCamera`))
  (bind _rotatingcamera_2 (`self.RotatingCamera`))
  (bind _camera (`/Game/Core/BP_RotatingCamera.Camera` (`self.RotatingCamera`)))
  (bind _springarm (`/Game/Core/BP_RotatingCamera.SpringArm` (`self.RotatingCamera`)))
  ;[1 1 1] Check if Camera Projection mode is Perspective or Orthographic.
  (set `self.MouseWheelValue` AxisValue)
  (if (`|EnumEquality` (`CameraComponent.ProjectionMode` (`/Game/Core/BP_RotatingCamera.Camera` (`self.RotatingCamera`))) "Perspective")
    ;[1 1 1] Zooming (Perspective mode)
    (set `SpringArmComponent.TargetArmLength` (`KismetMathLibrary.FClamp` (+ (`SpringArmComponent.TargetArmLength` _springarm) (* (`self.MouseWheelValue`) (`/Game/Core/BP_RotatingCamera.ZoomSpeed` (`self.RotatingCamera`)) -1.0)) (`/Game/Core/BP_RotatingCamera.Zoom_InfLimit` _rotatingcamera_2) (`/Game/Core/BP_RotatingCamera.Zoom_SupLimit` _rotatingcamera_2)) _springarm)
    (else
      ;[1 1 1] Zooming (Orthographic mode)
      (`CameraComponent.SetOrthoWidth` _camera (`KismetMathLibrary.FClamp` (+ (`CameraComponent.OrthoWidth` _camera) (* (`self.MouseWheelValue`) (`/Game/Core/BP_RotatingCamera.ZoomSpeed` (`self.RotatingCamera`)) -1.0)) (`/Game/Core/BP_RotatingCamera.Zoom_InfLimit` _rotatingcamera) (`/Game/Core/BP_RotatingCamera.Zoom_SupLimit` _rotatingcamera))))))

(fn `UserConstructionScript`)