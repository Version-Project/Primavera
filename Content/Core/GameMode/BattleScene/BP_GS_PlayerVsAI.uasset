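; Battle game state for Player vs. AI mode, which spawns a BP_AI actor and manages turns between the player's Spring faction and the AI's Winter faction.
; EndUnitTurn flags idle units in History, clears expired buffs, then alternates factions and triggers the AI on Winter's turn.
; After every unit acts, it starts a new turn, resetting unit states, until the turn limit prints Game Over.
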(event `self.ReceiveBeginPlay`
  (`KismetSystemLibrary.PrintString` "Player vs. AI" true true (struct :`R` 1.0 :`G` 1.0 :`B` 1.0 :`A` 1.0) 5.0)
  (`parent.ReceiveBeginPlay`)
  (set `self.BattleMode` "NewEnumerator1")
  (bind _returnvalue (`|SpawnActorFromClass` "/Game/AI/BP_AI.BP_AI_C" (`KismetMathLibrary.MakeTransform` (0.0 0.0 0.0)) "AlwaysSpawn" "OverrideRootScale" null null))
  (set `self.AI` _returnvalue))

(fn `EndUnitTurn`
  (bind (_history_turnsactions _history_currturnidx) (break `/Game/Core/S_GameHistory` (`self.History`)))
  (bind (_history_turnsactions_2 _history_currturnidx_2) (break `/Game/Core/S_GameHistory` (`self.History`)))
  (bind (_history_turnsactions_3 _history_currturnidx_3) (break `/Game/Core/S_GameHistory` (`self.History`)))
  (bind (_history_turnsactions_4 _history_currturnidx_4) (break `/Game/Core/S_GameHistory` (`self.History`)))
  (bind (_history_turnsactions_5 _history_currturnidx_5) (break `/Game/Core/S_GameHistory` (`self.History`)))
  (bind (_history_turnsactions_6 _history_currturnidx_6) (break `/Game/Core/S_GameHistory` (`self.History`)))
  (bind (_output_unitsactions _output_currentunitidx) (break `/Game/Core/S_TurnActionsHistory` (`|GetArrayItem` _history_turnsactions_4 _history_currturnidx_4)))
  (bind (_output_unitsactions_2 _output_currentunitidx_2) (break `/Game/Core/S_TurnActionsHistory` (`|GetArrayItem` _history_turnsactions_6 _history_currturnidx_6)))
  (bind (_output_unitsactions_3 _output_currentunitidx_3) (break `/Game/Core/S_TurnActionsHistory` (`|GetArrayItem` _history_turnsactions_5 _history_currturnidx_5)))
  (bind (_output_unitsactions_4 _output_currentunitidx_4) (break `/Game/Core/S_TurnActionsHistory` (`|GetArrayItem` _history_turnsactions_2 _history_currturnidx_2)))
  (bind (_output_unit _output_bmoved _output_battacked _output_bbuffed) (break `/Game/Core/S_UnitActions` (`|GetArrayItem` _output_unitsactions_4 _output_currentunitidx_4)))
  (bind _output_unit_2 (break `/Game/Core/S_UnitActions` (`|GetArrayItem` _output_unitsactions_3 _output_currentunitidx_3)))
  (bind (_output_unit_3 _output_bmoved_2 _output_battacked_2 _output_bbuffed_2 _output_busedcapacity) (break `/Game/Core/S_UnitActions` (`|GetArrayItem` _output_unitsactions_2 _output_currentunitidx_2)))
  (`|ExecutionSequence`
    (:`then_0`
      ;[1 1 1] Check if Unit has acted this turn.
      (if (and (== _output_bmoved_2 false) (== _output_battacked_2 false) (== _output_bbuffed_2 false) (== _output_busedcapacity false))
        (`KismetArrayLibrary.Array_Set` _output_unitsactions_2 _output_currentunitidx_2 (make `/Game/Core/S_UnitActions` _output_unit_3 false false false false true))))
    (:`then_1`
      ;[1 1 1] Unbuff Unit if it has not been buffed this turn.
      (if (and (`/Game/Units/BP_Unit.bBuffed` _output_unit) (!= _output_bbuffed true))
        (set `/Game/Units/BP_Unit.bBuffed` false _output_unit)))
    (:`then_2`
      ;[1 1 1] Increment index to go to the next Unit turn.
      (set `/Game/Units/BP_Unit.bAlreadyBeenPlayed` true _output_unit_2)
      (bind _result (`/Engine/EditorBlueprintResources/StandardMacros.IncrementInt` _output_currentunitidx_3)
        (:`  `
          (if (< _result (`KismetArrayLibrary.Array_Length` _output_unitsactions_3))
            ;[1 1 1] Next Unit turn management.
            (switch `/Game/Core/E_Faction` (`self.CurrFaction`)
              (:`NewEnumerator1`
                (set `self.CurrFaction` "NewEnumerator2")
                (set `self.bAIPlaying` false))
              (:`NewEnumerator2`
                (set `self.CurrFaction` "NewEnumerator1")
                (`/Game/AI/BP_AI.PlayUnitTurn` (`self.AI`) false)
                (set `self.bAIPlaying` true)))
            (`self.DisplayFactionMessage`)
            (`/Game/Core/BP_UIManager.UpdateActionsMenu` (`self.UIManager`) (`|GetArrayItem` _output_unitsactions _output_currentunitidx) :!label _label)
            (`/Game/Core/BP_UIManager.UndisplayActionsMenu` (`self.UIManager`))
            (`self.EndConfirmationStep`)
            (`/Game/UserInterface/Cursor/BP_Cursor.DetachCursorFromUnit` (`self.Cursor`))
            (`self.ResetUIElements`)
            (set `self.CurrPhase` "NewEnumerator0")
            (`/Game/Core/BP_UIManager.UpdateHistoryBoard` (`self.UIManager`) _history_currturnidx)
            (switch `/Game/Core/E_Faction` (`self.CurrFaction`)
              (:`NewEnumerator1`
                _)
              (:`NewEnumerator2`
                (`/Game/Core/BP_UIManager.ChangePlayableUnitsMenuVisibility` (`self.UIManager`) true)))
            (return)
            (else
              ;[1 1 1] Next Play turn management.
              (bind _result_2 (`/Engine/EditorBlueprintResources/StandardMacros.IncrementInt` _history_currturnidx_3)
                (:`  `
                  (if (< _result_2 (`self.MaxTurns`))
                    (`|ExecutionSequence`
                      (:`then_0`
                        (for _array_element (`self.WinterUnits`)
                          (set `/Game/Units/BP_Unit.bAlreadyBeenPlayed` false _array_element)
                          (set `/Game/Units/BP_Unit.bHasBeenStuck` false _array_element)
                          (`/Game/Units/BP_Unit.UpdateStunStatus` _array_element false)))
                      (:`then_1`
                        (for _array_element_2 (`self.SpringUnits`)
                          (set `/Game/Units/BP_Unit.bAlreadyBeenPlayed` false _array_element_2)
                          (set `/Game/Units/BP_Unit.bHasBeenStuck` false _array_element_2)
                          (`/Game/Units/BP_Unit.UpdateStunStatus` _array_element_2 false)))
                      (:`then_2`
                        (`self.DisplayTurnMessage`)
                        (switch `/Game/Core/E_Faction` (`self.CurrFaction`)
                          (:`NewEnumerator1`
                            (`/Game/AI/BP_AI.PlayUnitTurn` (`self.AI`) true)
                            (set `self.bAIPlaying` true)
                            (goto _label))
                          (:`NewEnumerator2`
                            (set `self.bAIPlaying` false)
                            (goto _label)))))
                    (else
                      (`KismetSystemLibrary.PrintString` "Game Over!" true true (struct :`R` 1.0 :`G` 0.96706 :`B` 0.977181 :`A` 1.0) 20.0)
                      (return))))))))))))

(fn `UserConstructionScript`
  (`parent.UserConstructionScript`))