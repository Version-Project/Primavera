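; Game state for a turn-based grid tactics game, alternating Blue and Orange units until the turn limit.
; BeginPlay caches UI, cursor, units, arrows and indexed battlefield blocks, then shows turn and faction banners.
; A History struct records each acting unit and its actions, driving phase confirmation, menu updates and turn advancement.
; It also triggers jumps on playable units and highlights move ranges, though the attack-range highlight loop is unwired.
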(event `self.ReceiveBeginPlay`
  (`|ExecutionSequence`
    (:`then_0`
      (bind _returnvalue (`GameplayStatics.GetActorOfClass` "/Game/Core/BP_UIManager.BP_UIManager_C"))
      (set `self.UIManager` _returnvalue))
    (:`then_1`
      (bind _returnvalue_2 (`GameplayStatics.GetActorOfClass` "/Game/UserInterface/Cursor/BP_Cursor.BP_Cursor_C"))
      (set `self.Cursor` _returnvalue_2))
    (:`then_2`
      (bind _outactors (`GameplayStatics.GetAllActorsOfClass` "/Game/Units/BP_Unit.BP_Unit_C"))
      (for _array_element _outactors
        (switch `/Game/Core/E_Faction` (`/Game/Units/BP_Unit.Faction` _array_element)
          (:`NewEnumerator1`
            (`KismetArrayLibrary.Array_Add` (`self.BlueUnits`) _array_element))
          (:`NewEnumerator2`
            (`KismetArrayLibrary.Array_Add` (`self.OrangeUnits`) _array_element)))))
    (:`then_3`
      (bind _outactors_2 (`GameplayStatics.GetAllActorsOfClass` "/Game/UserInterface/Arrow/BP_Arrow.BP_Arrow_C"))
      (for _array_element_2 _outactors_2
        (`BlueprintMapLibrary.Map_Add` (`self.Arrows`) (`/Game/UserInterface/Arrow/BP_Arrow.Direction` _array_element_2) _array_element_2)))
    (:`then_4`
      (`|ExecutionSequence`
        (:`then_0`
          ;[1 1 1] Fill the Battlefield array with all the BP_Block.
          (bind _outactors_3 (`GameplayStatics.GetAllActorsOfClass` "/Game/Battlefield/BP_Block.BP_Block_C"))
          (for _array_element_3 _outactors_3
            (`BlueprintMapLibrary.Map_Add` (`self.Battlefield`) (`/Game/Battlefield/BP_Block.Index` _array_element_3) _array_element_3)))
        (:`then_1`
          (`self.DisplayTurnMessage`))))))

(event `DisplayTurnMessage`
  (bind _uimanager (`self.UIManager`))
  (bind _playingturnmessage (`/Game/Core/BP_UIManager.PlayingTurnMessage` _uimanager))
  (bind _returnvalue (`WidgetAnimation.GetEndTime` (`/Game/UserInterface/WBP_PlayingTurnMessage.Appear` _playingturnmessage)))
  ;[1 1 1] Event called each time a new turn starts.
  (bind _currentturn (`self.GetCurrentTurn`))
  (`/Game/Core/BP_UIManager.DisplayPlayingTurnMessage` _uimanager _currentturn (`self.MaxTurns`))
  (`|ExecutionSequence`
    (:`then_0`
      (`KismetSystemLibrary.Delay` _returnvalue)
      (`Widget.RemoveFromParent` _playingturnmessage))
    (:`then_1`
      ;;[1 1 1] Display the FactionTurnMessage right before the previous InfoMessage disappears.
      (`KismetSystemLibrary.Delay` (- _returnvalue 1.25))
      (`self.DisplayFactionMessage`))))

(event `DisplayFactionMessage`
  (bind _uimanager (`self.UIManager`))
  (bind _unitturnmessage (`/Game/Core/BP_UIManager.UnitTurnMessage` _uimanager))
  ;[1 1 1] Event called each time the current playing faction changes.
  (`/Game/Core/BP_UIManager.DisplayUnitTurnMessage` _uimanager (`self.CurrFaction`))
  (`KismetSystemLibrary.Delay` (`WidgetAnimation.GetEndTime` (`/Game/UserInterface/WBP_UnitTurnMessage.Appear` _unitturnmessage)))
  (`Widget.RemoveFromParent` _unitturnmessage)
  (`self.SetIfValidUnitsMustJump` true))

(fn `DefineUnitToAct`
  (params (UnitToAct :type "/Game/Units/BP_Unit Object Reference"))
  (bind (_history_turnsactions _history_currturnidx) (break `/Game/Core/S_GameHistory` (`self.History`)))
  (bind (_output_unitsactions _output_currentunitidx) (break `/Game/Core/S_TurnActionsHistory` (`|GetArrayItem` _history_turnsactions _history_currturnidx)))
  (`KismetArrayLibrary.Array_Set` _output_unitsactions _output_currentunitidx (make `/Game/Core/S_UnitActions` UnitToAct))
  (`/Engine/EditorBlueprintResources/StandardMacros.IsValid` UnitToAct
    (:`Is Valid`
      ;[1 1 1] Adding Unit to act.
      (`/Game/Core/BP_UIManager.SetIsActionsMenuEnabled` (`self.UIManager`) true)
      (`/Game/UserInterface/Cursor/BP_Cursor.AttachCursorToUnit` (`self.Cursor`) UnitToAct)
      (`self.SetIfValidUnitsMustJump` false)
      (return))
    (:`Is Not Valid`
      ;[1 1 1] Removing Unit to act.
      (`/Game/Core/BP_UIManager.SetIsActionsMenuEnabled` (`self.UIManager`) false)
      (`/Game/UserInterface/Cursor/BP_Cursor.DetachCursorFromUnit` (`self.Cursor`))
      (`self.SetIfValidUnitsMustJump` true)
      (return))))

(fn `EndConfirmationStep`
  (`/Game/Core/BP_UIManager.DisplayActionsMenu` (`self.UIManager`))
  (set `self.bAwaitingConfirmation` false)
  (return))

(fn `EndCurrentPhase`
  (bind (_history_turnsactions _history_currturnidx) (break `/Game/Core/S_GameHistory` (`self.History`)))
  (bind (_history_turnsactions_2 _history_currturnidx_2) (break `/Game/Core/S_GameHistory` (`self.History`)))
  (bind (_history_turnsactions_3 _history_currturnidx_3) (break `/Game/Core/S_GameHistory` (`self.History`)))
  (bind (_history_turnsactions_4 _history_currturnidx_4) (break `/Game/Core/S_GameHistory` (`self.History`)))
  (bind (_history_turnsactions_5 _history_currturnidx_5) (break `/Game/Core/S_GameHistory` (`self.History`)))
  (bind (_output_unitsactions _output_currentunitidx) (break `/Game/Core/S_TurnActionsHistory` (`|GetArrayItem` _history_turnsactions _history_currturnidx)))
  (bind (_output_unitsactions_2 _output_currentunitidx_2) (break `/Game/Core/S_TurnActionsHistory` (`|GetArrayItem` _history_turnsactions_2 _history_currturnidx_2)))
  (bind (_output_unitsactions_3 _output_currentunitidx_3) (break `/Game/Core/S_TurnActionsHistory` (`|GetArrayItem` _history_turnsactions_3 _history_currturnidx_3)))
  (bind (_output_unitsactions_4 _output_currentunitidx_4) (break `/Game/Core/S_TurnActionsHistory` (`|GetArrayItem` _history_turnsactions_4 _history_currturnidx_4)))
  (bind (_output_unitsactions_5 _output_currentunitidx_5) (break `/Game/Core/S_TurnActionsHistory` (`|GetArrayItem` _history_turnsactions_5 _history_currturnidx_5)))
  (bind (_output_unit _output_bmoved _output_battacked _output_bbuffed) (break `/Game/Core/S_UnitActions` (`|GetArrayItem` _output_unitsactions _output_currentunitidx)))
  (bind (_output_unit_2 _output_bmoved_2 _output_battacked_2 _output_bbuffed_2 _output_busedcapacity) (break `/Game/Core/S_UnitActions` (`|GetArrayItem` _output_unitsactions_2 _output_currentunitidx_2)))
  (bind (_output_unit_3 _output_bmoved_3 _output_battacked_3 _output_bbuffed_3 _output_busedcapacity_2) (break `/Game/Core/S_UnitActions` (`|GetArrayItem` _output_unitsactions_4 _output_currentunitidx_4)))
  (bind (_output_unit_4 _output_bmoved_4 _output_battacked_4 _output_bbuffed_4 _output_busedcapacity_3) (break `/Game/Core/S_UnitActions` (`|GetArrayItem` _output_unitsactions_5 _output_currentunitidx_5)))
  (switch `/Game/Core/E_Phase` (`self.CurrPhase`)
    (:`NewEnumerator1`
      (`KismetArrayLibrary.Array_Set` _output_unitsactions_2 _output_currentunitidx_2 (make `/Game/Core/S_UnitActions` _output_unit_2 true _output_battacked_2 _output_bbuffed_2 _output_busedcapacity)))
    (:`NewEnumerator2`
      (`KismetArrayLibrary.Array_Set` _output_unitsactions_5 _output_currentunitidx_5 (make `/Game/Core/S_UnitActions` _output_unit_4 _output_bmoved_4 true _output_bbuffed_4 _output_busedcapacity_3)))
    (:`NewEnumerator3`
      (`KismetArrayLibrary.Array_Set` _output_unitsactions_4 _output_currentunitidx_4 (make `/Game/Core/S_UnitActions` _output_unit_3 _output_bmoved_3 _output_battacked_3 true _output_busedcapacity_2)))
    (:`NewEnumerator4`
      (`KismetArrayLibrary.Array_Set` _output_unitsactions _output_currentunitidx (make `/Game/Core/S_UnitActions` _output_unit _output_bmoved _output_battacked _output_bbuffed true))))
  (set `self.CurrPhase` "NewEnumerator0")
  (`self.EndConfirmationStep`)
  (`/Game/Core/BP_UIManager.UpdateActionsMenu` (`self.UIManager`) (`|GetArrayItem` _output_unitsactions_3 _output_currentunitidx_3))
  (return))

(fn `EndUnitTurn`
  (bind (_history_turnsactions _history_currturnidx) (break `/Game/Core/S_GameHistory` (`self.History`)))
  (bind (_history_turnsactions_2 _history_currturnidx_2) (break `/Game/Core/S_GameHistory` (`self.History`)))
  (bind (_history_turnsactions_3 _history_currturnidx_3) (break `/Game/Core/S_GameHistory` (`self.History`)))
  (bind (_output_unitsactions _output_currentunitidx) (break `/Game/Core/S_TurnActionsHistory` (`|GetArrayItem` _history_turnsactions _history_currturnidx)))
  (bind (_output_unitsactions_2 _output_currentunitidx_2) (break `/Game/Core/S_TurnActionsHistory` (`|GetArrayItem` _history_turnsactions_3 _history_currturnidx_3)))
  (bind _output_unit (break `/Game/Core/S_UnitActions` (`|GetArrayItem` _output_unitsactions_2 _output_currentunitidx_2)))
  (set `/Game/Units/BP_Unit.bAlreadyBeenPlayed` true _output_unit)
  (bind _result (`/Engine/EditorBlueprintResources/StandardMacros.IncrementInt` _output_currentunitidx_2)
    (:`  `
      (if (< _result (`KismetArrayLibrary.Array_Length` _output_unitsactions_2))
        ;[1 1 1] Next Unit Turn management.
        (switch `/Game/Core/E_Faction` (`self.CurrFaction`)
          (:`NewEnumerator1`
            (set `self.CurrFaction` "NewEnumerator2"))
          (:`NewEnumerator2`
            (set `self.CurrFaction` "NewEnumerator1")))
        (`self.DisplayFactionMessage`)
        (`/Game/Core/BP_UIManager.ChangeMenusFaction` (`self.UIManager`) (`self.CurrFaction`))
        (`/Game/Core/BP_UIManager.UpdateActionsMenu` (`self.UIManager`) (`|GetArrayItem` _output_unitsactions _output_currentunitidx) :!label _label)
        (`self.EndConfirmationStep`)
        (`/Game/UserInterface/Cursor/BP_Cursor.DetachCursorFromUnit` (`self.Cursor`))
        (set `self.CurrPhase` "NewEnumerator0")
        (return)
        (else
          ;[1 1 1] Next Play Turn management.
          (bind _result_2 (`/Engine/EditorBlueprintResources/StandardMacros.IncrementInt` _history_currturnidx_2)
            (:`  `
              (if (< _result_2 (`self.MaxTurns`))
                (`|ExecutionSequence`
                  (:`then_0`
                    (for _array_element (`self.BlueUnits`)
                      (set `/Game/Units/BP_Unit.bAlreadyBeenPlayed` false _array_element)))
                  (:`then_1`
                    (for _array_element_2 (`self.OrangeUnits`)
                      (set `/Game/Units/BP_Unit.bAlreadyBeenPlayed` false _array_element_2)))
                  (:`then_2`
                    (`self.DisplayTurnMessage`)
                    (goto _label)))
                (else
                  (`KismetSystemLibrary.PrintString` "Game Over!" true true (struct :`R` 1.0 :`G` 0.96706 :`B` 0.977181 :`A` 1.0) 20.0)
                  (return))))))))))

(fn `GetCurrentTurn`
  (returns (CurrentTurn :type Integer))
  (bind (_history_turnsactions _history_currturnidx) (break `/Game/Core/S_GameHistory` (`self.History`)))
  (return (+ _history_currturnidx 1)))

(fn `GetUnitToAct`
  (returns (UnitToAct :type "/Game/Units/BP_Unit Object Reference"))
  (bind (_history_turnsactions _history_currturnidx) (break `/Game/Core/S_GameHistory` (`self.History`)))
  (bind (_output_unitsactions _output_currentunitidx) (break `/Game/Core/S_TurnActionsHistory` (`|GetArrayItem` _history_turnsactions _history_currturnidx)))
  (bind _output_unit (break `/Game/Core/S_UnitActions` (`|GetArrayItem` _output_unitsactions _output_currentunitidx)))
  (return _output_unit))

(fn `GoToConfirmationStep`
  (params (Phase :type "/Game/Core/E_Phase Enum" :default "NewEnumerator0") (ClickedBlock :type "/Game/Battlefield/BP_Block Object Reference"))
  (locals (Block :type "/Game/Battlefield/BP_Block Object Reference"))
  (set `local.Block` ClickedBlock)
  (`/Game/Core/BP_UIManager.DisplayConfirmMenu` (`self.UIManager`) Phase)
  (switch `/Game/Core/E_Phase` Phase
    (:`NewEnumerator1`
      (`self.ShowArrow` "NewEnumerator0" (`local.Block`)))
    (:`NewEnumerator2`
      _)
    (:`NewEnumerator3`
      _)
    (:`NewEnumerator4`
      _)
    (:`NewEnumerator7`
      _))
  (set `self.bAwaitingConfirmation` true)
  (return))

(fn `HasUnitActed`
  (returns (HasActed :type Boolean))
  (bind (_history_turnsactions _history_currturnidx) (break `/Game/Core/S_GameHistory` (`self.History`)))
  (bind (_output_unitsactions _output_currentunitidx) (break `/Game/Core/S_TurnActionsHistory` (`|GetArrayItem` _history_turnsactions _history_currturnidx)))
  (bind (_output_unit _output_bmoved _output_battacked _output_bbuffed _output_busedcapacity) (break `/Game/Core/S_UnitActions` (`|GetArrayItem` _output_unitsactions _output_currentunitidx)))
  (return (or _output_bmoved _output_battacked _output_bbuffed _output_busedcapacity)))

(fn `HideActionRange`
  (for _index (range 176)
    (`SceneComponent.SetVisibility` (`/Game/Battlefield/BP_Block.ActionRangePlane` (`BlueprintMapLibrary.Map_Find` (`self.Battlefield`) _index)) false false))
  (return))

(fn `HideArrow`
  (params (Direction :type "/Game/Core/E_Direction Enum" :default "NewEnumerator0"))
  (`SceneComponent.SetVisibility` (`/Game/UserInterface/Arrow/BP_Arrow.SM_Arrow` (`BlueprintMapLibrary.Map_Find` (`self.Arrows`) Direction)) false false)
  (return))

(fn `ResetUIElements`
  (`|ExecutionSequence`
    (:`then_0`
      (`self.HideActionRange`))
    (:`then_1`
      ;[1 1 1] Reset all Arrows
      (bind _enumvalue (foreach `/Game/Core/E_Direction` false)
        (:`LoopBody`
          (`self.HideArrow` _enumvalue))))
    (:`then_2`
      (return))))

(fn `SetIfValidUnitsMustJump`
  (params (bMustJump :type Boolean))
  (if bMustJump
    (switch `/Game/Core/E_Faction` (`self.CurrFaction`)
      (:`NewEnumerator1`
        (for _array_element (`self.BlueUnits`)
          (if (not (`/Game/Units/BP_Unit.bAlreadyBeenPlayed` _array_element))
            (set `/Game/Units/BP_Unit.bMustJump` true _array_element)
            (`/Game/Units/BP_Unit.TriggerJump` _array_element)))
        (return))
      (:`NewEnumerator2`
        (for _array_element_2 (`self.OrangeUnits`)
          (if (not (`/Game/Units/BP_Unit.bAlreadyBeenPlayed` _array_element_2))
            (set `/Game/Units/BP_Unit.bMustJump` true _array_element_2)
            (`/Game/Units/BP_Unit.TriggerJump` _array_element_2)))
        (return)))
    (else
      (switch `/Game/Core/E_Faction` (`self.CurrFaction`)
        (:`NewEnumerator1`
          (for _array_element_3 (`self.BlueUnits`)
            (set `/Game/Units/BP_Unit.bMustJump` false _array_element_3))
          (return))
        (:`NewEnumerator2`
          (for _array_element_4 (`self.OrangeUnits`)
            (set `/Game/Units/BP_Unit.bMustJump` false _array_element_4))
          (return))))))

(fn `ShowArrow`
  (params (Direction :type "/Game/Core/E_Direction Enum" :default "NewEnumerator0") (Block :type "/Game/Battlefield/BP_Block Object Reference"))
  (locals (Cube :type "StaticMeshComponent Object Reference") (Coords :type "Vector Structure"))
  (bind (_returnvalue_x _returnvalue_y) (`KismetMathLibrary.BreakVector` (`SceneComponent.K2_GetComponentLocation` (`local.Cube`))))
  (bind (_returnvalue_x_2 _returnvalue_y_2) (`KismetMathLibrary.BreakVector` (`SceneComponent.K2_GetComponentLocation` (`local.Cube`))))
  (bind (_returnvalue_x_3 _returnvalue_y_3) (`KismetMathLibrary.BreakVector` (`SceneComponent.K2_GetComponentLocation` (`local.Cube`))))
  (bind (_returnvalue_x_4 _returnvalue_y_4) (`KismetMathLibrary.BreakVector` (`SceneComponent.K2_GetComponentLocation` (`local.Cube`))))
  (bind (_returnvalue_x_5 _returnvalue_y_5) (`KismetMathLibrary.BreakVector` (`SceneComponent.K2_GetComponentLocation` (`local.Cube`))))
  (bind _sm_arrow (`/Game/UserInterface/Arrow/BP_Arrow.SM_Arrow` (`BlueprintMapLibrary.Map_Find` (`self.Arrows`) Direction)))
  (set `local.Cube` (`/Game/Battlefield/BP_Block.Cube` Block))
  (switch `/Game/Core/E_Direction` Direction
    (:`NewEnumerator0`
      (set `local.Coords` (`KismetMathLibrary.MakeVector` _returnvalue_x_5 _returnvalue_y_5 100.0)))
    (:`NewEnumerator1`
      (set `local.Coords` (`KismetMathLibrary.MakeVector` _returnvalue_x_2 (- _returnvalue_y_2 100.0) 50.0)))
    (:`NewEnumerator2`
      (set `local.Coords` (`KismetMathLibrary.MakeVector` _returnvalue_x_3 (+ _returnvalue_y_3 100.0) 50.0)))
    (:`NewEnumerator3`
      (set `local.Coords` (`KismetMathLibrary.MakeVector` (- _returnvalue_x 100.0) _returnvalue_y 50.0)))
    (:`NewEnumerator4`
      (set `local.Coords` (`KismetMathLibrary.MakeVector` (+ _returnvalue_x_4 100.0) _returnvalue_y_4 50.0))))
  (`SceneComponent.K2_SetWorldLocation` _sm_arrow (`local.Coords`) false false)
  (`SceneComponent.SetVisibility` _sm_arrow true false)
  (return))

(fn `ShowAttackRange`
  (locals (CurrBlockCoords :type "/Game/Core/S_Coords Structure") (AbsoluteX :type Integer) (AbsoluteY :type Integer))
  (`self.HideActionRange`)
  (bind _unittoact (`self.GetUnitToAct`))
  (bind _coords (`/Game/Core/BP_CoordsFunctionLibrary.GetStructCoordsFromIndex` (`/Game/Battlefield/BP_Block.Index` (`/Game/Units/BP_Unit.BindedBlock` _unittoact))))
  (set `local.CurrBlockCoords` _coords))

(fn `ShowMoveRange`
  (locals (CurrBlockCoords :type "/Game/Core/S_Coords Structure") (AbsoluteX :type Integer) (AbsoluteY :type Integer))
  (`self.HideActionRange`)
  (bind _unittoact (`self.GetUnitToAct`))
  (bind _coords (`/Game/Core/BP_CoordsFunctionLibrary.GetStructCoordsFromIndex` (`/Game/Battlefield/BP_Block.Index` (`/Game/Units/BP_Unit.BindedBlock` _unittoact))))
  (set `local.CurrBlockCoords` _coords)
  (for _array_element (`/Game/Units/BP_Unit.MoveRange` _unittoact)
    (bind _absolutecoords (`/Game/Core/BP_CoordsFunctionLibrary.GetAbsoluteCoordsFromRelatives` (`local.CurrBlockCoords`) _array_element))
    (set `local.AbsoluteX` (break `/Game/Core/S_Coords` _absolutecoords))
    (bind _output_get (set `local.AbsoluteY` (`.Y_6_2DC6362D4EE28ABEA56491A3230A1BE6` (break `/Game/Core/S_Coords` _absolutecoords))))
    (bind _binbounds (`/Game/Core/BP_CoordsFunctionLibrary.AreCoordsInBounds` (break `/Game/Core/S_Coords` _absolutecoords) _output_get))
    (if _binbounds
      (bind _index (`/Game/Core/BP_CoordsFunctionLibrary.GetBlockIndex` (`local.AbsoluteX`) (`local.AbsoluteY`)))
      (bind _value (`BlueprintMapLibrary.Map_Find` (`self.Battlefield`) _index))
      ;[1 1 1] If there is already an Unit on the block, it should be out of the MoveRange.
      (`/Engine/EditorBlueprintResources/StandardMacros.IsValid` (`/Game/Battlefield/BP_Block.BindedUnit` _value)
        (:`Is Not Valid`
          (bind _actionrangeplane (`/Game/Battlefield/BP_Block.ActionRangePlane` _value))
          (`PrimitiveComponent.SetMaterial` _actionrangeplane 0 "/Game/Battlefield/M_MoveRange.M_MoveRange")
          (`SceneComponent.SetVisibility` _actionrangeplane true false)))))
  (return))

(fn `UserConstructionScript`
  (bind _history_turnsactions (break `/Game/Core/S_GameHistory` (`self.History`)))
  (`KismetArrayLibrary.Array_Resize` _history_turnsactions (`self.MaxTurns`)))