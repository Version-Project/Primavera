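; UI manager for a turn-based unit tactics game, owning the menus, turn messages, score and history board.
; BeginPlay creates the widgets, then exposed functions swap the actions and confirm menus, restyle menus per faction and refresh the HUD.
; Action shortcuts click the enabled actions menu or, while GameState awaits confirmation, confirm the matching phase; GoBack forwards to the confirm menu.
; BlockStatus is created but never added to the viewport here.
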(event `self.ReceiveBeginPlay`
  (bind _asbp_game_state (cast `/Game/Core/GameMode/BP_GameState` (`GameplayStatics.GetGameState`)))
  (set `self.GameState` _asbp_game_state)
  (`|ExecutionSequence`
    (:`then_0`
      (bind _returnvalue (`|CreateWidget` "/Game/UserInterface/PlayableUnitsMenu/WBP_PlayableUnitsMenu.WBP_PlayableUnitsMenu_C"))
      (bind _output_get (set `self.PlayableUnitsMenu` _returnvalue))
      (`UserWidget.AddToViewport` _output_get 0))
    (:`then_1`
      (bind _returnvalue_2 (`|CreateWidget` "/Game/UserInterface/WBP_ActionsMenu.WBP_ActionsMenu_C"))
      (bind _output_get_2 (set `self.ActionsMenu` _returnvalue_2))
      (`UserWidget.AddToViewport` _output_get_2 0)
      (`Widget.SetIsEnabled` _output_get_2 false))
    (:`then_2`
      (bind _returnvalue_3 (`|CreateWidget` "/Game/UserInterface/WBP_ConfirmMenu.WBP_ConfirmMenu_C"))
      (bind _output_get_3 (set `self.ConfirmMenu` _returnvalue_3))
      (`UserWidget.AddToViewport` _output_get_3 0)
      (`Widget.RemoveFromParent` _output_get_3)
      (`self.ChangeMenusFaction` "NewEnumerator2"))
    (:`then_3`
      (bind _returnvalue_4 (`|CreateWidget` "/Game/UserInterface/WBP_PlayingTurnMessage.WBP_PlayingTurnMessage_C"))
      (set `self.PlayingTurnMessage` _returnvalue_4))
    (:`then_4`
      (bind _returnvalue_5 (`|CreateWidget` "/Game/UserInterface/WBP_UnitTurnMessage.WBP_UnitTurnMessage_C"))
      (set `self.UnitTurnMessage` _returnvalue_5))
    (:`then_5`
      (bind _returnvalue_6 (`|CreateWidget` "/Game/UserInterface/WBP_Score.WBP_Score_C"))
      (bind _output_get_4 (set `self.Score` _returnvalue_6))
      (`UserWidget.AddToViewport` _output_get_4 0))
    (:`then_6`
      (bind _returnvalue_7 (`|CreateWidget` "/Game/UserInterface/HistoryBoard/WBP_HistoryBoard.WBP_HistoryBoard_C"))
      (bind _output_get_5 (set `self.HistoryBoard` _returnvalue_7))
      (`UserWidget.AddToViewport` _output_get_5 0))
    (:`then_7`
      (bind _returnvalue_8 (`|CreateWidget` "/Game/UserInterface/WBP_BlockStatus.WBP_BlockStatus_C"))
      (bind _output_get_6 (set `self.BlockStatus` _returnvalue_8)))))

(event `InputAction|InputAction_Move`
  (params (Key :type "Key Structure"))
  (bind _confirmmenu (`self.ConfirmMenu`))
  (bind _gamestate (`self.GameState`))
  ;[1 1 1] Move shortcut
  (:`Pressed`
    (if (`/Game/Core/GameMode/BP_GameState.bAwaitingConfirmation` _gamestate)
      (if (`|EnumEquality` "NewEnumerator1" (`/Game/Core/GameMode/BP_GameState.CurrPhase` _gamestate))
        (bind _bequals (`/Game/UserInterface/WBP_ConfirmMenu.IsShortcutEqualToLetter` _confirmmenu "M"))
        (if _bequals
          (`/Game/UserInterface/WBP_ConfirmMenu.HandleMoveButtonConfirm` _confirmmenu)))
      (elif (`Widget.bIsEnabled` (`self.ActionsMenu`))
        (`/Game/UserInterface/WBP_ActionsMenu.HandleMoveButtonClick` (`self.ActionsMenu`))))))

(event `InputAction|InputAction_Attack`
  (params (Key :type "Key Structure"))
  (bind _gamestate (`self.GameState`))
  (bind _confirmmenu (`self.ConfirmMenu`))
  ;[1 1 1] Attack shortcut
  (:`Pressed`
    (if (`/Game/Core/GameMode/BP_GameState.bAwaitingConfirmation` _gamestate)
      (if (`|EnumEquality` "NewEnumerator2" (`/Game/Core/GameMode/BP_GameState.CurrPhase` _gamestate))
        (bind _bequals (`/Game/UserInterface/WBP_ConfirmMenu.IsShortcutEqualToLetter` _confirmmenu "A"))
        (if _bequals
          (`/Game/UserInterface/WBP_ConfirmMenu.HandleAttackButtonConfirm` _confirmmenu)))
      (elif (`Widget.bIsEnabled` (`self.ActionsMenu`))
        (`/Game/UserInterface/WBP_ActionsMenu.HandleAttackButtonClick` (`self.ActionsMenu`))))))

(event `InputAction|InputAction_Buff`
  (params (Key :type "Key Structure"))
  (bind _confirmmenu (`self.ConfirmMenu`))
  (bind _gamestate (`self.GameState`))
  ;[1 1 1] Buff shortcut
  (:`Pressed`
    (if (`/Game/Core/GameMode/BP_GameState.bAwaitingConfirmation` _gamestate)
      (if (`|EnumEquality` "NewEnumerator3" (`/Game/Core/GameMode/BP_GameState.CurrPhase` _gamestate))
        (bind _bequals (`/Game/UserInterface/WBP_ConfirmMenu.IsShortcutEqualToLetter` _confirmmenu "B"))
        (if _bequals
          (`/Game/UserInterface/WBP_ConfirmMenu.HandleBuffButtonConfirm` _confirmmenu)))
      (elif (`Widget.bIsEnabled` (`self.ActionsMenu`))
        (`/Game/UserInterface/WBP_ActionsMenu.HandleBuffButtonClick` (`self.ActionsMenu`))))))

(event `InputAction|InputAction_Capacity`
  (params (Key :type "Key Structure"))
  (bind _confirmmenu (`self.ConfirmMenu`))
  (bind _gamestate (`self.GameState`))
  ;[1 1 1] Capacity shortcut
  (:`Pressed`
    (if (`/Game/Core/GameMode/BP_GameState.bAwaitingConfirmation` _gamestate)
      (if (`|EnumEquality` "NewEnumerator4" (`/Game/Core/GameMode/BP_GameState.CurrPhase` _gamestate))
        (bind _bequals (`/Game/UserInterface/WBP_ConfirmMenu.IsShortcutEqualToLetter` _confirmmenu "C"))
        (if _bequals
          (`/Game/UserInterface/WBP_ConfirmMenu.HandleCapacityButtonConfirm` _confirmmenu)))
      (elif (`Widget.bIsEnabled` (`self.ActionsMenu`))
        (`/Game/UserInterface/WBP_ActionsMenu.HandleCapacityButtonClick` (`self.ActionsMenu`))))))

(event `InputAction|InputAction_EndTurn`
  (params (Key :type "Key Structure"))
  (bind _confirmmenu (`self.ConfirmMenu`))
  (bind _gamestate (`self.GameState`))
  ;[1 1 1] EndTurn shortcut
  (:`Pressed`
    (if (`/Game/Core/GameMode/BP_GameState.bAwaitingConfirmation` _gamestate)
      (if (`|EnumEquality` "NewEnumerator7" (`/Game/Core/GameMode/BP_GameState.CurrPhase` _gamestate))
        (bind _bequals (`/Game/UserInterface/WBP_ConfirmMenu.IsShortcutEqualToLetter` _confirmmenu "E"))
        (if _bequals
          (`/Game/UserInterface/WBP_ConfirmMenu.HandleEndTurnButtonConfirm` _confirmmenu)))
      (elif (`Widget.bIsEnabled` (`self.ActionsMenu`))
        (`/Game/UserInterface/WBP_ActionsMenu.HandleEndTurnButtonClick` (`self.ActionsMenu`))))))

(event `InputAction|InputAction_GoBack`
  (params (Key :type "Key Structure"))
  ;[1 1 1] GoBack shortcut
  (:`Pressed`
    (`/Game/UserInterface/WBP_ConfirmMenu.HandleGoBackButtonClick` (`self.ConfirmMenu`))))

(fn `ChangeMenusFaction`
  (params (Faction :type "/Game/Core/E_Faction Enum" :default "NewEnumerator0"))
  (`self.UndisplayActionsMenu` false)
  (`/Game/UserInterface/WBP_ActionsMenu.SetButtonsStyle` (`self.ActionsMenu`) Faction)
  (`/Game/UserInterface/WBP_ConfirmMenu.SetButtonsStyle` (`self.ConfirmMenu`) Faction)
  (`/Game/UserInterface/PlayableUnitsMenu/WBP_PlayableUnitsMenu.ChangeCurrentFaction` (`self.PlayableUnitsMenu`) Faction)
  (return))

(fn `ChangePlayableUnitsMenuVisibility`
  (params (bDisplay :type Boolean))
  (`/Game/UserInterface/PlayableUnitsMenu/WBP_PlayableUnitsMenu.ChangeVisibility` (`self.PlayableUnitsMenu`) bDisplay)
  (return))

(fn `ChangePlayableUnitsMenuWhenBlockClicking`
  (bind _hasacted (`/Game/Core/GameMode/BP_GameState.HasUnitActed` (`self.GameState`)))
  (if (and (not _hasacted) (`Widget.IsInViewport` (`self.ConfirmMenu`)))
    (`self.ChangePlayableUnitsMenuVisibility` true)
    (return)
    (else
      (return))))

(fn `DisplayActionsMenu`
  (params (bLaunchAnimation :type Boolean))
  (bind _actionsmenu (`self.ActionsMenu`))
  (bind _actionsmenu_2 (`self.ActionsMenu`))
  (if bLaunchAnimation
    (if (not (`Widget.bIsEnabled` _actionsmenu))
      (`/Game/UserInterface/WBP_ActionsMenu.LaunchAppearAnimation` _actionsmenu)
      (return))
    (elif (not (`Widget.IsInViewport` _actionsmenu_2))
      (`UserWidget.AddToViewport` _actionsmenu_2 0)
      (`Widget.RemoveFromParent` (`self.ConfirmMenu`))
      (return))))

(fn `DisplayConfirmMenu`
  (params (Phase :type "/Game/Core/E_Phase Enum" :default "NewEnumerator0"))
  (bind _confirmmenu (`self.ConfirmMenu`))
  (if (not (`Widget.IsInViewport` _confirmmenu))
    (`UserWidget.AddToViewport` _confirmmenu 0)
    (`/Game/UserInterface/WBP_ConfirmMenu.SetActionText` _confirmmenu Phase)
    (`Widget.RemoveFromParent` (`self.ActionsMenu`))
    (bind _unittoact (`/Game/Core/GameMode/BP_GameState.GetUnitToAct` (`self.GameState`)))
    (`/Engine/EditorBlueprintResources/StandardMacros.IsValid` _unittoact
      (:`Is Valid`
        (bind _hasacted (`/Game/Core/GameMode/BP_GameState.HasUnitActed` (`self.GameState`)))
        (if _hasacted
          (return)
          (else
            (`self.ChangePlayableUnitsMenuVisibility` false)
            (return)))))))

(fn `DisplayPlayingTurnMessage`
  (params (CurrentTurn :type Integer) (MaxTurns :type Integer))
  (bind _playingturnmessage (`self.PlayingTurnMessage`))
  (`UserWidget.AddToViewport` _playingturnmessage 0)
  (`/Game/UserInterface/WBP_PlayingTurnMessage.DisplayMessage` _playingturnmessage (`KismetStringLibrary.Concat_StrStr` "TURN " (`KismetStringLibrary.Conv_IntToString` CurrentTurn) " / " (`KismetStringLibrary.Conv_IntToString` MaxTurns)))
  (`/Game/UserInterface/WBP_Score.UpdateTurn` (`self.Score`))
  (return))

(fn `DisplayUnitTurnMessage`
  (params (Faction :type "/Game/Core/E_Faction Enum" :default "NewEnumerator0"))
  (bind _unitturnmessage (`self.UnitTurnMessage`))
  (`UserWidget.AddToViewport` _unitturnmessage 0)
  (`/Game/UserInterface/WBP_UnitTurnMessage.DisplayFactionTurn` _unitturnmessage Faction)
  (return))

(fn `SetIsActionsMenuEnabled`
  (params (IsEnabled :type Boolean))
  (`Widget.SetIsEnabled` (`self.ActionsMenu`) IsEnabled)
  (return))

(fn `UndisplayActionsMenu`
  (params (bLaunchAnimation :type Boolean))
  (bind _actionsmenu (`self.ActionsMenu`))
  (if bLaunchAnimation
    (if (`Widget.bIsEnabled` (`self.ActionsMenu`))
      (`UserWidget.PlayAnimation` _actionsmenu (`/Game/UserInterface/WBP_ActionsMenu.Appear` _actionsmenu) 0.0 1 "Reverse" 1.0 false)
      (`Widget.SetIsEnabled` (`self.ActionsMenu`) false :!label _label)
      (return))
    (else
      (`/Game/UserInterface/WBP_ActionsMenu.MakeMenuGoOffScreen` (`self.ActionsMenu`))
      (goto _label))))

(fn `UpdateActionsMenu`
  (params (UnitActions :type "/Game/Core/S_UnitActions Structure"))
  (`/Game/UserInterface/WBP_ActionsMenu.UpdateMenu` (`self.ActionsMenu`) UnitActions)
  (return))

(fn `UpdateHistoryBoard`
  (params (TurnToDisplay :type Integer))
  (`/Game/UserInterface/HistoryBoard/WBP_HistoryBoard.UpdateBoard` (`self.HistoryBoard`) TurnToDisplay)
  (return))

(fn `UpdateHUDScores`
  (`/Game/UserInterface/WBP_Score.UpdateHUDScores` (`self.Score`))
  (return))

(fn `UserConstructionScript`)