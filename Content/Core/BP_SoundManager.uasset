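; BP_SoundManager is the audio manager that plays ambient music and unit action sounds for a faction-based, turn-based game.
; On BeginPlay it waits for the UI manager's turn message animations to nearly finish, then starts the environment music at zero volume.
; PlayActionSound picks an event from the unit's phase, faction and class, passes its buffed state as the AttackType parameter, plays it and prints a debug message.
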(event `self.ReceiveBeginPlay`
  (bind _env_music (`self.ENV_Music`))
  (bind _returnvalue (`GameplayStatics.GetActorOfClass` "/Game/Core/BP_UIManager.BP_UIManager_C"))
  (bind _output_get (set `self.UIManager` _returnvalue))
  (`KismetSystemLibrary.Delay` (+ (`WidgetAnimation.GetEndTime` (`/Game/UserInterface/WBP_PlayingTurnMessage.Appear` (`/Game/Core/BP_UIManager.PlayingTurnMessage` _output_get))) -1.25 (`WidgetAnimation.GetEndTime` (`/Game/UserInterface/WBP_UnitTurnMessage.Appear` (`/Game/Core/BP_UIManager.UnitTurnMessage` _output_get))) 0.5))
  (`FMODAudioComponent.SetVolume` _env_music 0.0)
  (`FMODAudioComponent.Play` _env_music))

(fn `PlayActionSound`
  (params (Unit :type "/Game/Units/BP_Unit Object Reference") (Phase :type "/Game/Core/E_Phase Enum" :default "NewEnumerator0"))
  (locals (Class :type "/Game/Core/E_Class Enum" :default "NewEnumerator0") (Faction :type "/Game/Core/E_Faction Enum" :default "NewEnumerator0") (bBuffed :type Boolean :default false))
  (bind _u_action (`self.U_Action`))
  (set `local.Class` (`/Game/Units/BP_Unit.Class` Unit))
  (set `local.Faction` (`/Game/Units/BP_Unit.Faction` Unit))
  (set `local.bBuffed` (`/Game/Units/BP_Unit.bBuffed` Unit))
  (`|ExecutionSequence`
    (:`then_0`
      (switch `/Game/Core/E_Phase` (`local.Phase`)
        (:`NewEnumerator2`
          (switch `/Game/Core/E_Faction` (`local.Faction`)
            (:`NewEnumerator1`
              (switch `/Game/Core/E_Class` (`local.Class`)
                (:`NewEnumerator0`
                  (set `self.ActionEvent` "/Game/FMOD/Events/Units/U_Winter/U_WI_Sniper/U_WI_SNI_Attack.U_WI_SNI_Attack"))
                (:`NewEnumerator1`
                  (set `self.ActionEvent` "/Game/FMOD/Events/Units/U_Winter/U_WI_Protector/U_WI_PRO_Attack.U_WI_PRO_Attack"))
                (:`NewEnumerator2`
                  (set `self.ActionEvent` "/Game/FMOD/Events/Units/U_Winter/U_WI_Inlayer/U_WI_INL_Attack.U_WI_INL_Attack"))))
            (:`NewEnumerator2`
              (switch `/Game/Core/E_Class` (`local.Class`)
                (:`NewEnumerator0`
                  (set `self.ActionEvent` "/Game/FMOD/Events/Units/U_Spring/U_SP_Sniper/U_SP_SNI_Attack.U_SP_SNI_Attack"))
                (:`NewEnumerator1`
                  (set `self.ActionEvent` "/Game/FMOD/Events/Units/U_Spring/U_SP_Protector/U_SP_PRO_Attack.U_SP_PRO_Attack"))
                (:`NewEnumerator2`
                  (set `self.ActionEvent` "/Game/FMOD/Events/Units/U_Spring/U_SP_Inlayer/U_SP_INL_Attack.U_SP_INL_Attack"))))))
        (:`NewEnumerator4`
          (switch `/Game/Core/E_Faction` (`local.Faction`)
            (:`NewEnumerator1`
              (switch `/Game/Core/E_Class` (`local.Class`)
                (:`NewEnumerator0`
                  (set `self.ActionEvent` "/Game/FMOD/Events/Units/U_Winter/U_WI_Sniper/U_WI_SNI_Capacity.U_WI_SNI_Capacity"))
                (:`NewEnumerator1`
                  (set `self.ActionEvent` "/Game/FMOD/Events/Units/U_Winter/U_WI_Protector/U_WI_PRO_Capacity.U_WI_PRO_Capacity"))
                (:`NewEnumerator2`
                  (set `self.ActionEvent` "/Game/FMOD/Events/Units/U_Winter/U_WI_Inlayer/U_WI_INL_Capacity.U_WI_INL_Capacity"))))
            (:`NewEnumerator2`
              (switch `/Game/Core/E_Class` (`local.Class`)
                (:`NewEnumerator0`
                  (set `self.ActionEvent` "/Game/FMOD/Events/Units/U_Spring/U_SP_Sniper/U_SP_SNI_Capacity.U_SP_SNI_Capacity"))
                (:`NewEnumerator1`
                  (set `self.ActionEvent` "/Game/FMOD/Events/Units/U_Spring/U_SP_Protector/U_SP_PRO_Capacity.U_SP_PRO_Capacity"))
                (:`NewEnumerator2`
                  (set `self.ActionEvent` "/Game/FMOD/Events/Units/U_Spring/U_SP_Inlayer/U_SP_INL_Capacity.U_SP_INL_Capacity"))))))))
    (:`then_1`
      (`FMODAudioComponent.SetEvent` (`self.U_Action`) (`self.ActionEvent`))
      (`FMODAudioComponent.SetParameter` (`self.U_Action`) "AttackType" (`KismetMathLibrary.Conv_BoolToDouble` (`local.bBuffed`)))
      (`FMODAudioComponent.Play` _u_action)
      (`KismetSystemLibrary.PrintString` (`KismetStringLibrary.Concat_StrStr` "Playing sound: \"" (`KismetSystemLibrary.GetDisplayName` (`FMODAudioComponent.Event` _u_action)) "\"") true true (struct :`R` 0.964954 :`G` 1.0 :`A` 1.0) 4.0)
      (return))))

(fn `UserConstructionScript`)