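; BP_Field builds the battlefield at BeginPlay, spawning a grid of BP_Block tiles 100 units apart and giving each its coordinates.
; As each tile spawns, SetSpawns marks mirrored Spring and Winter territories at opposite X edges, with incrustation fading outward from the middle row.
; PlayerSpawn binds existing Protector, Inlayer and Sniper actors to fixed tiles by faction.
; Protectors also bind to any tile directly beneath them by exact location match.
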(event `self.ReceiveBeginPlay`
  (bind _gridsize_x (`KismetMathLibrary.BreakVector2D` (`self.GridSize`)))
  (bind (_gridsize_x_2 _gridsize_y) (`KismetMathLibrary.BreakVector2D` (`self.GridSize`)))
  (bind _returnvalue_location (`KismetMathLibrary.BreakTransform` (`SceneComponent.K2_GetComponentToWorld` (`self.DefaultSceneRoot`))))
  (bind _returnvalue (+ (`KismetMathLibrary.MakeVector` (* (`self.X`) 100) (* (`self.Y`) 100)) _returnvalue_location))
  ;[1 1 1] Foreach Tiles
  (for _index (range (`KismetMathLibrary.Round` _gridsize_x))
    (set `self.X` _index)
    (for _index_2 (range (`KismetMathLibrary.Round` _gridsize_y))
      (set `self.Y` _index_2)
      (bind _returnvalue_2 (`|SpawnActorFromClass` "/Game/Battlefield/Block/BP_Block.BP_Block_C" (`KismetMathLibrary.MakeTransform` _returnvalue) "Undefined" "OverrideRootScale" null null))
      (set `self.CurrentBlock` _returnvalue_2)
      (`|ExecutionSequence`
        (:`then_0`
          (set `/Game/Battlefield/Block/BP_Block.Index` (`self.Index`) (`self.CurrentBlock`))
          (bind _result (`/Engine/EditorBlueprintResources/StandardMacros.IncrementInt` (`self.Index`))
            (:`  `
              (set `self.Index` _result))))
        (:`then_1`
          (set `/Game/Battlefield/Block/BP_Block.Coords` (make `/Game/Core/S_Coords` (`self.X`) (`self.Y`)) (`self.CurrentBlock`)))
        (:`then_2`
          (`self.Set Spawns`))
        (:`then_3`
          (bind _outactors (`GameplayStatics.GetAllActorsOfClass` "/Game/Units/BP_Protector.BP_Protector_C"))
          (for _array_element _outactors
            (if (== (`SceneComponent.K2_GetComponentLocation` (`/Game/Units/BP_Unit.DefaultSceneRoot` _array_element)) (+ _returnvalue (0.0 0.0 75.0)))
              (set `/Game/Battlefield/Block/BP_Block.BindedUnit` _array_element (`self.CurrentBlock`)))))))))

(fn `PlayerSpawn`
  (params (XGridValue :type Integer) (Side :type "/Game/Core/E_Faction Enum" :default "NewEnumerator0"))
  (locals (Direction :type Integer) (GridHorizontalSize :type Integer) (Faction :type "/Game/Core/E_Faction Enum"))
  (`|ExecutionSequence`
    (:`then_0`
      (set `local.GridHorizontalSize` XGridValue))
    (:`then_1`
      (set `local.Faction` Side))
    (:`then_2`
      (switch `/Game/Core/E_Faction` (`local.Faction`)
        (:`NewEnumerator1`
          (set `local.Direction` -1))
        (:`NewEnumerator2`
          (set `local.Direction` 1))))
    (:`then_3`
      (`|ExecutionSequence`
        (:`then_0`
          (bind _caseselected (`self.SelectCaseFromMiddleLeft` (+ (`local.GridHorizontalSize`) (* (`local.Direction`) 5)))))
        (:`then_1`
          (bind _caseselected_2 (`self.SelectCaseFromMiddleLeft` (+ (`local.GridHorizontalSize`) (* (`local.Direction`) 4)) 1)))
        (:`then_2`
          (bind _caseselected_3 (`self.SelectCaseFromMiddleLeft` (+ (`local.GridHorizontalSize`) (* (`local.Direction`) 4)) -1)))
        (:`then_3`
          (if _caseselected
            (`self.SetBindedBlock` "/Game/Units/BP_Protector.BP_Protector_C" (`local.Faction`))
            (elif _caseselected_2
              (`self.SetBindedBlock` "/Game/Units/BP_Inlayer.BP_Inlayer_C" (`local.Faction`))
              (elif _caseselected_3
                (`self.SetBindedBlock` "/Game/Units/BP_Sniper.BP_Sniper_C" (`local.Faction`))))))))))

(fn `SelectCaseFromMiddleLeft`
  (params (X :type Integer) (Y :type Integer))
  (returns (CaseSelected :type Boolean))
  (bind (_gridsize_x _gridsize_y) (`KismetMathLibrary.BreakVector2D` (`self.GridSize`)))
  (bind (_coords_x _coords_y) (break `/Game/Core/S_Coords` (`/Game/Battlefield/Block/BP_Block.Coords` (`self.CurrentBlock`))))
  (return (and (== _coords_x X) (== _coords_y (+ (- (`KismetMathLibrary.Round` (/ _gridsize_y 2.0)) 1) Y)))))

(fn `Set Spawns`
  (bind _gridsize_x (`KismetMathLibrary.BreakVector2D` (`self.GridSize`)))
  (bind _returnvalue (- (`KismetMathLibrary.Round` _gridsize_x) 1))
  (`|ExecutionSequence`
    (:`then_0`
      (`self.SetSpawnColors` 0 "NewEnumerator2")
      (`self.PlayerSpawn` 0 "NewEnumerator2"))
    (:`then_1`
      (`self.SetSpawnColors` _returnvalue "NewEnumerator1")
      (`self.PlayerSpawn` _returnvalue "NewEnumerator1"))))

(fn `SetBindedBlock`
  (params (UnitClass :type "/Game/Units/BP_Unit Class Reference") (NewParam :type "/Game/Core/E_Faction Enum" :default "NewEnumerator0"))
  (bind _outactors (`GameplayStatics.GetAllActorsOfClass` UnitClass))
  (for _array_element _outactors
    (if (`|EnumEquality` (`/Game/Units/BP_Unit.Faction` _array_element) NewParam)
      (set `/Game/Battlefield/Block/BP_Block.BindedUnit` _array_element (`self.CurrentBlock`)))))

(fn `SetFactions`
  (params (Team :type "/Game/Core/E_Faction Enum" :default "NewEnumerator0") (IncrustationLevel :type Integer))
  (`|ExecutionSequence`
    (:`then_0`
      (set `/Game/Battlefield/Block/BP_Block.BlockOwner` Team (`self.CurrentBlock`)))
    (:`then_1`
      (set `/Game/Battlefield/Block/BP_Block.IncrustationLevel` IncrustationLevel (`self.CurrentBlock`)))
    (:`then_2`
      (`/Game/Battlefield/Block/BP_Block.UpdateColor` (`self.CurrentBlock`) true))))

(fn `SetSpawnColors`
  (params (XGiridValue :type Integer) (Side :type "/Game/Core/E_Faction Enum" :default "NewEnumerator0"))
  (locals (GridHorizontalSize :type Integer) (Faction :type "/Game/Core/E_Faction Enum") (Direction :type Integer))
  (`|ExecutionSequence`
    (:`then_0`
      (set `local.GridHorizontalSize` XGiridValue))
    (:`then_1`
      (set `local.Faction` Side))
    (:`then_2`
      (switch `/Game/Core/E_Faction` (`local.Faction`)
        (:`NewEnumerator1`
          (set `local.Direction` -1))
        (:`NewEnumerator2`
          (set `local.Direction` 1))))
    (:`then_3`
      (bind _caseselected (`self.SelectCaseFromMiddleLeft` (`local.GridHorizontalSize`)))
      (if _caseselected
        (`self.SetFactions` (`local.Faction`) 3)
        (else
          (`|ExecutionSequence`
            (:`then_0`
              (bind _caseselected_2 (`self.SelectCaseFromMiddleLeft` (+ (`local.GridHorizontalSize`) (`local.Direction`)))))
            (:`then_1`
              (bind _caseselected_3 (`self.SelectCaseFromMiddleLeft` (`local.GridHorizontalSize`) 1)))
            (:`then_2`
              (bind _caseselected_4 (`self.SelectCaseFromMiddleLeft` (`local.GridHorizontalSize`) -1)))
            (:`then_3`
              (if (or _caseselected_2 _caseselected_3 _caseselected_4)
                (`self.SetFactions` (`local.Faction`) 2)
                (else
                  (`|ExecutionSequence`
                    (:`then_0`
                      (bind _caseselected_5 (`self.SelectCaseFromMiddleLeft` (`local.GridHorizontalSize`) 2)))
                    (:`then_1`
                      (bind _caseselected_6 (`self.SelectCaseFromMiddleLeft` (+ (`local.GridHorizontalSize`) (`local.Direction`)) 1)))
                    (:`then_2`
                      (bind _caseselected_7 (`self.SelectCaseFromMiddleLeft` (+ (`local.GridHorizontalSize`) (* (`local.Direction`) 2)))))
                    (:`then_3`
                      (bind _caseselected_8 (`self.SelectCaseFromMiddleLeft` (+ (`local.GridHorizontalSize`) (`local.Direction`)) -1)))
                    (:`then_4`
                      (bind _caseselected_9 (`self.SelectCaseFromMiddleLeft` (`local.GridHorizontalSize`) -2)))
                    (:`then_5`
                      (if (or _caseselected_5 _caseselected_6 _caseselected_7 _caseselected_8 _caseselected_9)
                        (`self.SetFactions` (`local.Faction`) 1)))))))))))))

(fn `UserConstructionScript`)