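; BP_SceneryBlock is a battlefield block whose look reflects its owning faction and incrustation level.
; UpdateColor picks a neutral, Winter or Spring mesh and a height per level, then moves the hover plane and action-range area above it.
; The construction script runs UpdateColor, parses the block index from the actor's display name after the last "k", derives coordinates from it, and hides both overlays.
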(fn `UpdateColor`
  (bind _actionrangearea (`self.ActionRangeArea`))
  (bind _hoveringplane (`self.HoveringPlane`))
  (bind (_returnvalue_x _returnvalue_y) (`KismetMathLibrary.BreakVector` (`SceneComponent.K2_GetComponentLocation` _hoveringplane)))
  (bind (_returnvalue_x_2 _returnvalue_y_2) (`KismetMathLibrary.BreakVector` (`SceneComponent.K2_GetComponentLocation` _actionrangearea)))
  (switch `int` (`self.IncrustationLevel`)
    (:`0`
      (set `self.Height` 10.0)
      (`StaticMeshComponent.SetStaticMesh` (`self.Cube`) "/Game/Battlefield/Block/Neutral_Block/SM_Neutral_Block.SM_Neutral_Block"))
    (:`1`
      (set `self.Height` 36.0)
      (switch `/Game/Core/E_Faction` (`self.BlockOwner`)
        (:`NewEnumerator1`
          (`StaticMeshComponent.SetStaticMesh` (`self.Cube`) "/Game/Battlefield/Block/Winter_Block_LV1/SM_Winter_Block_LV1.SM_Winter_Block_LV1"))
        (:`NewEnumerator2`
          (`StaticMeshComponent.SetStaticMesh` (`self.Cube`) "/Game/Battlefield/Block/Spring_Block_LV1/SM_Spring_Block_LV1.SM_Spring_Block_LV1"))))
    (:`2`
      (set `self.Height` 65.0)
      (switch `/Game/Core/E_Faction` (`self.BlockOwner`)
        (:`NewEnumerator1`
          (`StaticMeshComponent.SetStaticMesh` (`self.Cube`) "/Game/Battlefield/Block/Winter_Block_LV2/SM_Winter_Block_LV2.SM_Winter_Block_LV2"))
        (:`NewEnumerator2`
          (`StaticMeshComponent.SetStaticMesh` (`self.Cube`) "/Game/Battlefield/Block/Spring_Block_LV2/SM_Spring_Block_LV2.SM_Spring_Block_LV2"))))
    (:`3`
      (set `self.Height` 100.0)
      (switch `/Game/Core/E_Faction` (`self.BlockOwner`)
        (:`NewEnumerator1`
          (`StaticMeshComponent.SetStaticMesh` (`self.Cube`) "/Game/Battlefield/Block/Winter_Block_LV3/SM_Winter_Block_LV3.SM_Winter_Block_LV3"))
        (:`NewEnumerator2`
          (`StaticMeshComponent.SetStaticMesh` (`self.Cube`) "/Game/Battlefield/Block/Spring_Block_LV3/SM_Spring_Block_LV3.SM_Spring_Block_LV3")))))
  (`SceneComponent.K2_SetWorldLocation` _hoveringplane (`KismetMathLibrary.MakeVector` _returnvalue_x _returnvalue_y (+ (`self.Height`) 0.2)) false false)
  (`SceneComponent.K2_SetWorldLocation` _actionrangearea (`KismetMathLibrary.MakeVector` _returnvalue_x_2 _returnvalue_y_2 (+ (`self.Height`) 50.0)) false false)
  (return))

(fn `UserConstructionScript`
  (`self.UpdateColor`)
  (bind _output_get (set `self.Index` (`KismetStringLibrary.Conv_StringToInt` (`.RightS` (`KismetStringLibrary.Split` (`KismetSystemLibrary.GetDisplayName` self) "k" "IgnoreCase" "FromEnd")))))
  (bind (_x _y) (`/Game/Core/BP_CoordsFunctionLibrary.CalculateBlockCoordinates` _output_get))
  (set `self.Coords` (make `/Game/Core/S_Coords` _x _y))
  (`SceneComponent.SetVisibility` (`self.HoveringPlane`) false false)
  (`SceneComponent.SetVisibility` (`self.ActionRangeArea`) false false))