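; BP_Block is a clickable battlefield tile in a turn-based tactics game, owned by the Winter or Spring faction or neutral.
; Clicks route by the GameState's current phase to handlers that select, move, attack or use class capacities, usually through a confirmation step.
; ApplyIncrustation shifts its level and owner; UpdateColor then sets mesh, height and FMOD sound, repositioning any bound unit.
; Construction derives its grid coordinates from the number in its display name.
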(event `self.ReceiveBeginPlay`
  (bind _bindedunit (`self.BindedUnit`))
  (bind _asbp_gs_battle (cast `/Game/Core/GameMode/BattleScene/BP_GS_Battle` (`GameplayStatics.GetGameState`)))
  (set `self.GameState` _asbp_gs_battle)
  ;[1 1 1] Bind Block to Unit
  (`/Engine/EditorBlueprintResources/StandardMacros.IsValid` _bindedunit
    (:`Is Valid`
      (`/Game/Units/BP_Unit.BindBlock` _bindedunit self))))

(event `self.ReceiveActorBeginCursorOver`
  ;[1 1 1] Manage Hovering Plane visibility
  (`SceneComponent.SetVisibility` (`self.HoveringPlane`) true false)
  (`FMODBlueprintStatics.PlayEvent2D` "/Game/FMOD/Events/UI/UI_Buttons/UI_BU_Hover.UI_BU_Hover"))

(event `self.ReceiveActorEndCursorOver`
  ;[1 1 1] Manage Hovering Plane visibility
  (`SceneComponent.SetVisibility` (`self.HoveringPlane`) false false))

(event `self.ReceiveActorOnClicked`
  (params (ButtonPressed :type "Key Structure"))
  (`self.HandleClick`)
  (`KismetSystemLibrary.PrintString` (`KismetStringLibrary.Concat_StrStr` "Clicked index : " (`KismetStringLibrary.Conv_IntToString` (`self.Index`))) true true (struct :`G` 0.037146 :`B` 1.0 :`A` 1.0)))

(fn `ApplyIncrustation`
  (params (UnitFaction :type "/Game/Core/E_Faction Enum" :default "NewEnumerator0") (AttackPower :type Integer))
  (bind _returnvalue (- (`self.IncrustationLevel`) (`local.AttackPower`)))
  (if (`|EnumEquality` UnitFaction (`self.BlockOwner`))
    (set `self.IncrustationLevel` (`KismetMathLibrary.Clamp` (+ (`self.IncrustationLevel`) (`local.AttackPower`)) 0 3))
    (elif (== _returnvalue 0)
      (set `self.BlockOwner` "NewEnumerator0")
      (set `self.IncrustationLevel` 0)
      (elif (< _returnvalue 0)
        (set `self.BlockOwner` (`local.UnitFaction`))
        (set `self.IncrustationLevel` (`KismetMathLibrary.Abs_Int` _returnvalue))
        (else
          (set `self.IncrustationLevel` _returnvalue)))))
  (`self.UpdateColor` false)
  (return))

(fn `HandleAttackPhase`
  (returns (bResetLastBlockPosToCursor :type Boolean))
  (bind _gamestate (`self.GameState`))
  (if (`/Game/Core/GameMode/BattleScene/BP_GS_Battle.bAwaitingConfirmation` (`self.GameState`))
    (if (`self.bMarked`)
      (bind _unittoact (`/Game/Core/GameMode/BattleScene/BP_GS_Battle.GetUnitToAct` (`self.GameState`)))
      (`/Game/Units/BP_Unit.Attack` _unittoact)
      (return true)
      (else
        _))
    (else
      (bind _direction (`/Game/Core/BP_CoordsFunctionLibrary.GetDirectionOfAdjacentBlock` (`/Game/Core/GameMode/BattleScene/BP_GS_Battle.LastClickedBlock` (`self.GameState`)) self))
      (if (`|EnumEquality` _direction "NewEnumerator0")
        _
        (else
          (bind _unittoact_2 (`/Game/Core/GameMode/BattleScene/BP_GS_Battle.GetUnitToAct` (`self.GameState`)))
          (bind _output_get (set `/Game/Units/BP_Unit.CurrActionDirection` _direction _unittoact_2))
          (`/Game/Units/BP_Unit.Rotate` _unittoact_2 _output_get)
          (`/Game/Core/GameMode/BattleScene/BP_GS_Battle.GoToConfirmationStep` (`self.GameState`) "NewEnumerator2" null)
          (return true)))))
  (`/Game/Core/BP_UIManager.ChangePlayableUnitsMenuWhenBlockClicking` (`/Game/Core/GameMode/BattleScene/BP_GS_Battle.UIManager` _gamestate))
  (`/Game/Core/GameMode/BattleScene/BP_GS_Battle.EndCurrentPhase` _gamestate false)
  (return true))

(fn `HandleCapacityPhase`
  (returns (bResetLastBlockPosToCursor :type Boolean))
  (locals (UnitToAct :type "/Game/Units/BP_Unit Object Reference"))
  (bind _gamestate (`self.GameState`))
  (bind _gamestate_2 (`self.GameState`))
  (bind _gamestate_3 (`self.GameState`))
  (bind _gamestate_4 (`self.GameState`))
  (bind _unittoact (`/Game/Core/GameMode/BattleScene/BP_GS_Battle.GetUnitToAct` (`self.GameState`)))
  (bind _output_get (set `local.UnitToAct` _unittoact))
  (switch `/Game/Core/E_Class` (`/Game/Units/BP_Unit.Class` _output_get)
    (:`NewEnumerator0`
      ;[1 1 1] Handle Sniper Capacity Phase.
      (if (or (`self.bMarked`) (`self.bSubMarked`))
        (if (`/Game/Core/GameMode/BattleScene/BP_GS_Battle.bAwaitingConfirmation` (`self.GameState`))
          (bind _unittoact_2 (`/Game/Core/GameMode/BattleScene/BP_GS_Battle.GetUnitToAct` _gamestate))
          (`/Game/Units/BP_Unit.UseCapacity` _unittoact_2 (`/Game/Core/GameMode/BattleScene/BP_GS_Battle.LastClickedBlock` _gamestate))
          (return true)
          (else
            (`/Game/Core/GameMode/BattleScene/BP_GS_Battle.HideActionRange` (`self.GameState`) false false)
            (bind _unittoact_3 (`/Game/Core/GameMode/BattleScene/BP_GS_Battle.GetUnitToAct` (`self.GameState`)))
            (bind _direction (`/Game/Core/BP_CoordsFunctionLibrary.GetDirectionToDestination` (`/Game/Units/BP_Unit.BindedBlock` _unittoact_3) self))
            (bind _output_get_2 (set `/Game/Units/BP_Unit.CurrActionDirection` _direction _unittoact_3))
            (`/Game/Units/BP_Unit.Rotate` _unittoact_3 _output_get_2)
            (`/Game/Core/GameMode/BattleScene/BP_GS_Battle.GoToConfirmationStep` (`self.GameState`) "NewEnumerator4" self)
            (return false)))
        (else
          (`/Game/Core/BP_UIManager.ChangePlayableUnitsMenuWhenBlockClicking` (`/Game/Core/GameMode/BattleScene/BP_GS_Battle.UIManager` _gamestate_3))
          (`/Game/Core/GameMode/BattleScene/BP_GS_Battle.EndCurrentPhase` _gamestate_3 false)
          (return true))))
    (:`NewEnumerator1`
      ;[1 1 1] Handle Protector Capacity Phase.
      (if (or (`self.bMarked`) (`self.bSubMarked`))
        (`/Game/Units/BP_Unit.UseCapacity` (`local.UnitToAct`) null)
        (else
          (`/Game/Core/BP_UIManager.ChangePlayableUnitsMenuWhenBlockClicking` (`/Game/Core/GameMode/BattleScene/BP_GS_Battle.UIManager` _gamestate_2))
          (`/Game/Core/GameMode/BattleScene/BP_GS_Battle.EndCurrentPhase` _gamestate_2 false)))
      (return true))
    (:`NewEnumerator2`
      ;[1 1 1] Handle Inlayer Capacity Phase.
      (if (`/Game/Core/GameMode/BattleScene/BP_GS_Battle.bAwaitingConfirmation` (`self.GameState`))
        (if (or (`self.bMarked`) (`self.bSubMarked`))
          (bind _unittoact_4 (`/Game/Core/GameMode/BattleScene/BP_GS_Battle.GetUnitToAct` (`self.GameState`)))
          (`/Game/Units/BP_Unit.UseCapacity` _unittoact_4 null)
          (return true)
          (else
            _))
        (else
          (bind _direction_2 (`/Game/Core/BP_CoordsFunctionLibrary.GetDirectionOfAdjacentBlock` (`/Game/Core/GameMode/BattleScene/BP_GS_Battle.LastClickedBlock` (`self.GameState`)) self))
          (if (`|EnumEquality` _direction_2 "NewEnumerator0")
            _
            (else
              (bind _unittoact_5 (`/Game/Core/GameMode/BattleScene/BP_GS_Battle.GetUnitToAct` (`self.GameState`)))
              (bind _output_get_3 (set `/Game/Units/BP_Unit.CurrActionDirection` _direction_2 _unittoact_5))
              (`/Game/Units/BP_Unit.Rotate` _unittoact_5 _output_get_3)
              (`/Game/Core/GameMode/BattleScene/BP_GS_Battle.GoToConfirmationStep` (`self.GameState`) "NewEnumerator4" null)
              (return true)))))
      (`/Game/Core/BP_UIManager.ChangePlayableUnitsMenuWhenBlockClicking` (`/Game/Core/GameMode/BattleScene/BP_GS_Battle.UIManager` _gamestate_4))
      (`/Game/Core/GameMode/BattleScene/BP_GS_Battle.EndCurrentPhase` _gamestate_4 false)
      (return true))))

(fn `HandleClick`
  (bind _gamestate (`self.GameState`))
  (bind _gamestate_2 (`self.GameState`))
  (if (`/Game/Core/GameMode/BattleScene/BP_GS_Battle.bAIPlaying` _gamestate_2)
    (return)
    (else
      (`FMODBlueprintStatics.PlayEvent2D` "/Game/FMOD/Events/UI/UI_Buttons/UI_BU_Click.UI_BU_Click")
      (switch `/Game/Core/E_Phase` (`/Game/Core/GameMode/BattleScene/BP_GS_Battle.CurrPhase` _gamestate_2)
        (:`NewEnumerator0`
          (bind _bresetlastblockpostocursor (`self.HandleNonePhase`))
          (if _bresetlastblockpostocursor
            ;[1 1 1] If LastClickedBlock must be reset, we set it to the current Cursor position.
            (bind _unittoact (`/Game/Core/GameMode/BattleScene/BP_GS_Battle.GetUnitToAct` _gamestate :!label _label))
            (`/Engine/EditorBlueprintResources/StandardMacros.IsValid` _unittoact
              (:`Is Valid`
                (set `/Game/Core/GameMode/BattleScene/BP_GS_Battle.LastClickedBlock` (`/Game/Units/BP_Unit.BindedBlock` _unittoact) _gamestate)
                (return))
              (:`Is Not Valid`
                _))))
        (:`NewEnumerator1`
          (bind _bresetlastblockpostocursor_2 (`self.HandleMovePhase`))
          (if _bresetlastblockpostocursor_2
            (goto _label)
            (else
              _)))
        (:`NewEnumerator2`
          (bind _bresetlastblockpostocursor_3 (`self.HandleAttackPhase`))
          (if _bresetlastblockpostocursor_3
            (goto _label)
            (else
              _)))
        (:`NewEnumerator3`
          (`/Game/Core/BP_UIManager.ChangePlayableUnitsMenuWhenBlockClicking` (`/Game/Core/GameMode/BattleScene/BP_GS_Battle.UIManager` (`self.GameState`)))
          (`/Game/Core/GameMode/BattleScene/BP_GS_Battle.EndCurrentPhase` (`self.GameState`) false :!label _label_2)
          (return))
        (:`NewEnumerator4`
          (bind _bresetlastblockpostocursor_4 (`self.HandleCapacityPhase`))
          (if _bresetlastblockpostocursor_4
            (goto _label)
            (else
              _)))
        (:`NewEnumerator7`
          (goto _label_2)))
      ;[1 1 1] If LastClickedBlock has not to be reset, we set it to the real Block on which the player clicked.
      (set `/Game/Core/GameMode/BattleScene/BP_GS_Battle.LastClickedBlock` self (`self.GameState`))
      (return))))

(fn `HandleMovePhase`
  (returns (bResetLastBlockPosToCursor :type Boolean))
  (bind _gamestate (`self.GameState`))
  (if (`self.bMarked`)
    (if (`/Game/Core/GameMode/BattleScene/BP_GS_Battle.bAwaitingConfirmation` (`self.GameState`))
      (if (== self (`/Game/Core/GameMode/BattleScene/BP_GS_Battle.LastClickedBlock` (`self.GameState`)))
        (bind _unittoact (`/Game/Core/GameMode/BattleScene/BP_GS_Battle.GetUnitToAct` (`self.GameState`)))
        (`/Game/Units/BP_Unit.Move` _unittoact self)
        (return true)
        (else
          _)))
    (bind _unittoact_2 (`/Game/Core/GameMode/BattleScene/BP_GS_Battle.GetUnitToAct` (`self.GameState`)))
    (bind _direction (`/Game/Core/BP_CoordsFunctionLibrary.GetDirectionToDestination` (`/Game/Units/BP_Unit.BindedBlock` _unittoact_2) self))
    (bind _output_get (set `/Game/Units/BP_Unit.CurrActionDirection` _direction _unittoact_2))
    (`/Game/Units/BP_Unit.Rotate` _unittoact_2 _output_get)
    (`/Game/Core/GameMode/BattleScene/BP_GS_Battle.GoToConfirmationStep` (`self.GameState`) "NewEnumerator1" self)
    (return false)
    (else
      (`/Game/Core/BP_UIManager.ChangePlayableUnitsMenuWhenBlockClicking` (`/Game/Core/GameMode/BattleScene/BP_GS_Battle.UIManager` _gamestate))
      (`/Game/Core/GameMode/BattleScene/BP_GS_Battle.EndCurrentPhase` _gamestate false)
      (return true))))

(fn `HandleNonePhase`
  (returns (bResetLastBlockPosToCursor :type Boolean))
  (bind _bindedunit (`self.BindedUnit`))
  (bind _gamestate (`self.GameState`))
  (bind (_history_turnsactions _history_currturnidx) (break `/Game/Core/S_GameHistory` (`/Game/Core/GameMode/BattleScene/BP_GS_Battle.History` (`self.GameState`))))
  (bind (_output_unitsactions _output_currentunitidx) (break `/Game/Core/S_TurnActionsHistory` (`|GetArrayItem` _history_turnsactions _history_currturnidx)))
  (bind _hasacted (`/Game/Core/GameMode/BattleScene/BP_GS_Battle.HasUnitActed` (`self.GameState`)))
  (if _hasacted
    (return true)
    (else
      (`/Engine/EditorBlueprintResources/StandardMacros.IsValid` _bindedunit
        (:`Is Valid`
          (if (`|EnumEquality` (`/Game/Core/GameMode/BattleScene/BP_GS_Battle.CurrFaction` (`self.GameState`)) (`/Game/Units/BP_Unit.Faction` _bindedunit))
            (if (`/Game/Units/BP_Unit.bAlreadyBeenPlayed` (`self.BindedUnit`))
              (`/Game/Core/GameMode/BattleScene/BP_GS_Battle.DefineUnitToAct` _gamestate null :!label _label)
              (else
                (`/Game/Core/GameMode/BattleScene/BP_GS_Battle.DefineUnitToAct` (`self.GameState`) (`self.BindedUnit`))))
            (else
              (goto _label))))
        (:`Is Not Valid`
          (goto _label)))
      (`/Game/Core/BP_UIManager.UpdateActionsMenu` (`/Game/Core/GameMode/BattleScene/BP_GS_Battle.UIManager` _gamestate) (`|GetArrayItem` _output_unitsactions _output_currentunitidx))
      (return false))))

(fn `UpdateColor`
  (params (bWithoutSound :type Boolean))
  (bind _actionrangearea (`self.ActionRangeArea`))
  (bind _hoveringplane (`self.HoveringPlane`))
  (bind _bindedunit (`self.BindedUnit`))
  (bind (_returnvalue_x _returnvalue_y) (`KismetMathLibrary.BreakVector` (`SceneComponent.K2_GetComponentLocation` _hoveringplane)))
  (bind (_returnvalue_x_2 _returnvalue_y_2) (`KismetMathLibrary.BreakVector` (`SceneComponent.K2_GetComponentLocation` _actionrangearea)))
  (bind (_returnvalue_x_3 _returnvalue_y_3) (`KismetMathLibrary.BreakVector` (`self.K2_GetActorLocation` _bindedunit)))
  (switch `int` (`self.IncrustationLevel`)
    (:`0`
      (set `self.Height` 10.0)
      (`StaticMeshComponent.SetStaticMesh` (`self.Cube`) "/Game/Battlefield/Block/Neutral_Block/SM_Neutral_Block.SM_Neutral_Block"))
    (:`1`
      (set `self.Height` 36.0)
      (switch `/Game/Core/E_Faction` (`self.BlockOwner`)
        (:`NewEnumerator1`
          (`StaticMeshComponent.SetStaticMesh` (`self.Cube`) "/Game/Battlefield/Block/Winter_Block_LV1/SM_Winter_Block_LV1.SM_Winter_Block_LV1"))
        (:`NewEnumerator2`
          (`StaticMeshComponent.SetStaticMesh` (`self.Cube`) "/Game/Battlefield/Block/Spring_Block_LV1/SM_Spring_Block_LV1.SM_Spring_Block_LV1"))))
    (:`2`
      (set `self.Height` 65.0)
      (switch `/Game/Core/E_Faction` (`self.BlockOwner`)
        (:`NewEnumerator1`
          (`StaticMeshComponent.SetStaticMesh` (`self.Cube`) "/Game/Battlefield/Block/Winter_Block_LV2/SM_Winter_Block_LV2.SM_Winter_Block_LV2"))
        (:`NewEnumerator2`
          (`StaticMeshComponent.SetStaticMesh` (`self.Cube`) "/Game/Battlefield/Block/Spring_Block_LV2/SM_Spring_Block_LV2.SM_Spring_Block_LV2"))))
    (:`3`
      (set `self.Height` 100.0)
      (switch `/Game/Core/E_Faction` (`self.BlockOwner`)
        (:`NewEnumerator1`
          (`StaticMeshComponent.SetStaticMesh` (`self.Cube`) "/Game/Battlefield/Block/Winter_Block_LV3/SM_Winter_Block_LV3.SM_Winter_Block_LV3"))
        (:`NewEnumerator2`
          (`StaticMeshComponent.SetStaticMesh` (`self.Cube`) "/Game/Battlefield/Block/Spring_Block_LV3/SM_Spring_Block_LV3.SM_Spring_Block_LV3")))))
  (if (not (`local.bWithoutSound`))
    (switch `/Game/Core/E_Faction` (`self.BlockOwner`)
      (:`NewEnumerator0`
        (`FMODAudioComponent.SetEvent` (`self.FMODAudio`) "/Game/FMOD/Events/Blocks/B_Neutral.B_Neutral"))
      (:`NewEnumerator1`
        (`FMODAudioComponent.SetEvent` (`self.FMODAudio`) "/Game/FMOD/Events/Blocks/B_WinterUpgrade.B_WinterUpgrade"))
      (:`NewEnumerator2`
        (`FMODAudioComponent.SetEvent` (`self.FMODAudio`) "/Game/FMOD/Events/Blocks/B_SpringUpgrade.B_SpringUpgrade")))
    (`FMODAudioComponent.Play` (`self.FMODAudio`)))
  (`SceneComponent.K2_SetWorldLocation` _hoveringplane (`KismetMathLibrary.MakeVector` _returnvalue_x _returnvalue_y (+ (`self.Height`) 0.2)) false false)
  (`SceneComponent.K2_SetWorldLocation` _actionrangearea (`KismetMathLibrary.MakeVector` _returnvalue_x_2 _returnvalue_y_2 (+ (`self.Height`) 50.0)) false false)
  (`/Engine/EditorBlueprintResources/StandardMacros.IsValid` _bindedunit
    (:`Is Valid`
      (`self.K2_SetActorLocation` _bindedunit (`KismetMathLibrary.MakeVector` _returnvalue_x_3 _returnvalue_y_3 (`self.Height`)) false false))
    (:`Is Not Valid`
      _))
  (return))

(fn `UserConstructionScript`
  (`self.UpdateColor` true)
  (bind _output_get (set `self.Index` (`KismetStringLibrary.Conv_StringToInt` (`.RightS` (`KismetStringLibrary.Split` (`KismetSystemLibrary.GetDisplayName` self) "k" "IgnoreCase" "FromEnd")))))
  (bind (_x _y) (`/Game/Core/BP_CoordsFunctionLibrary.CalculateBlockCoordinates` _output_get))
  (set `self.Coords` (make `/Game/Core/S_Coords` _x _y))
  (`SceneComponent.SetVisibility` (`self.HoveringPlane`) false false)
  (`SceneComponent.SetVisibility` (`self.ActionRangeArea`) false false))