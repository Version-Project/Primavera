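; BP_Block is a battlefield grid tile that can hold a Unit and handles player clicks for unit selection and movement.
; Construction colors it by owning faction and incrustation level, and derives coordinates from the number in its display name.
; Clicks branch on the GameState phase: None selects an eligible unit, Move confirms a move with a second click on an in-range block.
; Hover toggles a highlight plane; confirmation UI is still PrintString placeholders.
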(event `self.ReceiveBeginPlay`
  (bind _bindedunit (`self.BindedUnit`))
  (bind _asbp_game_state (cast `/Game/Core/GameMode/BP_GameState` (`GameplayStatics.GetGameState`)))
  (set `self.GameState` _asbp_game_state)
  ;[1 1 1] Bind Block to Unit
  (`/Engine/EditorBlueprintResources/StandardMacros.IsValid` _bindedunit
    (:`Is Valid`
      (`/Game/Units/BP_Unit.BindBlock` _bindedunit self))))

(event `self.ReceiveActorBeginCursorOver`
  ;[1 1 1] Manage Hovering Plane visibility
  (`SceneComponent.SetVisibility` (`self.HoveringPlane`) true false))

(event `self.ReceiveActorEndCursorOver`
  ;[1 1 1] Manage Hovering Plane visibility
  (`SceneComponent.SetVisibility` (`self.HoveringPlane`) false false))

(event `self.ReceiveActorOnClicked`
  (params (ButtonPressed :type "Key Structure"))
  (`self.ManageClick`))

(fn `ManageClick`
  (switch `/Game/Core/E_Phase` (`/Game/Core/GameMode/BP_GameState.CurrPhase` (`self.GameState`))
    (:`NewEnumerator0`
      (`self.ManageNonePhase`))
    (:`NewEnumerator1`
      (`self.ManageMovePhase`)))
  (set `/Game/Core/GameMode/BP_GameState.LastClickedBlock` self (`self.GameState`))
  (return))

(fn `ManageMovePhase`
  (bind _gamestate (`self.GameState`))
  (if (`SceneComponent.IsVisible` (`self.ActionRangePlane`))
    (if (`/Game/Core/GameMode/BP_GameState.bAwaitingConfirmation` (`self.GameState`))
      (if (== self (`/Game/Core/GameMode/BP_GameState.LastClickedBlock` (`self.GameState`)))
        (bind _unittoact (`/Game/Core/GameMode/BP_GameState.GetUnitToAct` (`self.GameState`)))
        (`/Game/Units/BP_Unit.MoveUnit` _unittoact self)
        (return)
        (else
          _))
      (else
        (set `/Game/Core/GameMode/BP_GameState.bAwaitingConfirmation` true (`self.GameState`))
        (`KismetSystemLibrary.PrintString` "Display ConfirmMenu.")))
    (`KismetSystemLibrary.PrintString` "Display ConfirmArrow at the current Block location.")
    (return)
    (else
      (`/Game/Core/GameMode/BP_GameState.HideActionRange` _gamestate)
      (set `/Game/Core/GameMode/BP_GameState.CurrPhase` "NewEnumerator0" _gamestate)
      (return))))

(fn `ManageNonePhase`
  (bind _bindedunit (`self.BindedUnit`))
  (bind _hasacted (`/Game/Core/GameMode/BP_GameState.HasUnitActed` (`self.GameState`)))
  (if (not _hasacted)
    (`/Engine/EditorBlueprintResources/StandardMacros.IsValid` _bindedunit
      (:`Is Valid`
        (if (`|EnumEquality` (`/Game/Core/GameMode/BP_GameState.CurrFaction` (`self.GameState`)) (`/Game/Units/BP_Unit.Faction` _bindedunit))
          (if (`/Game/Units/BP_Unit.bAlreadyBeenPlayed` (`self.BindedUnit`))
            (`/Game/Core/GameMode/BP_GameState.DefineUnitToAct` (`self.GameState`) null :!label _label)
            (else
              (`/Game/Core/GameMode/BP_GameState.DefineUnitToAct` (`self.GameState`) (`self.BindedUnit`))))
          (else
            (goto _label))))
      (:`Is Not Valid`
        (goto _label)))
    (return)))

(fn `UpdateColor`
  (bind _cube (`self.Cube`))
  (switch `/Game/Core/E_Faction` (`self.BlockOwner`)
    (:`NewEnumerator1`
      (switch `int` (`self.IncrustationLevel`)
        (:`1`
          (`PrimitiveComponent.SetMaterial` _cube 0 "/Game/MaterialLibrary/M_BlueLV1.M_BlueLV1"))
        (:`2`
          (`PrimitiveComponent.SetMaterial` _cube 0 "/Game/MaterialLibrary/M_BlueLV2.M_BlueLV2"))
        (:`3`
          (`PrimitiveComponent.SetMaterial` _cube 0 "/Game/MaterialLibrary/M_BlueLV3.M_BlueLV3"))))
    (:`NewEnumerator2`
      (switch `int` (`self.IncrustationLevel`)
        (:`1`
          (`PrimitiveComponent.SetMaterial` _cube 0 "/Game/MaterialLibrary/M_OrangeLV1.M_OrangeLV1"))
        (:`2`
          (`PrimitiveComponent.SetMaterial` _cube 0 "/Game/MaterialLibrary/M_OrangeLV2.M_OrangeLV2"))
        (:`3`
          (`PrimitiveComponent.SetMaterial` _cube 0 "/Game/MaterialLibrary/M_OrangeLV3.M_OrangeLV3")))))
  (return))

(fn `UserConstructionScript`
  (`self.UpdateColor`)
  (bind _output_get (set `self.Index` (`KismetStringLibrary.Conv_StringToInt` (`.RightS` (`KismetStringLibrary.Split` (`KismetSystemLibrary.GetDisplayName` self) "k" "IgnoreCase" "FromEnd")))))
  (bind (_x _y) (`/Game/Core/BP_CoordsFunctionLibrary.GetBlockCoordinates` _output_get))
  (set `self.Coords` (make `/Game/Core/S_Coords` _x _y))
  (`SceneComponent.SetVisibility` (`self.HoveringPlane`) false false)
  (`SceneComponent.SetVisibility` (`self.ActionRangePlane`) false false))