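; BP_RandomField randomly generates a mirrored starting layout of faction-owned blocks on the battlefield at BeginPlay.
; It picks random coordinates among unbound, unowned BP_Block tiles on the left half, extending the loop on duplicate or invalid picks.
; Percentage settings move some picks into incrustation levels 2 and 3, then each set is mirrored across X.
; Matching blocks receive an owner by side and their incrustation level, then refresh their color.
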(event `self.ReceiveBeginPlay`
  (bind _outactors (`GameplayStatics.GetAllActorsOfClass` "/Game/Battlefield/Block/BP_Block.BP_Block_C"))
  (bind _output_get (set `self.AllBlocks` _outactors))
  (for _array_element _output_get
    (`self.GetValidBlocks` _array_element))
  (`self.RandomBlocks`)
  (`self.RandomIncrustation`)
  (`self.MirrorBlocks`)
  (for _array_element_2 (`self.AllBlocks`)
    (set `self.CurrentBlock` _array_element_2)
    (`|ExecutionSequence`
      (:`then_0`
        (`self.SetCololor` (`self.BlocksCoords`) 1))
      (:`then_1`
        (`self.SetCololor` (`self.BlocksCoordsInc2`) 2))
      (:`then_2`
        (`self.SetCololor` (`self.BlocksCoordsInc3`) 3)))))

(fn `CurrentMirror`
  (params (`Current Inc` :type "Array of /Game/Core/S_Coords Structure"))
  (locals (MirrorBlocks :type "Array of /Game/Core/S_Coords Structure"))
  (for _array_element `Current Inc`
    (`KismetArrayLibrary.Array_Add` (`local.MirrorBlocks`) (make `/Game/Core/S_Coords` (- 15 (break `/Game/Core/S_Coords` _array_element)) (`.Y_6_2DC6362D4EE28ABEA56491A3230A1BE6` (break `/Game/Core/S_Coords` _array_element)))))
  (`KismetArrayLibrary.Array_Append` `Current Inc` (`local.MirrorBlocks`)))

(fn `GetValidBlocks`
  (params (SetCurrentBlock :type "/Game/Battlefield/Block/BP_Block Object Reference"))
  (set `self.CurrentBlock` SetCurrentBlock)
  ;[1 1 1] Middle Left
  (if (<= (`.X_5_364656D3417FA6B1F82E4585A34E5C6B` (break `/Game/Core/S_Coords` (`/Game/Battlefield/Block/BP_Block.Coords` (`self.CurrentBlock`)))) 7)
    (`/Engine/EditorBlueprintResources/StandardMacros.IncrementInt` (`self.TotalLeftLength`)
      (:`  `
        ;[1 1 1] Not Binded
        (if (`KismetStringLibrary.EqualEqual_StrStr` (`KismetSystemLibrary.GetDisplayName` (`/Game/Battlefield/Block/BP_Block.BindedUnit` (`self.CurrentBlock`))))
          ;[1 1 1] Not colored
          (if (`KismetStringLibrary.EqualEqual_StrStr` (`|GetEnumeratorNameAsString` (`/Game/Battlefield/Block/BP_Block.BlockOwner` (`self.CurrentBlock`))))
            (`KismetArrayLibrary.Array_Add` (`self.AllValidBlocks`) (`self.CurrentBlock`))))))))

(fn `MirrorBlocks`
  (`self.CurrentMirror` (`self.BlocksCoords`))
  (`self.CurrentMirror` (`self.BlocksCoordsInc2`))
  (`self.CurrentMirror` (`self.BlocksCoordsInc3`)))

(fn `RandomBlocks`
  (locals (AllValidIndexes :type "Array of Integer") (RandomValue :type Integer) (AllValidCoords :type "Array of /Game/Core/S_Coords Structure") (RandomCoord :type "/Game/Core/S_Coords Structure"))
  (for _array_element (`self.AllValidBlocks`)
    (`KismetArrayLibrary.Array_Add` (`local.AllValidCoords`) (`/Game/Battlefield/Block/BP_Block.Coords` _array_element)))
  (for _ (range (+ (`self.MaxTiles`) 1))
    (set `local.RandomCoord` (make `/Game/Core/S_Coords` (`KismetMathLibrary.RandomIntegerInRange` 0 7) (`KismetMathLibrary.RandomIntegerInRange` 0 10)))
    (if (`KismetArrayLibrary.Array_Contains` (`self.BlocksCoords`) (`local.RandomCoord`))
      (`/Engine/EditorBlueprintResources/StandardMacros.IncrementInt` (`self.MaxTiles`) :!label _label)
      (elif (not (`KismetArrayLibrary.Array_Contains` (`local.AllValidCoords`) (`local.RandomCoord`)))
        (goto _label)
        (else
          (`KismetArrayLibrary.Array_Add` (`self.BlocksCoords`) (`local.RandomCoord`)))))))

(fn `RandomIncrustation`
  (for _index (range (/ (`KismetArrayLibrary.Array_Length` (`self.BlocksCoords`)) (/ 100 (`self.Incrustation2Percent`))))
    (`KismetArrayLibrary.Array_Add` (`self.BlocksCoordsInc2`) (`|GetArrayItem` (`self.BlocksCoords`) _index))
    (`KismetArrayLibrary.Array_Remove` (`self.BlocksCoords`)))
  (for _index_2 (range (/ (`KismetArrayLibrary.Array_Length` (`self.BlocksCoords`)) (/ 100 (`self.Incrustation3Percent`))))
    (`KismetArrayLibrary.Array_Add` (`self.BlocksCoordsInc3`) (`|GetArrayItem` (`self.BlocksCoords`) _index_2))
    (`KismetArrayLibrary.Array_Remove` (`self.BlocksCoords`))))

(fn `SetCololor`
  (params (BlockCoords :type "Array of /Game/Core/S_Coords Structure") (Incrustation :type Integer))
  (bind _coords_x (break `/Game/Core/S_Coords` (`/Game/Battlefield/Block/BP_Block.Coords` (`self.CurrentBlock`))))
  (if (`KismetArrayLibrary.Array_Contains` BlockCoords (`/Game/Battlefield/Block/BP_Block.Coords` (`self.CurrentBlock`)))
    (if (<= _coords_x 7)
      (`self.UpdateCaseColor` "NewEnumerator2" (`self.CurrentBlock`) Incrustation)
      (else
        (`self.UpdateCaseColor` "NewEnumerator1" (`self.CurrentBlock`) Incrustation)))))

(fn `UpdateCaseColor`
  (params (Faction :type "/Game/Core/E_Faction Enum" :default "NewEnumerator0") (CurrentBlock :type "/Game/Battlefield/Block/BP_Block Object Reference") (Incrustation :type Integer))
  (set `/Game/Battlefield/Block/BP_Block.BlockOwner` Faction CurrentBlock)
  (set `/Game/Battlefield/Block/BP_Block.IncrustationLevel` Incrustation CurrentBlock)
  (`/Game/Battlefield/Block/BP_Block.UpdateColor` CurrentBlock))

(fn `UserConstructionScript`)