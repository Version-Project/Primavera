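; Scenery manager for the battlefield that reflects which faction, Spring or Winter, leads in score.
; UpdateScenery turns the score difference into a winner, or neutral, and a lead level from one to three using threshold variables.
; It swaps mountain and tree materials per faction and level, and leaf materials per faction only.
; It also passes winner and level to the BP_Light found at BeginPlay to update its temperature.
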(event `self.ReceiveBeginPlay`
  (bind _returnvalue (`GameplayStatics.GetActorOfClass` "/Game/Battlefield/Scenery/BP_Light.BP_Light_C"))
  (set `self.Light` _returnvalue))

(fn `UpdateScenery`
  (params (SpringScore :type Integer) (WinterScore :type Integer))
  (locals (Difference :type Integer) (CurrWinner :type "/Game/Core/E_Faction Enum"))
  (bind _staticmeshcomponent (`StaticMeshActor.StaticMeshComponent` (`self.Leaves`)))
  ;[1 1 1] Get current winner.
  (bind _output_get (set `local.Difference` (- SpringScore WinterScore)))
  (if (>= _output_get (`self.LowLimitLevel1`))
    (set `local.CurrWinner` "NewEnumerator2")
    (`PrimitiveComponent.SetMaterial` _staticmeshcomponent 0 "/Game/Battlefield/Scenery/Leaves/Spring/M_Leaves_Spring.M_Leaves_Spring")
    (elif (<= (`local.Difference`) (* (`self.LowLimitLevel1`) -1))
      (set `local.CurrWinner` "NewEnumerator1")
      (`PrimitiveComponent.SetMaterial` _staticmeshcomponent 0 "/Game/Battlefield/Scenery/Leaves/Winter/M_Leaves_Winter.M_Leaves_Winter")
      (else
        (set `local.CurrWinner` "NewEnumerator0")
        ;[1 1 1] Neutral
        (`PrimitiveComponent.SetMaterial` (`StaticMeshActor.StaticMeshComponent` (`self.Mountain`)) 0 "/Game/Battlefield/Scenery/Moutain/Neutral/M_Mountain_Neutral.M_Mountain_Neutral")
        (`PrimitiveComponent.SetMaterial` (`StaticMeshActor.StaticMeshComponent` (`self.Tree`)) 0 "/Game/Battlefield/Scenery/Tree/Neutral/M_Tree_Neutral.M_Tree_Neutral")
        (`PrimitiveComponent.SetMaterial` (`StaticMeshActor.StaticMeshComponent` (`self.Leaves`)) 0 "/Game/Battlefield/Scenery/Leaves/Neutral/M_Leaves_Neutral.M_Leaves_Neutral")
        (`/Game/Battlefield/Scenery/BP_Light.UpdateTemperature` (`self.Light`) (`local.CurrWinner`) 0)
        (return))))
  (set `local.Difference` (`KismetMathLibrary.Abs_Int` (`local.Difference`)))
  (if (>= (`local.Difference`) (`self.LowLimitLevel3`))
    (switch `/Game/Core/E_Faction` (`local.CurrWinner`)
      (:`NewEnumerator1`
        ;[1 1 1] Winter Level 3
        (`PrimitiveComponent.SetMaterial` (`StaticMeshActor.StaticMeshComponent` (`self.Mountain`)) 0 "/Game/Battlefield/Scenery/Moutain/Winter3/M_Mountain_Winter3.M_Mountain_Winter3")
        (`PrimitiveComponent.SetMaterial` (`StaticMeshActor.StaticMeshComponent` (`self.Tree`)) 0 "/Game/Battlefield/Scenery/Tree/Winter3/M_Tree_Winter3.M_Tree_Winter3")
        (`/Game/Battlefield/Scenery/BP_Light.UpdateTemperature` (`self.Light`) (`local.CurrWinner`) 3)
        (return))
      (:`NewEnumerator2`
        ;[1 1 1] Spring Level 3
        (`PrimitiveComponent.SetMaterial` (`StaticMeshActor.StaticMeshComponent` (`self.Mountain`)) 0 "/Game/Battlefield/Scenery/Moutain/Spring3/M_Mountain_Spring3.M_Mountain_Spring3")
        (`PrimitiveComponent.SetMaterial` (`StaticMeshActor.StaticMeshComponent` (`self.Tree`)) 0 "/Game/Battlefield/Scenery/Tree/Spring3/M_Tree_Spring3.M_Tree_Spring3")
        (`/Game/Battlefield/Scenery/BP_Light.UpdateTemperature` (`self.Light`) (`local.CurrWinner`) 3)
        (return)))
    (elif (>= (`local.Difference`) (`self.LowLimitLevel2`))
      (switch `/Game/Core/E_Faction` (`local.CurrWinner`)
        (:`NewEnumerator1`
          ;[1 1 1] Winter Level 2
          (`PrimitiveComponent.SetMaterial` (`StaticMeshActor.StaticMeshComponent` (`self.Mountain`)) 0 "/Game/Battlefield/Scenery/Moutain/Winter2/M_Mountain_Winter2.M_Mountain_Winter2")
          (`PrimitiveComponent.SetMaterial` (`StaticMeshActor.StaticMeshComponent` (`self.Tree`)) 0 "/Game/Battlefield/Scenery/Tree/Winter2/M_Tree_Winter2.M_Tree_Winter2")
          (`/Game/Battlefield/Scenery/BP_Light.UpdateTemperature` (`self.Light`) (`local.CurrWinner`) 2)
          (return))
        (:`NewEnumerator2`
          ;[1 1 1] Spring Level 2
          (`PrimitiveComponent.SetMaterial` (`StaticMeshActor.StaticMeshComponent` (`self.Mountain`)) 0 "/Game/Battlefield/Scenery/Moutain/Spring2/M_Mountain_Spring2.M_Mountain_Spring2")
          (`PrimitiveComponent.SetMaterial` (`StaticMeshActor.StaticMeshComponent` (`self.Tree`)) 0 "/Game/Battlefield/Scenery/Tree/Spring2/M_Tree_Spring2.M_Tree_Spring2")
          (`/Game/Battlefield/Scenery/BP_Light.UpdateTemperature` (`self.Light`) (`local.CurrWinner`) 2)
          (return)))
      (else
        (switch `/Game/Core/E_Faction` (`local.CurrWinner`)
          (:`NewEnumerator1`
            ;[1 1 1] Winter Level 1
            (`PrimitiveComponent.SetMaterial` (`StaticMeshActor.StaticMeshComponent` (`self.Mountain`)) 0 "/Game/Battlefield/Scenery/Moutain/Winter1/M_Mountain_Winter1.M_Mountain_Winter1")
            (`PrimitiveComponent.SetMaterial` (`StaticMeshActor.StaticMeshComponent` (`self.Tree`)) 0 "/Game/Battlefield/Scenery/Tree/Winter1/M_Tree_Winter1.M_Tree_Winter1")
            (`/Game/Battlefield/Scenery/BP_Light.UpdateTemperature` (`self.Light`) (`local.CurrWinner`) 1)
            (return))
          (:`NewEnumerator2`
            ;[1 1 1] Spring Level 1
            (`PrimitiveComponent.SetMaterial` (`StaticMeshActor.StaticMeshComponent` (`self.Mountain`)) 0 "/Game/Battlefield/Scenery/Moutain/Spring1/M_Mountain_Spring1.M_Mountain_Spring1")
            (`PrimitiveComponent.SetMaterial` (`StaticMeshActor.StaticMeshComponent` (`self.Tree`)) 0 "/Game/Battlefield/Scenery/Tree/Spring1/M_Tree_Spring1.M_Tree_Spring1")
            (`/Game/Battlefield/Scenery/BP_Light.UpdateTemperature` (`self.Light`) (`local.CurrWinner`) 1)
            (return)))))))

(fn `UserConstructionScript`)