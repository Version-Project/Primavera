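; BP_Light is a battlefield scenery light whose directional light rotates continuously and shifts colour temperature with the leading faction.
; Tick decrements the yaw angle by Speed each frame, without delta-time scaling, at a fixed pitch that the construction script also applies.
; UpdateTemperature maps Level to an offset from BaseTemperature, raising it for Winter (cooler) and lowering it for Spring (warmer), with level zero restoring the base.
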(event `self.ReceiveTick`
  (params (DeltaSeconds :type "Float (single-precision)"))
  (bind _output_get (set `self.Angle` (- (`self.Angle`) (`self.Speed`))))
  (`SceneComponent.K2_SetWorldRotation` (`self.DirectionalLight`) (`KismetMathLibrary.MakeRotator` 0.0 -40.0 _output_get) false false))

(fn `UpdateTemperature`
  (params (CurrentWinner :type "/Game/Core/E_Faction Enum" :default "NewEnumerator0") (Level :type Integer))
  (locals (DiffFromBaseTemperature :type "Float (double-precision)"))
  (switch `int` Level
    (:`0`
      (`LightComponent.SetTemperature` (`self.DirectionalLight`) (`self.BaseTemperature`))
      (return))
    (:`1`
      (set `local.DiffFromBaseTemperature` 400.0))
    (:`2`
      (set `local.DiffFromBaseTemperature` 900.0))
    (:`3`
      (set `local.DiffFromBaseTemperature` 1800.0)))
  (switch `/Game/Core/E_Faction` (`local.CurrentWinner`)
    (:`NewEnumerator1`
      (`LightComponent.SetTemperature` (`self.DirectionalLight`) (+ (`self.BaseTemperature`) (`local.DiffFromBaseTemperature`))))
    (:`NewEnumerator2`
      (`LightComponent.SetTemperature` (`self.DirectionalLight`) (- (`self.BaseTemperature`) (`local.DiffFromBaseTemperature`)))))
  (return))

(fn `UserConstructionScript`
  (`SceneComponent.K2_SetWorldRotation` (`self.DirectionalLight`) (`KismetMathLibrary.MakeRotator` 0.0 -40.0 (`self.Angle`)) false false))